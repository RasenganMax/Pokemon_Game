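; Test NPC actor that the player's MannequinCharacter can register as its interaction target.
; The construction script slaves modular clothing and accessory meshes to the body SkeletalMesh through Master Pose.
; BeginPlay caches the player character, and Sphere overlaps set or clear that character's InteractActor reference to this NPC.
; Interact is a stub that only returns false.
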(event `self.ReceiveBeginPlay`
  (bind _asmannequin_character (cast `/Game/AdvancedLocomotionV3/Blueprints/MannequinCharacter` (`GameplayStatics.GetPlayerCharacter` 0)))
  (set `self.PlayerRef` _asmannequin_character))

(event `self.Sphere.OnComponentBeginOverlap`
  (params (OverlappedComponent :type "PrimitiveComponent Object Reference") (OtherActor :type "Actor Object Reference") (OtherComp :type "PrimitiveComponent Object Reference") (OtherBodyIndex :type Integer) (bFromSweep :type Boolean) (SweepResult :type "HitResult Structure (by ref)"))
  (bind _playerref (`self.PlayerRef`))
  (if (== OtherActor _playerref)
    (set `/Game/AdvancedLocomotionV3/Blueprints/ALS_BaseCharacter.Interact Actor` self _playerref)))

(event `self.Sphere.OnComponentEndOverlap`
  (params (OverlappedComponent :type "PrimitiveComponent Object Reference") (OtherActor :type "Actor Object Reference") (OtherComp :type "PrimitiveComponent Object Reference") (OtherBodyIndex :type Integer))
  (bind _playerref (`self.PlayerRef`))
  (if (== OtherActor _playerref)
    (set `/Game/AdvancedLocomotionV3/Blueprints/ALS_BaseCharacter.Interact Actor` null _playerref)))

(fn `Interact`
  (returns (Result :type Boolean))
  (return false))

(fn `UserConstructionScript`
  ;[1 1 1] Master Pose
  (`SkinnedMeshComponent.SetLeaderPoseComponent` (`self.Scarf`) (`self.SkeletalMesh`) false)
  (`SkinnedMeshComponent.SetLeaderPoseComponent` (`self.Shirt`) (`self.SkeletalMesh`) false)
  (`SkinnedMeshComponent.SetLeaderPoseComponent` (`self.Shoes`) (`self.SkeletalMesh`) false)
  (`SkinnedMeshComponent.SetLeaderPoseComponent` (`self.Shorts`) (`self.SkeletalMesh`) false)
  (`SkinnedMeshComponent.SetLeaderPoseComponent` (`self.Bag`) (`self.SkeletalMesh`) false)
  (`SkinnedMeshComponent.SetLeaderPoseComponent` (`self.MagikarpHat`) (`self.SkeletalMesh`) false))