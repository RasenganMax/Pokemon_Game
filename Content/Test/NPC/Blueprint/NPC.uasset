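; Interactable NPC character that turns to face the player and starts a dialogue through its AI controller.
; On BeginPlay it adds an NPC UI widget to the viewport and passes its dialogue tree to the controller.
; Sphere overlap sets it as the player's InteractActor, so Interact can trigger Chat.
; Timelines drive facing, spin a marker mesh and show it near the player; clothing follows the body via master pose.
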(event `self.ReceiveBeginPlay`
  (bind _asmannequin_character (cast `/Game/AdvancedLocomotionV3/Blueprints/MannequinCharacter` (`GameplayStatics.GetPlayerCharacter` 0)))
  (set `self.PlayerRef` _asmannequin_character)
  (bind _returnvalue (`|CreateWidget` "/Game/Test/NPC/UserInterface/NPC_WidgetUI.NPC_WidgetUI_C"))
  (bind _output_get (set `self.NPC_Display` _returnvalue))
  (`UserWidget.AddToViewport` _output_get 0)
  (bind _asnpc_controller (cast `/Game/Test/NPC/AI/NPC_Controller` (`AIBlueprintHelperLibrary.GetAIController` self)))
  (bind _output_get_2 (set `self.NPC_Ai_Controller` _asnpc_controller))
  (set `/Game/Test/NPC/AI/NPC_Controller.DialogueTree` (`self.DialagueTree`) _output_get_2)
  (`self.NPCWidget Distance`)
  (`self.WidgetRotation`))

(event `self.Sphere.OnComponentBeginOverlap`
  (params (OverlappedComponent :type "PrimitiveComponent Object Reference") (OtherActor :type "Actor Object Reference") (OtherComp :type "PrimitiveComponent Object Reference") (OtherBodyIndex :type Integer) (bFromSweep :type Boolean) (SweepResult :type "HitResult Structure (by ref)"))
  (bind _playerref (`self.PlayerRef`))
  (bind (_returnvalue_roll _returnvalue_pitch _returnvalue_yaw) (`KismetMathLibrary.BreakRotator` (`KismetMathLibrary.FindLookAtRotation` (`self.K2_GetActorLocation`) (`self.K2_GetActorLocation` (`GameplayStatics.GetPlayerCharacter` 0)))))
  ;[1 1 1] Sphere Overlap
  (if (== OtherActor _playerref)
    (set `/Game/AdvancedLocomotionV3/Blueprints/ALS_BaseCharacter.Interact Actor` self _playerref)
    (`Timeline|ChangeNPCRotation` :!label _label
      (:`Update`
        (`SceneComponent.K2_SetWorldRotation` (`self.CapsuleComponent`) (`KismetMathLibrary.MakeRotator` 0.0 0.0 _returnvalue_yaw) true false)))))

(event `self.Sphere.OnComponentEndOverlap`
  (params (OverlappedComponent :type "PrimitiveComponent Object Reference") (OtherActor :type "Actor Object Reference") (OtherComp :type "PrimitiveComponent Object Reference") (OtherBodyIndex :type Integer))
  (bind _playerref (`self.PlayerRef`))
  ;[1 1 1] Sphere Overlap
  (if (== OtherActor _playerref)
    (set `/Game/AdvancedLocomotionV3/Blueprints/ALS_BaseCharacter.Interact Actor` null _playerref)
    (goto _label :!via `Stop`)))

(event `Chat`
  ;[1 1 1] Chat Interaction
  (`/Game/Test/NPC/AI/NPC_Controller.StartDialogue` (`self.NPC_Ai_Controller`)))

(event `NPCWidget Distance`
  (bind _staticmesh (`self.StaticMesh`))
  ;[1 1 1] NPC Distance From Player For Widget Visibility
  (`Timeline|WidgetDistance`
    (:`Update`
      (if (< (`KismetMathLibrary.VSize` (- (`self.K2_GetActorLocation`) (`self.K2_GetActorLocation` (`GameplayStatics.GetPlayerCharacter` 0)))) 1200.0)
        (`SceneComponent.SetVisibility` _staticmesh true false)
        (else
          (`SceneComponent.SetVisibility` _staticmesh false false))))))

(event `WidgetRotation`
  ;[1 1 1] Widget Rotation
  (`Timeline|Timeline_0`
    (:`Update`
      (`SceneComponent.K2_AddRelativeRotation` (`self.StaticMesh`) (`KismetMathLibrary.MakeRotator` 0.0 0.0 1.0) false false))))

(fn `Interact`
  (returns (Result :type Boolean))
  (`self.Chat`)
  (return false))

(fn `UserConstructionScript`
  (`SkinnedMeshComponent.SetLeaderPoseComponent` (`self.Scarf`) (`self.Mesh`) false)
  (`SkinnedMeshComponent.SetLeaderPoseComponent` (`self.Shirt`) (`self.Mesh`) false)
  (`SkinnedMeshComponent.SetLeaderPoseComponent` (`self.Shoes`) (`self.Mesh`) false)
  (`SkinnedMeshComponent.SetLeaderPoseComponent` (`self.Shorts`) (`self.Mesh`) false)
  (`SkinnedMeshComponent.SetLeaderPoseComponent` (`self.MagikarpHat`) (`self.Mesh`) false))