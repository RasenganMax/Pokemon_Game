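; Bellsprout's Razor Leaf attack actor, which deals damage to an uncaptured Pokemon it hits.
; On spawn it moves its static mesh to a raised relative offset over a short time.
; A Sphere overlap with any BasePokemon arms a per-tick multi-sphere trace on the Camera channel at the Sphere's location.
; The first hit on an uncaptured Pokemon's capsule applies damage once and destroys the actor.
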(event `self.ReceiveBeginPlay`
  (`KismetSystemLibrary.MoveComponentTo` (`self.StaticMesh`) (0.0 0.0 79.0) (struct) false false 2.0))

(event `self.ReceiveTick`
  (params (DeltaSeconds :type "Float (single-precision)"))
  (bind _returnvalue (`SceneComponent.K2_GetComponentLocation` (`self.Sphere`)))
  (if (`self.trace`)
    (bind _outhits (`KismetSystemLibrary.SphereTraceMulti` _returnvalue _returnvalue 45.0 "TraceTypeQuery2"))
    (for _array_element _outhits
      (bind (_bblockinghit _binitialoverlap _time _distance _location _impactpoint _normal _impactnormal _physmat _hitactor _hitcomponent) (`GameplayStatics.BreakHitResult` _array_element))
      (bind _asbase_pokemon (cast `/Game/Test/Pokemon/BasePokemon` _hitactor))
      (if (`.Captured?_49_FCFCC2A54AA9F707F6B658A57C56BE1B` (break `/Game/Test/Details/PokeDetails_St` (`/Game/Test/Pokemon/BasePokemon.PokemonDetails` _asbase_pokemon)))
        _
        (elif (== _hitcomponent (`Character.CapsuleComponent` _asbase_pokemon))
          (`/Engine/EditorBlueprintResources/StandardMacros.DoOnce` false
            (:`Completed`
              (`GameplayStatics.ApplyDamage` _hitactor 40.0 null self)
              (`self.K2_DestroyActor`))))))))

(event `self.Sphere.OnComponentBeginOverlap`
  (params (OverlappedComponent :type "PrimitiveComponent Object Reference") (OtherActor :type "Actor Object Reference") (OtherComp :type "PrimitiveComponent Object Reference") (OtherBodyIndex :type Integer) (bFromSweep :type Boolean) (SweepResult :type "HitResult Structure (by ref)"))
  (cast `/Game/Test/Pokemon/BasePokemon` OtherActor)
  (set `self.trace` true))

(fn `UserConstructionScript`)