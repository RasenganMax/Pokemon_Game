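; Bellsprout Pokémon character with a randomized eye blink and two abilities bound to keys 1 and 2.
; Blinking swaps the eye texture on a dynamic material in an endless delay loop.
; Razor Leaf halts movement, animates, then spawns, launches and destroys a leaf actor.
; Poison Powder spawns particle and sprite effects, repeatedly sphere-tracing to damage uncaptured BasePokemon through a delayed loop while active.
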(event `self.ReceiveBeginPlay`
  (bind _mesh (`self.Mesh`))
  (`parent.ReceiveBeginPlay`)
  (bind _returnvalue (`PrimitiveComponent.CreateDynamicMaterialInstance` _mesh 1 (`PrimitiveComponent.GetMaterial` _mesh 1) "None"))
  (set `self.Eyes Material` _returnvalue)
  (`self.Blinking`))

(event `Blinking`
  ;[1 1 1] Blinking
  (`MaterialInstanceDynamic.SetTextureParameterValue` (`self.Eyes Material`) "Eyes Texture" "/Game/Test/Pokemon/Bellsprout/Materials/Blinked.Blinked" :!label _label)
  (`KismetSystemLibrary.Delay` 0.1)
  (`MaterialInstanceDynamic.SetTextureParameterValue` (`self.Eyes Material`) "Eyes Texture" "/Game/Test/Pokemon/Bellsprout/Materials/pm0069_00_Eye1.pm0069_00_Eye1")
  (`KismetSystemLibrary.Delay` (`KismetMathLibrary.RandomFloatInRange` 1.0 3.5))
  (goto _label))

(event `Key|One`
  (params (Key :type "Key Structure"))
  (:`Pressed`
    (`self.razor_leaf`)))

(event `Key|Two`
  (params (Key :type "Key Structure"))
  (:`Pressed`
    (`self.poison powder`)))

(event `razor_leaf`
  ;[0.2193 1 0.237] razor_leaf
  (if (not (`self.ability_in_use`))
    (`|ExecutionSequence`
      (:`then_0`
        (`ActorComponent.Deactivate` (`self.CharacterMovement`))
        (set `self.ability_in_use` true)
        (`SkeletalMeshComponent.PlayAnimation` (`self.Mesh`) "/Game/Test/Pokemon/Bellsprout/Anims/FlappingLeafs.FlappingLeafs" true))
      (:`then_1`
        (bind _returnvalue (`|SpawnActorFromClass` "/Game/Test/Pokemon/Bellsprout/Blueprint/bell_razor_leaf.bell_razor_leaf_C" (`KismetMathLibrary.MakeTransform` (- (`SceneComponent.K2_GetComponentLocation` (`self.Mesh`)) (0.0 0.0 50.0))) "AlwaysSpawn" "OverrideRootScale" null null)))
      (:`then_2`))
    (`KismetSystemLibrary.Delay` 1.3)
    (`/Engine/EditorBlueprintResources/StandardMacros.IsValid` _returnvalue
      (:`Is Valid`
        (`ActorComponent.Deactivate` (`/Game/Test/Pokemon/Bellsprout/Blueprint/bell_razor_leaf.RotatingMovement` _returnvalue)))
      (:`Is Not Valid`
        _))
    (`SkeletalMeshComponent.PlayAnimation` (`self.Mesh`) "/Game/Test/Pokemon/Bellsprout/Anims/Razorleaf.Razorleaf" false)
    (`KismetSystemLibrary.Delay` 1.0)
    (`/Engine/EditorBlueprintResources/StandardMacros.IsValid` _returnvalue
      (:`Is Valid`
        (`KismetSystemLibrary.MoveComponentTo` (`/Game/Test/Pokemon/Bellsprout/Blueprint/bell_razor_leaf.DefaultSceneRoot` _returnvalue) (- (+ (`self.K2_GetActorLocation`) (* (`self.GetActorForwardVector`) 500.0)) (0.0 0.0 80.0)) (`self.K2_GetActorRotation`) false false 1.0))
      (:`Is Not Valid`
        _))
    (`|ExecutionSequence`
      (:`then_0`
        (`KismetSystemLibrary.Delay` 1.0)
        (`SkeletalMeshComponent.SetAnimationMode` (`self.Mesh`) "AnimationBlueprint"))
      (:`then_1`
        (`/Engine/EditorBlueprintResources/StandardMacros.IsValid` _returnvalue
          (:`Is Valid`
            (`self.K2_DestroyActor` _returnvalue))
          (:`Is Not Valid`
            _))))
    (set `self.ability_in_use` false)
    (`ActorComponent.Activate` (`self.CharacterMovement`) false)))

(event `poison powder`
  (bind _returnvalue (`self.K2_GetActorLocation`))
  (bind _returnvalue_2 (`self.K2_GetActorLocation`))
  ;[1 0 0.09911] poison_powder
  (if (not (`self.poison_powder`))
    ;[0.9809 1 0.2776] damage opponent
    (`|ExecutionSequence`
      (:`then_0`
        (set `self.poison_powder` true)
        (set `self.ability_in_use` true)
        (`ActorComponent.Deactivate` (`self.CharacterMovement`))
        (`SkeletalMeshComponent.PlayAnimation` (`self.Mesh`) "/Game/Test/Pokemon/Bellsprout/Anims/PowderMove.PowderMove" true)
        (bind _returnvalue_3 (`GameplayStatics.SpawnEmitterAtLocation` "/Game/ParticleEffects/AuraFX01/Particles/PoisonPowder.PoisonPowder" _returnvalue (struct) (5.0 5.0 1.0) false))
        (bind _returnvalue_4 (`|SpawnActorFromClass` "/Game/ParticleEffects/Particles_Wind_Control_System/Blueprints/PoisonPowder_Sprites.PoisonPowder_Sprites_C" (`KismetMathLibrary.MakeTransform` _returnvalue) "AlwaysSpawn" "OverrideRootScale" null null))
        (`KismetSystemLibrary.Delay` 2.39)
        (`SkeletalMeshComponent.SetAnimationMode` (`self.Mesh`) "AnimationBlueprint")
        (`ActorComponent.Activate` (`self.CharacterMovement`) false)
        (set `self.ability_in_use` false)
        (`KismetSystemLibrary.Delay` 10.0)
        (`ActorComponent.K2_DestroyComponent` _returnvalue_3)
        (`self.K2_DestroyActor` _returnvalue_4)
        (set `self.poison_powder` false))
      (:`then_1`
        (if (`self.poison_powder`) :!label _label
          (bind _outhits (`KismetSystemLibrary.SphereTraceMulti` :`Start` _returnvalue_2 :`End` _returnvalue_2 :`Radius` 700.0 :`TraceChannel` "TraceTypeQuery2" :`DrawTime` 0.5))
          (for _array_element _outhits
            (bind (_bblockinghit _binitialoverlap _time _distance _location _impactpoint _normal _impactnormal _physmat _hitactor _hitcomponent) (`GameplayStatics.BreakHitResult` _array_element))
            (bind _asbase_pokemon (cast `/Game/Test/Pokemon/BasePokemon` _hitactor))
            (if (`.Captured?_49_FCFCC2A54AA9F707F6B658A57C56BE1B` (break `/Game/Test/Details/PokeDetails_St` (`/Game/Test/Pokemon/BasePokemon.PokemonDetails` _asbase_pokemon)))
              _
              (elif (== (`Character.CapsuleComponent` _asbase_pokemon) _hitcomponent)
                (`GameplayStatics.ApplyDamage` _hitactor 3.0 null self)
                (`KismetSystemLibrary.Delay` 0.5)
                (goto _label)))))))))

(fn `UserConstructionScript`
  (`parent.UserConstructionScript`))