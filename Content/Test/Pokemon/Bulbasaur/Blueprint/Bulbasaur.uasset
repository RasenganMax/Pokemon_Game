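; Bulbasaur character Blueprint implementing its attack moves, with keys 1-4 triggering Tackle, Sleep Powder, Poison Powder and Razor Leaf.
; A shared Ability flag blocks overlapping moves, which combine montages, capsule movement, timed particles and spawned actors.
; Razor Leaf and Leech Seed launch physics projectiles along the camera's forward vector; Leech Seed, Growl, Growth and Vine Whip lack input bindings.
; A dynamic eye material loops random blinks, and Vines follows the body through master pose.
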(event `self.ReceiveBeginPlay`
  (bind _mesh (`self.Mesh`))
  (`parent.ReceiveBeginPlay`)
  (bind _returnvalue (`PrimitiveComponent.CreateDynamicMaterialInstance` _mesh 2 (`PrimitiveComponent.GetMaterial` _mesh 2) "None"))
  (set `self.Eyes Material` _returnvalue)
  (`self.Blinking`)
  (`/Engine/EditorBlueprintResources/StandardMacros.DoOnce` false
    (:`Completed`
      (`self.GetPokeRef`)
      (`PrimitiveComponent.SetCollisionEnabled` (`self.LeftCol`) "NoCollision")
      (`PrimitiveComponent.SetCollisionEnabled` (`self.RightCol`) "NoCollision"))))

(event `GetPokeRef`
  ;[1 1 1] Get Enemy Pokemon
  (bind _asbase_pokemon (cast `/Game/Test/Pokemon/BasePokemon` (`GameplayStatics.GetPlayerCharacter` 0)))
  (set `self.EnemyPokemon` _asbase_pokemon))

(event `self.CapsuleComponent.OnComponentHit`
  (params (HitComponent :type "PrimitiveComponent Object Reference") (OtherActor :type "Actor Object Reference") (OtherComp :type "PrimitiveComponent Object Reference") (NormalImpulse :type "Vector Structure") (Hit :type "HitResult Structure (by ref)"))
  ;[1 1 1] On Hit
)

(event `Blinking`
  ;[1 1 1] Blinking
  (`MaterialInstanceDynamic.SetTextureParameterValue` (`self.Eyes Material`) "Eyes Texture" "/Game/Test/Pokemon/Bulbasaur/Textures/ClosedEyes.ClosedEyes" :!label _label)
  (`KismetSystemLibrary.Delay` 0.1)
  (`MaterialInstanceDynamic.SetTextureParameterValue` (`self.Eyes Material`) "Eyes Texture" "/Game/Test/Pokemon/Bulbasaur/Textures/pm0001_00_Eye1_Merged.pm0001_00_Eye1_Merged")
  (`KismetSystemLibrary.Delay` (`KismetMathLibrary.RandomFloatInRange` 1.0 3.5))
  (goto _label))

(event `Tackle`
  (bind _capsulecomponent (`self.CapsuleComponent`))
  (bind (_returnvalue_roll _returnvalue_pitch _returnvalue_yaw) (`KismetMathLibrary.BreakRotator` (`SceneComponent.K2_GetComponentRotation` (`self.FollowCamera`))))
  ;[1 1 1] Attack Events
  (if (not (`self.Ability`))
    (set `self.Ability` true)
    (`|PlayMontage` (`self.Mesh`) "/Game/Test/Pokemon/Bulbasaur/Anims/Tackle_Montage.Tackle_Montage" 0.8 0.0 "attack"
      (:`then`
        (`KismetSystemLibrary.MoveComponentTo` (`self.CapsuleComponent`) (+ (`SceneComponent.K2_GetComponentLocation` _capsulecomponent) (* (`SceneComponent.GetForwardVector` _capsulecomponent) 300.0)) (`KismetMathLibrary.MakeRotator` 0.0 0.0 _returnvalue_yaw) true true 0.5 true)
        (set `self.Ability` false)))))

(event `Growl`
  (bind _mesh (`self.Mesh`))
  (bind (_returnvalue_x _returnvalue_y _returnvalue_z) (`KismetMathLibrary.BreakVector` (`SceneComponent.K2_GetComponentLocation` _mesh)))
  (bind (_returnvalue_roll _returnvalue_pitch _returnvalue_yaw) (`KismetMathLibrary.BreakRotator` (`SceneComponent.K2_GetComponentRotation` _mesh)))
  ;[1 1 1] Attack Events
  (if (not (`self.Ability`))
    (`|ExecutionSequence`
      (:`then_0`
        (set `self.Ability` true)
        (`|PlayMontage` (`self.Mesh`) "/Game/Test/Pokemon/Bulbasaur/Anims/Cry_Montage.Cry_Montage" 1.0 0.0 "Growl"
          (:`OnCompleted`
            (set `self.Ability` false))))
      (:`then_1`
        (`KismetSystemLibrary.Delay` 0.8)
        (bind _returnvalue (`GameplayStatics.SpawnEmitterAtLocation` "/Game/ParticleEffects/BeamAndLaserFX01/Particles/BulbasaurGrowl.BulbasaurGrowl" (`KismetMathLibrary.MakeVector` (+ _returnvalue_x -10.0) _returnvalue_y (+ _returnvalue_z 30.0)) (`KismetMathLibrary.MakeRotator` _returnvalue_roll _returnvalue_pitch (+ _returnvalue_yaw 90.0))))
        (`ParticleSystemComponent.SetBeamTargetPoint` _returnvalue 6 (`self.K2_GetActorLocation` (`self.EnemyPokemon`)) 0)))))

(event `VineWhip`
  ;[1 1 1] Attack Events
  (if (not (`self.Ability`))
    (set `self.Ability` true)
    (`|PlayMontage` (`self.Mesh`) "/Game/Test/Pokemon/Bulbasaur/Anims/VineWhip_Montage.VineWhip_Montage" 1.0 0.0 "Vine"
      (:`OnCompleted`
        (set `self.Ability` false)))))

(event `Growth`
  (bind _mesh (`self.Mesh`))
  ;[1 1 1] Attack Events
  (if (not (`self.Ability`))
    (set `self.Ability` true)
    (bind _returnvalue (`GameplayStatics.SpawnEmitterAttached` "/Game/ParticleEffects/AuraFX01/Particles/Growth_1.Growth_1" _mesh "None" (0.0 0.0 25.0) (struct) (0.6 0.6 0.6) "SnapToTarget" false))
    (`KismetSystemLibrary.Delay` 1.0)
    (bind _returnvalue_2 (`GameplayStatics.SpawnEmitterAttached` "/Game/ParticleEffects/AuraFX01/Particles/Growth_2.Growth_2" _mesh "None" (0.0 0.0 25.0) (struct) (0.6 0.6 0.6) "SnapToTarget" false))
    (`KismetSystemLibrary.Delay` 5.0)
    (`ActorComponent.K2_DestroyComponent` _returnvalue_2)
    (`ActorComponent.K2_DestroyComponent` _returnvalue)
    (set `self.Ability` false)))

(event `RazorLeaf`
  (bind _delayleaf (`self.DelayLeaf`))
  (bind _returnvalue (`SceneComponent.K2_GetComponentLocation` (`self.CapsuleComponent`)))
  ;[1 1 1] Attack Events
  (if (not (`self.Ability`))
    (set `self.Ability` true)
    (`|ExecutionSequence`
      (:`then_0`
        (bind _returnvalue_2 (`|SpawnActorFromClass` "/Game/Test/Pokemon/Bulbasaur/StaticMesh/RazorLeaf_BP.RazorLeaf_BP_C" (`KismetMathLibrary.MakeTransform` (`KismetMathLibrary.MakeVector` (.x _returnvalue) (+ (.y _returnvalue) 50.0) (.z _returnvalue))) "AdjustIfPossibleButAlwaysSpawn" "OverrideRootScale" self null))
        (bind _output_get (set `self.RazorLeafRight` _returnvalue_2))
        (`self.K2_SetActorRotation` _output_get (struct :`Roll` -25.0) false)
        (bind _razorleaf (`/Game/Test/Pokemon/Bulbasaur/StaticMesh/RazorLeaf_BP.RazorLeaf` _output_get))
        (`PrimitiveComponent.SetSimulatePhysics` _razorleaf false)
        (`KismetSystemLibrary.MoveComponentTo` _razorleaf (+ (`SceneComponent.K2_GetComponentLocation` _razorleaf) (`KismetMathLibrary.MakeVector` 0.0 10.0 (`self.RazorLeafUp`))) (`SceneComponent.K2_GetComponentRotation` _razorleaf) true true 0.2 true)
        (`PrimitiveComponent.SetSimulatePhysics` _razorleaf true)
        (`KismetSystemLibrary.Delay` _delayleaf)
        (`PrimitiveComponent.AddImpulse` _razorleaf (`self.GetRazorLeafVelocity`) "None" false))
      (:`then_1`
        (bind _returnvalue_3 (`|SpawnActorFromClass` "/Game/Test/Pokemon/Bulbasaur/StaticMesh/RazorLeaf_BP.RazorLeaf_BP_C" (`KismetMathLibrary.MakeTransform` (`KismetMathLibrary.MakeVector` (.x _returnvalue) (+ (.y _returnvalue) -50.0) (.z _returnvalue))) "AdjustIfPossibleButAlwaysSpawn" "OverrideRootScale" null null))
        (bind _output_get_2 (set `self.RazorLeafLeft` _returnvalue_3))
        (`self.K2_SetActorRotation` _output_get_2 (struct :`Roll` 25.0) false)
        (bind _razorleaf_2 (`/Game/Test/Pokemon/Bulbasaur/StaticMesh/RazorLeaf_BP.RazorLeaf` _output_get_2))
        (`PrimitiveComponent.SetSimulatePhysics` _razorleaf_2 false)
        (`KismetSystemLibrary.MoveComponentTo` _razorleaf_2 (+ (`SceneComponent.K2_GetComponentLocation` _razorleaf_2) (`KismetMathLibrary.MakeVector` 0.0 -10.0 (`self.RazorLeafUp`))) (`SceneComponent.K2_GetComponentRotation` _razorleaf_2) true true 0.2 true)
        (`PrimitiveComponent.SetSimulatePhysics` _razorleaf_2 true)
        (`KismetSystemLibrary.Delay` _delayleaf)
        (`PrimitiveComponent.AddImpulse` _razorleaf_2 (`self.GetRazorLeafVelocity`) "None" false)))
    (`KismetSystemLibrary.Delay` 2.0)
    (`self.K2_DestroyActor` _output_get)
    (`self.K2_DestroyActor` _output_get_2)
    (set `self.Ability` false)))

(event `LeechSeed`
  (bind _bulletseed (`self.BulletSeed`))
  (bind (_returnvalue_x _returnvalue_y _returnvalue_z) (`KismetMathLibrary.BreakVector` (`SceneComponent.GetSocketLocation` (`self.Mesh`) "BulletSeed")))
  ;[1 1 1] Attack Events
  (if (not (`self.Ability`))
    (set `self.Ability` true)
    (`|ExecutionSequence`
      (:`then_0`
        (`|PlayMontage` (`self.Mesh`) "/Game/Test/Pokemon/Bulbasaur/Anims/BulletSeed_Montage.BulletSeed_Montage" 1.0 0.0 "None"
          (:`OnCompleted`
            (set `self.Ability` false))))
      (:`then_1`
        (`SceneComponent.SetVisibility` _bulletseed true false)
        (`KismetSystemLibrary.Delay` 0.95)
        (`SceneComponent.SetVisibility` _bulletseed false false)
        (bind _returnvalue (`|SpawnActorFromClass` "/Game/Test/Pokemon/Bulbasaur/StaticMesh/BulletSeed_BP.BulletSeed_BP_C" (`KismetMathLibrary.MakeTransform` (`KismetMathLibrary.MakeVector` _returnvalue_x _returnvalue_y (+ _returnvalue_z (`self.BulletSeendHeight`)))) "AdjustIfPossibleButAlwaysSpawn" "OverrideRootScale" self null))
        (bind _output_get (set `self.NewVar_1` _returnvalue))
        (`PrimitiveComponent.AddImpulse` (`/Game/Test/Pokemon/Bulbasaur/StaticMesh/BulletSeed_BP.BulletSeed` _output_get) (`self.GetBulletSeedVelocity`) "None" false)
        (`KismetSystemLibrary.Delay` 2.0)
        (`self.K2_DestroyActor` _returnvalue)))))

(event `PoisonPowder`
  (bind _returnvalue (`self.K2_GetActorLocation`))
  ;[1 1 1] Attack Events
  (if (not (`self.Ability`))
    (set `self.Ability` true)
    (`|ExecutionSequence`
      (:`then_0`
        (bind _returnvalue_2 (`GameplayStatics.SpawnEmitterAtLocation` "/Game/ParticleEffects/AuraFX01/Particles/PoisonPowder.PoisonPowder" _returnvalue (struct) (5.0 5.0 1.0) false))
        (bind _returnvalue_3 (`|SpawnActorFromClass` "/Game/ParticleEffects/Particles_Wind_Control_System/Blueprints/PoisonPowder_Sprites.PoisonPowder_Sprites_C" (`KismetMathLibrary.MakeTransform` _returnvalue) "AlwaysSpawn" "OverrideRootScale" null null))
        (`KismetSystemLibrary.Delay` 15.0)
        (`ActorComponent.K2_DestroyComponent` _returnvalue_2)
        (`self.K2_DestroyActor` _returnvalue_3)
        (set `self.Ability` false))
      (:`then_1`
        (bind _returnvalue_4 (`GameplayStatics.SpawnEmitterAttached` "/Game/Test/Pokemon/Bulbasaur/StaticMesh/Poisonpowder_smoke.Poisonpowder_smoke" (`self.Mesh`) "BulletSeed" (0.0 0.0 0.0) (struct :`Pitch` -90.0)))
        (`KismetSystemLibrary.Delay` 10.0)
        (`ActorComponent.K2_DestroyComponent` _returnvalue_4)))))

(event `SleepPowder`
  (bind _returnvalue (`self.K2_GetActorLocation`))
  ;[1 1 1] Attack Events
  (if (not (`self.Ability`))
    (set `self.Ability` true)
    (`|ExecutionSequence`
      (:`then_0`
        (bind _returnvalue_2 (`GameplayStatics.SpawnEmitterAtLocation` "/Game/ParticleEffects/AuraFX01/Particles/SleepPowder.SleepPowder" _returnvalue (struct) (5.0 5.0 2.0) false))
        (bind _returnvalue_3 (`|SpawnActorFromClass` "/Game/ParticleEffects/Particles_Wind_Control_System/Blueprints/SleepPowder_Sprites.SleepPowder_Sprites_C" (`KismetMathLibrary.MakeTransform` _returnvalue) "AlwaysSpawn" "OverrideRootScale" null null))
        (`KismetSystemLibrary.Delay` 15.0)
        (`ActorComponent.K2_DestroyComponent` _returnvalue_2)
        (`self.K2_DestroyActor` _returnvalue_3)
        (set `self.Ability` false))
      (:`then_1`
        (bind _returnvalue_4 (`GameplayStatics.SpawnEmitterAttached` "/Game/Test/Pokemon/Bulbasaur/StaticMesh/sleeppowder_smoke.sleeppowder_smoke" (`self.Mesh`) "BulletSeed" (0.0 0.0 0.0) (struct :`Pitch` -90.0)))
        (`KismetSystemLibrary.Delay` 10.0)
        (`ActorComponent.K2_DestroyComponent` _returnvalue_4)))))

(event `Key|Three`
  (params (Key :type "Key Structure"))
  ;[1 1 1] Ability 3
  (:`Pressed`
    (`self.PoisonPowder`)))

(event `Key|Four`
  (params (Key :type "Key Structure"))
  ;[1 1 1] Ability 4
  (:`Pressed`
    (`self.RazorLeaf`)))

(event `Key|One`
  (params (Key :type "Key Structure"))
  ;[1 1 1] Ability 1
  (:`Pressed`
    (`self.Tackle`)))

(event `Key|Two`
  (params (Key :type "Key Structure"))
  ;[1 1 1] Ability 2
  (:`Pressed`
    (`self.SleepPowder`)))

(fn `GetBulletSeedVelocity`
  (returns (Direction :type "Vector Structure"))
  (return (* (`SceneComponent.GetForwardVector` (`self.FollowCamera`)) (`self.BulletSeedSpeed`))))

(fn `GetRazorLeafVelocity`
  (returns (Direction :type "Vector Structure"))
  (return (* (`SceneComponent.GetForwardVector` (`self.FollowCamera`)) (`self.RazorLeafSpeed`))))

(fn `UserConstructionScript`
  (`parent.UserConstructionScript`)
  (`SkinnedMeshComponent.SetLeaderPoseComponent` (`self.Vines`) (`self.Mesh`) false))