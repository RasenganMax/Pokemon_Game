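; RazorLeaf_BP is a Razor Leaf projectile actor for Bulbasaur that can home in on Pokémon.
; MoveToTarget zeroes velocity and enables projectile homing on the mesh returned by HomingTarget, which searches all BasePokemon for the nearest uncaptured one.
; Hit fires a radial force impulse and destroys the actor.
; BeginPlay is empty and the only MoveToTarget call here is disconnected, so homing relies on an external trigger.
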(event `self.ReceiveHit`
  (params (MyComp :type "PrimitiveComponent Object Reference") (Other :type "Actor Object Reference") (OtherComp :type "PrimitiveComponent Object Reference") (bSelfMoved :type Boolean) (HitLocation :type "Vector Structure") (HitNormal :type "Vector Structure") (NormalImpulse :type "Vector Structure") (Hit :type "HitResult Structure (by ref)"))
  (`RadialForceComponent.FireImpulse` (`self.RadialForce`))
  (`self.K2_DestroyActor`))

(event `MoveToTarget`
  (bind _projectilemovement (`self.ProjectileMovement`))
  (bind _mytarget (`self.HomingTarget`))
  (set `ProjectileMovementComponent.HomingTargetComponent` _mytarget _projectilemovement)
  (set `ProjectileMovementComponent.bIsHomingProjectile` true _projectilemovement)
  (set `MovementComponent.Velocity` (0.0 0.0 0.0) _projectilemovement))

(event `self.ReceiveBeginPlay`)

(fn `HomingTarget`
  (returns (MyTarget :type "SceneComponent Object Reference"))
  (locals (ClosestDistance :type "Float (double-precision)") (ClosestTarget :type "/Game/Test/Pokemon/BasePokemon Object Reference"))
  (bind _outactors (`GameplayStatics.GetAllActorsOfClass` "/Game/Test/Pokemon/BasePokemon.BasePokemon_C"))
  (for _array_element _outactors
    (bind (_pokemondetails_pokemon_type _pokemondetails_pokemon_type2 _pokemondetails_pokemon_image _pokemondetails_pokemon_class _pokemondetails_pokemon_speed _pokemondetails_pokemon_hp _pokemondetails_pokemonatk1_dmg _pokemondetails_pokemonatk2_dmg _pokemondetails_pokemonatk3_dmg _pokemondetails_pokemonatk4_dmg _pokemondetails_pokemonatk_vfx _pokemondetails_pokemonatk_sfx _pokemondetails_pokemon_number _pokemondetails_pokemon_index _pokemondetails_pokemon_level _pokemondetails_pokemoncurrent_xp _pokemondetails_pokmonneeded_xp _pokemondetails_pokemon_name _pokemondetails_captured_) (break `/Game/Test/Details/PokeDetails_St` (`/Game/Test/Pokemon/BasePokemon.PokemonDetails` _array_element)))
    (if (not _pokemondetails_captured_)
      (bind _returnvalue (`KismetMathLibrary.VSize` (- (`self.K2_GetActorLocation`) (`SceneComponent.K2_GetComponentLocation` (`Character.Mesh` _array_element)))))
      (if (< _returnvalue (`local.ClosestDistance`))
        (set `local.ClosestDistance` _returnvalue)
        (set `local.ClosestTarget` _array_element))))
  (return (`Character.Mesh` (`local.ClosestTarget`))))

(fn `UserConstructionScript`)