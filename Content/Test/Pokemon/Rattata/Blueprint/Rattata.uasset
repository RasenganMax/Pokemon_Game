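; Rattata Pokémon actor Blueprint that gives its mesh an endless eye-blink animation.
; On BeginPlay, after calling the parent, it creates a dynamic material instance for the eye slot of the mesh and starts the blink loop.
; The loop briefly swaps the eye texture parameter to a closed-eye texture, restores it, then waits a random interval before repeating, so blinks look irregular.
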(event `self.ReceiveBeginPlay`
  (bind _mesh (`self.Mesh`))
  (`parent.ReceiveBeginPlay`)
  (bind _returnvalue (`PrimitiveComponent.CreateDynamicMaterialInstance` _mesh 2 (`PrimitiveComponent.GetMaterial` _mesh 2) "None"))
  (set `self.Eyes Material` _returnvalue)
  (`self.Blinking`))

(event `Blinking`
  ;[1 1 1] Blinking
  (`MaterialInstanceDynamic.SetTextureParameterValue` (`self.Eyes Material`) "Eyes Texture" "/Game/Test/Pokemon/Rattata/Textures/BlinkEyes.BlinkEyes" :!label _label)
  (`KismetSystemLibrary.Delay` 0.1)
  (`MaterialInstanceDynamic.SetTextureParameterValue` (`self.Eyes Material`) "Eyes Texture" "/Game/Test/Pokemon/Rattata/Textures/eyes.eyes")
  (`KismetSystemLibrary.Delay` (`KismetMathLibrary.RandomFloatInRange` 1.0 3.5))
  (goto _label))

(fn `UserConstructionScript`
  (`parent.UserConstructionScript`))