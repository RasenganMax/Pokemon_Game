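; Eevee companion Pokémon character that the player can interact with and pick up to carry.
; On BeginPlay it makes a dynamic eye material and loops random blinks by swapping textures.
; Sphere overlap toggles a prompt widget and registers it as the player's interact actor.
; Equipping makes the player kneel, then Eevee walks over, jumps, and attaches to the player's equip location with movement and collision off, all timed by delays.
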(event `self.ReceiveBeginPlay`
  (bind _mesh (`self.Mesh`))
  (`parent.ReceiveBeginPlay`)
  (bind _returnvalue (`PrimitiveComponent.CreateDynamicMaterialInstance` _mesh 1 (`PrimitiveComponent.GetMaterial` _mesh 1) "None"))
  (set `self.Eyes Material` _returnvalue)
  (`self.Blinking`)
  (bind _asmannequin_character (cast `/Game/AdvancedLocomotionV3/Blueprints/MannequinCharacter` (`GameplayStatics.GetPlayerCharacter` 0)))
  (set `self.MainCharacter` _asmannequin_character))

(event `Blinking`
  ;[1 1 1] Blinking
  (`MaterialInstanceDynamic.SetTextureParameterValue` (`self.Eyes Material`) "Eyes Texture" "/Game/Test/Pokemon/Eevee/Mats/EyesBlink.EyesBlink" :!label _label)
  (`KismetSystemLibrary.Delay` 0.1)
  (`MaterialInstanceDynamic.SetTextureParameterValue` (`self.Eyes Material`) "Eyes Texture" "/Game/Test/Pokemon/Eevee/Mats/Eyes.Eyes")
  (`KismetSystemLibrary.Delay` (`KismetMathLibrary.RandomFloatInRange` 1.0 3.5))
  (goto _label))

(event `self.Sphere.OnComponentBeginOverlap`
  (params (OverlappedComponent :type "PrimitiveComponent Object Reference") (OtherActor :type "Actor Object Reference") (OtherComp :type "PrimitiveComponent Object Reference") (OtherBodyIndex :type Integer) (bFromSweep :type Boolean) (SweepResult :type "HitResult Structure (by ref)"))
  (bind _playerref (`self.PlayerRef`))
  ;[0.3496 1 0.6541] Icon Visibility
  (if (== OtherActor _playerref)
    (set `/Game/AdvancedLocomotionV3/Blueprints/ALS_BaseCharacter.Interact Actor` self _playerref)
    (`SceneComponent.SetVisibility` (`self.Widget`) true false)))

(event `self.Sphere.OnComponentEndOverlap`
  (params (OverlappedComponent :type "PrimitiveComponent Object Reference") (OtherActor :type "Actor Object Reference") (OtherComp :type "PrimitiveComponent Object Reference") (OtherBodyIndex :type Integer))
  (bind _playerref (`self.PlayerRef`))
  ;[0.3496 1 0.6541] Icon Visibility
  (if (== _playerref OtherActor)
    (set `/Game/AdvancedLocomotionV3/Blueprints/ALS_BaseCharacter.Interact Actor` null _playerref)
    (`SceneComponent.SetVisibility` (`self.Widget`) false false)))

(event `EquipToCharacter`
  (`|ExecutionSequence`
    (:`then_0`
      (`/Game/AdvancedLocomotionV3/Blueprints/MannequinCharacter.KneelingToPickUp` (`self.MainCharacter`)))
    (:`then_1`
      (`self.AttachPokemon`))))

(event `AttachPokemon`
  (bind _maincharacter (`self.MainCharacter`))
  (bind _equiplocation (`/Game/AdvancedLocomotionV3/Blueprints/MannequinCharacter.EquipLocation` _maincharacter))
  (`KismetSystemLibrary.Delay` 2.767)
  (`AIBlueprintHelperLibrary.SimpleMoveToActor` (`AIBlueprintHelperLibrary.GetAIController` self) (`self.MainCharacter`))
  (`KismetSystemLibrary.Delay` 2.767)
  (`MovementComponent.StopMovementImmediately` (`self.CharacterMovement`))
  (`self.PlayAnimMontage` null 1.0 "Jump")
  (`KismetSystemLibrary.Delay` 1.7)
  (`self.K2_AttachToComponent` _equiplocation (`SceneComponent.GetAttachSocketName` _equiplocation) "SnapToTarget" "SnapToTarget" "KeepWorld" false)
  (`CharacterMovementComponent.DisableMovement` (`self.CharacterMovement`))
  (`PrimitiveComponent.SetCollisionEnabled` (`self.CapsuleComponent`) "NoCollision")
  (`/Game/AdvancedLocomotionV3/Blueprints/MannequinCharacter.StandingUp` _maincharacter)
  (set `/Game/AdvancedLocomotionV3/Blueprints/MannequinCharacter.PokemonEquipped` true (`self.MainCharacter`)))

(fn `UserConstructionScript`
  (`parent.UserConstructionScript`))