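; Charmander Pokémon character that the player can interact with, with animated blinking eyes.
; A looping event swaps the eye texture on a dynamic material at random intervals.
; Sphere overlaps toggle an icon widget and set or clear the player's InteractActor.
; Interact turns it toward the player and plays a playful montage, then after a short delay spawns its default controller, sets walking mode and levels its rotation.
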(event `self.ReceiveBeginPlay`
  (bind _mesh (`self.Mesh`))
  (`parent.ReceiveBeginPlay`)
  (bind _returnvalue (`PrimitiveComponent.CreateDynamicMaterialInstance` _mesh 1 (`PrimitiveComponent.GetMaterial` _mesh 1) "None"))
  (set `self.Eyes Material` _returnvalue)
  (`self.Blinking`))

(event `Blinking`
  ;[1 1 1] Blinking
  (`MaterialInstanceDynamic.SetTextureParameterValue` (`self.Eyes Material`) "Eyes Texture" "/Game/Test/Pokemon/Charmander/Textures/Base/Blink.Blink" :!label _label)
  (`KismetSystemLibrary.Delay` 0.1)
  (`MaterialInstanceDynamic.SetTextureParameterValue` (`self.Eyes Material`) "Eyes Texture" "/Game/Test/Pokemon/Charmander/Textures/Base/pm0004_00_Eye1_tga.pm0004_00_Eye1_tga")
  (`KismetSystemLibrary.Delay` (`KismetMathLibrary.RandomFloatInRange` 1.0 3.5))
  (goto _label))

(event `Interaction`
  (bind (_returnvalue_roll _returnvalue_pitch _returnvalue_yaw) (`KismetMathLibrary.BreakRotator` (`self.K2_GetActorRotation`)))
  (bind (_returnvalue_roll_2 _returnvalue_pitch_2 _returnvalue_yaw_2) (`KismetMathLibrary.BreakRotator` (`KismetMathLibrary.FindLookAtRotation` (`self.K2_GetActorLocation`) (`self.K2_GetActorLocation` (`GameplayStatics.GetPlayerCharacter` 0)))))
  ;[1 1 1] Inteacting With Main
  (`SceneComponent.K2_SetWorldRotation` (`self.CapsuleComponent`) (`KismetMathLibrary.MakeRotator` 0.0 0.0 _returnvalue_yaw_2) true false)
  (`|PlayMontage` (`self.Mesh`) "/Game/Test/Pokemon/Charmander/Anims/Playful2_Montage.Playful2_Montage"
    (:`then`
      (`KismetSystemLibrary.Delay` 1.208)
      (`self.SpawnDefaultController`)
      (`CharacterMovementComponent.SetMovementMode` (`self.CharacterMovement`) "MOVE_Walking" 0)
      (`SceneComponent.K2_SetWorldRotation` (`self.CapsuleComponent`) (`KismetMathLibrary.MakeRotator` 0.0 0.0 _returnvalue_yaw) false false))))

(event `self.Sphere.OnComponentBeginOverlap`
  (params (OverlappedComponent :type "PrimitiveComponent Object Reference") (OtherActor :type "Actor Object Reference") (OtherComp :type "PrimitiveComponent Object Reference") (OtherBodyIndex :type Integer) (bFromSweep :type Boolean) (SweepResult :type "HitResult Structure (by ref)"))
  (bind _playerref (`self.PlayerRef`))
  ;[0.3496 1 0.6541] Icon Visibility
  (if (== OtherActor _playerref)
    (set `/Game/AdvancedLocomotionV3/Blueprints/ALS_BaseCharacter.Interact Actor` self _playerref)
    (`SceneComponent.SetVisibility` (`self.Widget`) true false)))

(event `self.Sphere.OnComponentEndOverlap`
  (params (OverlappedComponent :type "PrimitiveComponent Object Reference") (OtherActor :type "Actor Object Reference") (OtherComp :type "PrimitiveComponent Object Reference") (OtherBodyIndex :type Integer))
  (bind _playerref (`self.PlayerRef`))
  ;[0.3496 1 0.6541] Icon Visibility
  (if (== _playerref OtherActor)
    (set `/Game/AdvancedLocomotionV3/Blueprints/ALS_BaseCharacter.Interact Actor` null _playerref)
    (`SceneComponent.SetVisibility` (`self.Widget`) false false)))

(fn `Interact`
  (returns (Result :type Boolean))
  (`self.Interaction`)
  (return false))

(fn `UserConstructionScript`
  (`parent.UserConstructionScript`))