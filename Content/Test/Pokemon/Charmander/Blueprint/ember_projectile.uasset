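; Ember projectile, apparently Charmander's attack, that damages Pokemon and explodes into fire when it stops moving.
; A Sphere overlap with any BasePokemon arms a per-tick sphere trace that ignores the player Charmander, damages capsule hits and destroys the projectile.
; Zero velocity triggers an explosion, a FireStarter_BP spawn and a wider, stronger damage trace, destroying the projectile only inside that hit loop.
; Mesh collision switches on shortly after BeginPlay.
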(event `self.ReceiveTick`
  (params (DeltaSeconds :type "Float (single-precision)"))
  (bind _projectilemovement (`self.ProjectileMovement`))
  (bind _staticmesh (`self.StaticMesh`))
  (bind _returnvalue (`SceneComponent.K2_GetComponentLocation` _staticmesh))
  (bind _returnvalue_2 (`SceneComponent.K2_GetComponentLocation` (`self.StaticMesh`)))
  (bind _returnvalue_3 (`SceneComponent.K2_GetComponentLocation` (`self.StaticMesh`)))
  (`|ExecutionSequence`
    (:`then_0`
      (if (`self.trace`)
        (bind _ascharmander (cast `/Game/Test/Pokemon/Charmander/Blueprint/Charmander` (`GameplayStatics.GetPlayerCharacter` 0)))
        (bind _outhits (`KismetSystemLibrary.SphereTraceMulti` _returnvalue_3 _returnvalue_3 75.0 "TraceTypeQuery2" false (`|MakeArray` _ascharmander :!type "Actor Object Reference")))
        (for _array_element _outhits
          (bind (_bblockinghit _binitialoverlap _time _distance _location _impactpoint _normal _impactnormal _physmat _hitactor _hitcomponent) (`GameplayStatics.BreakHitResult` _array_element))
          (bind _asbase_pokemon (cast `/Game/Test/Pokemon/BasePokemon` _hitactor))
          (if (== (`Character.CapsuleComponent` _asbase_pokemon) _hitcomponent)
            (`GameplayStatics.ApplyDamage` _hitactor 40.0 null self)
            (`GameplayStatics.SpawnEmitterAtLocation` "/Game/ParticleEffects/AdvancedMagicFX11/Particles/Hit_Test.Hit_Test" (`self.K2_GetActorLocation` _hitactor))
            (`self.K2_DestroyActor`)))))
    (:`then_1`
      (`/Engine/EditorBlueprintResources/StandardMacros.IsValid` _projectilemovement
        (:`Is Valid`
          (if (== (`KismetMathLibrary.VSize` (`MovementComponent.Velocity` _projectilemovement)) 0.0)
            (`/Engine/EditorBlueprintResources/StandardMacros.IsValid` _staticmesh
              (:`Is Valid`
                (`GameplayStatics.SpawnEmitterAtLocation` "/Game/ParticleEffects/AdvancedMagicFX17/Particles/P_ky_bomb2.P_ky_bomb2" _returnvalue (struct) (0.4 0.4 0.4))
                (`|SpawnActorFromClass` "/Game/Landscape/DynamicGrassSystem/Blueprints/FireStarter_BP.FireStarter_BP_C" (`KismetMathLibrary.MakeTransform` _returnvalue) "AlwaysSpawn" "OverrideRootScale" null true true 20 null false null true null)
                (bind _outhits_2 (`KismetSystemLibrary.SphereTraceMulti` _returnvalue_2 _returnvalue_2 159.0 "TraceTypeQuery2"))
                (for _array_element_2 _outhits_2
                  (bind (_bblockinghit_2 _binitialoverlap_2 _time_2 _distance_2 _location_2 _impactpoint_2 _normal_2 _impactnormal_2 _physmat_2 _hitactor_2 _hitcomponent_2) (`GameplayStatics.BreakHitResult` _array_element_2))
                  (bind _asbase_pokemon_2 (cast `/Game/Test/Pokemon/BasePokemon` _hitactor_2))
                  (if (== (`Character.CapsuleComponent` _asbase_pokemon_2) _hitcomponent_2)
                    (`GameplayStatics.ApplyDamage` _hitactor_2 80.0 null self)
                    (`GameplayStatics.SpawnEmitterAtLocation` "/Game/ParticleEffects/AdvancedMagicFX11/Particles/Hit_Test.Hit_Test" (`self.K2_GetActorLocation` _hitactor_2)))
                  (`self.K2_DestroyActor`))))))))))

(event `self.Sphere.OnComponentBeginOverlap`
  (params (OverlappedComponent :type "PrimitiveComponent Object Reference") (OtherActor :type "Actor Object Reference") (OtherComp :type "PrimitiveComponent Object Reference") (OtherBodyIndex :type Integer) (bFromSweep :type Boolean) (SweepResult :type "HitResult Structure (by ref)"))
  (cast `/Game/Test/Pokemon/BasePokemon` OtherActor)
  (set `self.trace` true))

(event `self.ReceiveBeginPlay`
  (`KismetSystemLibrary.Delay` 0.4)
  (`PrimitiveComponent.SetCollisionEnabled` (`self.StaticMesh`) "QueryAndPhysics")
  (`KismetSystemLibrary.Delay` 0.7))

(fn `UserConstructionScript`)