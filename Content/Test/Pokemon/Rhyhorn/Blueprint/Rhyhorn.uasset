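; Rhyhorn is a mountable Pokemon character that the player can ride.
; A sphere overlap shows an interaction widget and registers it as the player's InteractActor; Interact then calls Mount.
; Mount sequences delayed lie-down, sit and stand-up montages, attaches the player with collision off and calls ChangeToPokemon, while pressing Interact when mounted reverses this.
; A looping event swaps eye textures on a dynamic material for random blinking.
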(event `self.ReceiveBeginPlay`
  (bind _mesh (`self.Mesh`))
  (`parent.ReceiveBeginPlay`)
  (bind _returnvalue (`PrimitiveComponent.CreateDynamicMaterialInstance` _mesh 2 (`PrimitiveComponent.GetMaterial` _mesh 2) "None"))
  (set `self.Eyes Material` _returnvalue)
  (`self.Blinking`)
  (bind _asmannequin_character (cast `/Game/AdvancedLocomotionV3/Blueprints/MannequinCharacter` (`GameplayStatics.GetPlayerCharacter` 0)))
  (set `self.MainChar_0` _asmannequin_character))

(event `Blinking`
  ;[1 1 1] Blinking
  (`MaterialInstanceDynamic.SetTextureParameterValue` (`self.Eyes Material`) "Eyes Texture" "/Game/Test/Pokemon/Rhyhorn/Textures/Base/EyesClosed.EyesClosed" :!label _label)
  (`KismetSystemLibrary.Delay` 0.1)
  (`MaterialInstanceDynamic.SetTextureParameterValue` (`self.Eyes Material`) "Eyes Texture" "/Game/Test/Pokemon/Rhyhorn/Textures/Base/pm0111_00_Eye1.pm0111_00_Eye1")
  (`KismetSystemLibrary.Delay` (`KismetMathLibrary.RandomFloatInRange` 1.0 3.5))
  (goto _label))

(event `self.Sphere.OnComponentBeginOverlap`
  (params (OverlappedComponent :type "PrimitiveComponent Object Reference") (OtherActor :type "Actor Object Reference") (OtherComp :type "PrimitiveComponent Object Reference") (OtherBodyIndex :type Integer) (bFromSweep :type Boolean) (SweepResult :type "HitResult Structure (by ref)"))
  (bind _playerref (`self.PlayerRef`))
  ;[0.3496 1 0.6541] Icon Visibility
  (if (== OtherActor _playerref)
    (set `/Game/AdvancedLocomotionV3/Blueprints/ALS_BaseCharacter.Interact Actor` self _playerref)
    (`SceneComponent.SetVisibility` (`self.Widget`) true false)))

(event `self.Sphere.OnComponentEndOverlap`
  (params (OverlappedComponent :type "PrimitiveComponent Object Reference") (OtherActor :type "Actor Object Reference") (OtherComp :type "PrimitiveComponent Object Reference") (OtherBodyIndex :type Integer))
  (bind _playerref (`self.PlayerRef`))
  ;[0.3496 1 0.6541] Icon Visibility
  (if (== _playerref OtherActor)
    (set `/Game/AdvancedLocomotionV3/Blueprints/ALS_BaseCharacter.Interact Actor` null _playerref)
    (`SceneComponent.SetVisibility` (`self.Widget`) false false)))

(event `Mount`
  (bind _mainchar_0 (`self.MainChar_0`))
  (bind _mainchar_0_2 (`self.MainChar_0`))
  (bind _charactermovement (`Character.CharacterMovement` _mainchar_0))
  (`/Engine/EditorBlueprintResources/StandardMacros.IsValid` (`/Game/AdvancedLocomotionV3/Blueprints/MannequinCharacter.PokemonRef` _mainchar_0)
    (:`Is Valid`
      (if (not (`/Game/AdvancedLocomotionV3/Blueprints/MannequinCharacter.IsCharacterMounted?` _mainchar_0))
        (`PrimitiveComponent.SetCollisionEnabled` (`Character.CapsuleComponent` _mainchar_0) "NoCollision")
        (`CharacterMovementComponent.DisableMovement` (`self.CharacterMovement`))
        (`MovementComponent.StopMovementImmediately` _charactermovement)
        (`CharacterMovementComponent.SetMovementMode` _charactermovement "MOVE_Flying" 0)
        (`|PlayMontage` (`self.Mesh`) "/Game/Test/Pokemon/Rhyhorn/Anims/Mount_Montage.Mount_Montage" 1.0 0.0 "laydown"
          (:`then`
            (`KismetSystemLibrary.Delay` 2.2)
            (`|PlayMontage` (`Character.Mesh` (`self.MainChar_0`)) "/Game/Test/MainCharacter/Male/Anims/Custom/Mounting/Rhyhorn/MountRhyhorn_Montage.MountRhyhorn_Montage" 1.0 0.0 "Sit"
              (:`then`
                (`self.K2_AttachToComponent` _mainchar_0_2 (`self.RiderLoaction`) "None" "SnapToTarget" "SnapToTarget" "KeepRelative" true)
                (`|ExecutionSequence`
                  (:`then_0`
                    (`|PlayMontage` (`self.Mesh`) "/Game/Test/Pokemon/Rhyhorn/Anims/Mount_Montage.Mount_Montage" 1.0 0.0 "standup"))
                  (:`then_1`
                    (`KismetSystemLibrary.Delay` 0.5)
                    (`/Game/AdvancedLocomotionV3/Blueprints/MannequinCharacter.ChangeToPokemon` _mainchar_0_2)
                    (set `/Game/AdvancedLocomotionV3/Blueprints/MannequinCharacter.IsCharacterMounted?` true _mainchar_0_2)))))))))))

(event `InputAction|Interact`
  (params (Key :type "Key Structure"))
  (bind _mainchar_0 (`self.MainChar_0`))
  (bind _mainchar_0_2 (`self.MainChar_0`))
  (:`Pressed`
    (if (`/Game/AdvancedLocomotionV3/Blueprints/MannequinCharacter.IsCharacterMounted?` _mainchar_0_2)
      (`self.SwitchToCharacter`)
      (`CharacterMovementComponent.SetMovementMode` (`Character.CharacterMovement` _mainchar_0) "MOVE_Falling" 0)
      (`self.K2_SetActorLocation` _mainchar_0 (`SceneComponent.K2_GetComponentLocation` (`self.GetDownLoacation`)) false false)
      (`PrimitiveComponent.SetCollisionEnabled` (`Character.CapsuleComponent` _mainchar_0) "QueryAndPhysics")
      (`self.K2_DetachFromActor` _mainchar_0 "KeepWorld" "KeepWorld" "KeepRelative")
      (`self.StopAnimMontage` _mainchar_0_2 "/Game/Test/MainCharacter/Male/Anims/Custom/Mounting/Rhyhorn/MountRhyhorn_Montage.MountRhyhorn_Montage")
      (set `/Game/AdvancedLocomotionV3/Blueprints/MannequinCharacter.IsCharacterMounted?` false (`self.MainChar_0`)))))

(fn `Interact`
  (returns (Result :type Boolean))
  (`self.Mount`)
  (return false))

(fn `UserConstructionScript`
  (`parent.UserConstructionScript`))