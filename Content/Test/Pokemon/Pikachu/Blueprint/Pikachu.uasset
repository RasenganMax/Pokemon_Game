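; Pikachu character Blueprint for a companion Pokémon that blinks via eye-texture swaps and can be attacked with.
; An overlap sphere shows an interact widget, and Interact either lets it down or runs a timed walk, jump and attach to the player's shoulder socket.
; Keys 1-3 trigger Swat, Iron Tail and Thunder Shock montages with camera-facing moves.
; Thunder Shock adds a beam and an unused trace; Tackle and Thunderbolt are empty.
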(event `self.ReceiveBeginPlay`
  (bind _mesh (`self.Mesh`))
  (`parent.ReceiveBeginPlay`)
  (bind _returnvalue (`PrimitiveComponent.CreateDynamicMaterialInstance` _mesh 3 (`PrimitiveComponent.GetMaterial` _mesh 3) "None"))
  (set `self.Eyes Material` _returnvalue)
  (`self.Blinking`)
  (bind _asmannequin_character (cast `/Game/AdvancedLocomotionV3/Blueprints/MannequinCharacter` (`GameplayStatics.GetPlayerCharacter` 0)))
  (set `self.MainCharacter` _asmannequin_character))

(event `Blinking`
  ;[1 1 1] Blinking
  (`MaterialInstanceDynamic.SetTextureParameterValue` (`self.Eyes Material`) "Eyes Texture" "/Game/Test/Pokemon/Pikachu/Textures/Normal/EyesClosed.EyesClosed" :!label _label)
  (`KismetSystemLibrary.Delay` 0.1)
  (`MaterialInstanceDynamic.SetTextureParameterValue` (`self.Eyes Material`) "Eyes Texture" "/Game/Test/Pokemon/Pikachu/Textures/Normal/pm0025_00_Eye1.pm0025_00_Eye1")
  (`KismetSystemLibrary.Delay` (`KismetMathLibrary.RandomFloatInRange` 1.0 3.5))
  (goto _label))

(event `Interaction`
  (bind (_returnvalue_roll _returnvalue_pitch _returnvalue_yaw) (`KismetMathLibrary.BreakRotator` (`self.K2_GetActorRotation`)))
  (bind (_returnvalue_roll_2 _returnvalue_pitch_2 _returnvalue_yaw_2) (`KismetMathLibrary.BreakRotator` (`KismetMathLibrary.FindLookAtRotation` (`self.K2_GetActorLocation`) (`self.K2_GetActorLocation` (`GameplayStatics.GetPlayerCharacter` 0)))))
  ;[1 1 1] Inteacting With Main
  (`MovementComponent.StopMovementImmediately` (`self.CharacterMovement`))
  (`SceneComponent.K2_SetWorldRotation` (`self.Mesh`) (`KismetMathLibrary.MakeRotator` 0.0 0.0 (- _returnvalue_yaw_2 90.0)) false false)
  (set `self.IsplayingAnim` true)
  (`KismetSystemLibrary.Delay` 2.042)
  (set `self.IsplayingAnim` false)
  (`self.SpawnDefaultController`)
  (set `CharacterMovementComponent.MaxWalkSpeed` (`self.WalkSpeed`) (`self.CharacterMovement`))
  (`SceneComponent.K2_SetWorldRotation` (`self.Mesh`) (`KismetMathLibrary.MakeRotator` 0.0 0.0 (+ _returnvalue_yaw -90.0)) false false))

(event `self.Sphere.OnComponentBeginOverlap`
  (params (OverlappedComponent :type "PrimitiveComponent Object Reference") (OtherActor :type "Actor Object Reference") (OtherComp :type "PrimitiveComponent Object Reference") (OtherBodyIndex :type Integer) (bFromSweep :type Boolean) (SweepResult :type "HitResult Structure (by ref)"))
  (bind _playerref (`self.PlayerRef`))
  ;[0.3496 1 0.6541] Icon Visibility
  (if (== OtherActor _playerref)
    (set `/Game/AdvancedLocomotionV3/Blueprints/ALS_BaseCharacter.Interact Actor` self _playerref)
    (`SceneComponent.SetVisibility` (`self.Widget`) true false)))

(event `self.Sphere.OnComponentEndOverlap`
  (params (OverlappedComponent :type "PrimitiveComponent Object Reference") (OtherActor :type "Actor Object Reference") (OtherComp :type "PrimitiveComponent Object Reference") (OtherBodyIndex :type Integer))
  (bind _playerref (`self.PlayerRef`))
  ;[0.3496 1 0.6541] Icon Visibility
  (if (== _playerref OtherActor)
    (set `/Game/AdvancedLocomotionV3/Blueprints/ALS_BaseCharacter.Interact Actor` null _playerref)
    (`SceneComponent.SetVisibility` (`self.Widget`) false false)))

(event `EquipToCharacter`
  (`|ExecutionSequence`
    (:`then_0`
      (`/Game/AdvancedLocomotionV3/Blueprints/MannequinCharacter.KneelingToPickUp` (`self.MainCharacter`)))
    (:`then_1`
      (`self.AttachPokemon`))))

(event `AttachPokemon`
  (bind _maincharacter (`self.MainCharacter`))
  (`KismetSystemLibrary.Delay` 2.767)
  (`AIBlueprintHelperLibrary.SimpleMoveToActor` (`AIBlueprintHelperLibrary.GetAIController` self) (`self.MainCharacter`))
  (`KismetSystemLibrary.Delay` 2.767)
  (`MovementComponent.StopMovementImmediately` (`self.CharacterMovement`))
  (`self.PlayAnimMontage` "/Game/Test/Pokemon/Pikachu/Anims/JumpingToShoulder_Montage.JumpingToShoulder_Montage" 1.0 "Jump")
  (`KismetSystemLibrary.Delay` 1.7)
  (`self.K2_AttachToComponent` (`/Game/AdvancedLocomotionV3/Blueprints/MannequinCharacter.EquipLocation` _maincharacter) "Shoulder" "SnapToTarget" "SnapToTarget" "KeepWorld" false)
  (`CharacterMovementComponent.DisableMovement` (`self.CharacterMovement`))
  (`PrimitiveComponent.SetCollisionEnabled` (`self.CapsuleComponent`) "NoCollision")
  (`/Game/AdvancedLocomotionV3/Blueprints/MannequinCharacter.StandingUp` _maincharacter)
  (set `/Game/AdvancedLocomotionV3/Blueprints/MannequinCharacter.PokemonEquipped` true (`self.MainCharacter`)))

(event `Key|Two`
  (params (Key :type "Key Structure"))
  (:`Pressed`
    (`self.iron_tail`)))

(event `Key|One`
  (params (Key :type "Key Structure"))
  (:`Pressed`
    (`self.swat`)))

(event `Key|Three`
  (params (Key :type "Key Structure"))
  (:`Pressed`
    (`self.thunder shock`)))

(event `swat`
  (bind _capsulecomponent (`self.CapsuleComponent`))
  (bind (_returnvalue_roll _returnvalue_pitch _returnvalue_yaw) (`KismetMathLibrary.BreakRotator` (`SceneComponent.K2_GetComponentRotation` (`self.FollowCamera`))))
  ;[1 1 1] swat
  (if (not (`self.ability in use`))
    (`ActorComponent.Deactivate` (`self.CharacterMovement`))
    (set `self.player is attacking` true)
    (set `self.ability in use` true)
    (`|PlayMontage` (`self.Mesh`) "/Game/Test/Pokemon/Pikachu/Anims/swat_montage.swat_montage" 0.8 0.0 "attack"
      (:`then`
        (`KismetSystemLibrary.MoveComponentTo` (`self.CapsuleComponent`) (+ (`SceneComponent.K2_GetComponentLocation` _capsulecomponent) (* (`SceneComponent.GetForwardVector` _capsulecomponent) 95.0)) (`KismetMathLibrary.MakeRotator` 0.0 0.0 _returnvalue_yaw) true true 0.5 true)
        (`KismetSystemLibrary.Delay` 1.0)
        (`ActorComponent.Activate` (`self.CharacterMovement`) false)))))

(event `iron_tail`
  (bind _capsulecomponent (`self.CapsuleComponent`))
  (bind (_returnvalue_roll _returnvalue_pitch _returnvalue_yaw) (`KismetMathLibrary.BreakRotator` (`SceneComponent.K2_GetComponentRotation` (`self.FollowCamera`))))
  ;[1 1 1] iron_tail
  (if (not (`self.ability in use`))
    (`ActorComponent.Deactivate` (`self.CharacterMovement`))
    (`PrimitiveComponent.SetMaterial` (`self.Mesh`) 4 "/Game/Test/Pokemon/Pikachu/Materials/e_tail.e_tail")
    (set `self.player is attacking` true)
    (set `self.ability in use` true)
    (`|PlayMontage` (`self.Mesh`) "/Game/Test/Pokemon/Pikachu/Anims/iron_tail_m.iron_tail_m" 0.8 0.0 "attack"
      (:`then`
        (`KismetSystemLibrary.MoveComponentTo` (`self.CapsuleComponent`) (+ (`SceneComponent.K2_GetComponentLocation` _capsulecomponent) (* (`SceneComponent.GetForwardVector` _capsulecomponent) 95.0)) (`KismetMathLibrary.MakeRotator` 0.0 0.0 _returnvalue_yaw) true true 0.5 true)
        (`KismetSystemLibrary.Delay` 1.0)
        (`PrimitiveComponent.SetMaterial` (`self.Mesh`) 4 "/Game/Test/Pokemon/Pikachu/Materials/pm0025_00_BodyA1_Mat.pm0025_00_BodyA1_Mat")
        (`ActorComponent.Activate` (`self.CharacterMovement`) false)))))

(event `thunder shock`
  (bind _capsulecomponent (`self.CapsuleComponent`))
  (bind (_returnvalue_roll _returnvalue_pitch _returnvalue_yaw) (`KismetMathLibrary.BreakRotator` (`SceneComponent.K2_GetComponentRotation` (`self.FollowCamera`))))
  (bind _returnvalue (`SceneComponent.GetForwardVector` (`self.FollowCamera`)))
  (bind _returnvalue_2 (`SceneComponent.K2_GetComponentLocation` (`self.Mesh`)))
  ;[1 1 1] thunder_shock
  (if (not (`self.ability in use`))
    (`ActorComponent.Deactivate` (`self.CharacterMovement`))
    (`|ExecutionSequence`
      (:`then_0`
        (set `self.player is attacking` true)
        (set `self.ability in use` true)
        (`|PlayMontage` (`self.Mesh`) "/Game/Test/Pokemon/Pikachu/Anims/thunder_shock.thunder_shock" 0.8 0.0 "attack"
          (:`then`
            (`KismetSystemLibrary.MoveComponentTo` (`self.CapsuleComponent`) (+ (`SceneComponent.K2_GetComponentLocation` _capsulecomponent) (* (`SceneComponent.GetForwardVector` _capsulecomponent) 0.0)) (`KismetMathLibrary.MakeRotator` 0.0 0.0 _returnvalue_yaw) true true 0.5 true))))
      (:`then_1`
        ;;[1 1 1] thunder_shock_emitter
        (`KismetSystemLibrary.Delay` 0.8)
        (`PrimitiveComponent.SetMaterial` (`self.Mesh`) 4 "/Game/Test/Pokemon/Pikachu/Materials/e_tail1.e_tail1")
        (bind _returnvalue_3 (`GameplayStatics.SpawnEmitterAtLocation` "/Game/ParticleEffects/BeamAndLaserFX01/Particles/P_ky_beam03.P_ky_beam03" (+ (+ (`SceneComponent.K2_GetComponentLocation` (`self.Mesh`)) (* _returnvalue 50.0)) (0.0 0.0 34.0)) (`KismetMathLibrary.MakeRotFromX` _returnvalue)))
        (`KismetSystemLibrary.Delay` 1.6)
        (`ActorComponent.K2_DestroyComponent` _returnvalue_3)
        (`PrimitiveComponent.SetMaterial` (`self.Mesh`) 4 "/Game/Test/Pokemon/Pikachu/Materials/pm0025_00_BodyA1_Mat.pm0025_00_BodyA1_Mat")
        (`ActorComponent.Activate` (`self.CharacterMovement`) false)
        (set `self.player is attacking` false)
        (set `self.ability in use` false))
      (:`then_2`
        ;;[1 1 1] apply damage with this traace
        (`KismetSystemLibrary.LineTraceMulti` _returnvalue_2 (+ (+ _returnvalue_2 (* (`SceneComponent.GetForwardVector` (`self.FollowCamera`)) 700.0)) (0.0 0.0 34.0)) "TraceTypeQuery2")
        (if (`self.ability in use`) :!label _label
          (`KismetSystemLibrary.Delay` 0.2)
          (goto _label))))))

(event `tackle`)

(event `thunder bolt`)

(fn `Interact`
  (returns (Result :type Boolean))
  (`/Engine/EditorBlueprintResources/StandardMacros.IsValid` (`/Game/AdvancedLocomotionV3/Blueprints/MannequinCharacter.PokemonRef` (`self.MainCharacter`))
    (:`Is Valid`
      (if (`/Game/AdvancedLocomotionV3/Blueprints/MannequinCharacter.PokemonEquipped` (`self.MainCharacter`))
        (`self.PokemonLetDown`)
        (else
          (`self.EquipToCharacter`)))
      (return false))))

(fn `UserConstructionScript`
  (`parent.UserConstructionScript`))