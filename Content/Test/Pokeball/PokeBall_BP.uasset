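; Thrown Pokeball actor that captures a BasePokemon and can be picked up to add it to the player's party.
; A valid hit plays a beam and material swap, then hides the Pokemon.
; The next non-Pokemon hit starts up to four random rolls between wiggles, one scaled by level and HP, with escape destroying the ball.
; Sphere overlap drives pickup, Tick can home the ball to the hand, and camera close-up code is disconnected.
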(event `self.ReceiveBeginPlay`
  ;[1 1 1] On Begin Play
  (bind _asmannequin_character (cast `/Game/AdvancedLocomotionV3/Blueprints/MannequinCharacter` (`self.GetOwner`)))
  (bind _output_get (set `self.MainCharRef` _asmannequin_character))
  (bind _asplayer_controller (cast `PlayerController` (`Pawn.GetController` _output_get)))
  (set `self.PlayerController` _asplayer_controller)
  (`PrimitiveComponent.SetAngularDamping` (`self.Pokeball`) 12.0))

(event `self.Pokeball.OnComponentHit`
  (params (HitComponent :type "PrimitiveComponent Object Reference") (OtherActor :type "Actor Object Reference") (OtherComp :type "PrimitiveComponent Object Reference") (NormalImpulse :type "Vector Structure") (Hit :type "HitResult Structure (by ref)"))
  (bind _pokemon (`self.Pokemon`))
  (bind _returnvalue (`SceneComponent.K2_GetComponentLocation` (`self.Pokeball`)))
  (bind _returnvalue_2 (`SkeletalMeshComponent.GetAnimInstance` (`self.Pokeball`)))
  (bind _returnvalue_3 (`self.K2_GetActorLocation` (`self.Pokemon`)))
  (bind _mesh (`Character.Mesh` (`self.Pokemon`)))
  (bind _returnvalue_4 (`SceneComponent.K2_GetComponentLocation` _mesh))
  (bind _returnvalue_5 (+ _returnvalue_3 (`KismetMathLibrary.MakeVector` (`self.Left/Right`) (`self.Forward`) (`self.Height`))))
  (`self.PlayHitSound` NormalImpulse)
  (`/Engine/EditorBlueprintResources/StandardMacros.IsValid` (`self.Pokemon`)
    (:`Is Valid`
      (cast `/Game/Test/Pokemon/BasePokemon` OtherActor
        (:`CastFailed`
          (`self.Capturing Pokemon`))))
    (:`Is Not Valid`
      (if (== (`/Game/AdvancedLocomotionV3/Blueprints/MannequinCharacter.CatchorLetOut` (`self.MainCharRef`)) 1)
        (bind _asbase_pokemon (cast `/Game/Test/Pokemon/BasePokemon` OtherActor)
          (:`then`
            (if (and (`self.CanCapture?`) (`/Game/AdvancedLocomotionV3/Blueprints/MannequinCharacter.CanAddPokemonToParty` (`self.MainCharRef`) _asbase_pokemon))
              (bind _output_get (set `self.Pokemon` _asbase_pokemon))
              (`CharacterMovementComponent.DisableMovement` (`Character.CharacterMovement` _output_get))
              (`PrimitiveComponent.SetSimulatePhysics` (`self.Pokeball`) false)
              ;[1 1 1] Pokeball Move To Location
              (`KismetSystemLibrary.MoveComponentTo` (`self.Pokeball`) _returnvalue_5 (`KismetMathLibrary.FindLookAtRotation` _returnvalue_5 _returnvalue_3) true true 0.35 true)
              ;[0.5276 0.8895 1] Play Open Anim
              (`AnimInstance.Montage_Play` _returnvalue_2 "/Game/Test/Pokeball/Animation/Pokeball_Montage.Pokeball_Montage" 1.0 "Duration" 0.0 true)
              (`AnimInstance.Montage_JumpToSection` _returnvalue_2 "Open" "/Game/Test/Pokeball/Animation/Pokeball_Montage.Pokeball_Montage")
              (`|ExecutionSequence`
                (:`then_0`
                  (bind _returnvalue_6 (`GameplayStatics.SpawnEmitterAtLocation` "/Game/ParticleEffects/BeamAndLaserFX01/Particles/CatchBeam.CatchBeam" _returnvalue (`KismetMathLibrary.FindLookAtRotation` _returnvalue _returnvalue_4) (0.4 1.0 1.0)))
                  (`ParticleSystemComponent.SetBeamTargetPoint` _returnvalue_6 1 _returnvalue_4 0))
                (:`then_1`
                  (`GameplayStatics.SpawnEmitterAttached` "/Game/ParticleEffects/AdvancedMagicFX11/Particles/P_ky_wind3.P_ky_wind3" _mesh "None" (0.0 0.0 5.0) (struct) (7.0 7.0 7.0) "SnapToTargetIncludingScale"))
                (:`then_2`
                  (for _index (range (`PrimitiveComponent.GetNumMaterials` (`Character.Mesh` (`self.Pokemon`))))
                    (`KismetArrayLibrary.Array_Set` (`self.DefaultPokemonMaterials`) _index (`PrimitiveComponent.GetMaterial` _mesh _index) true)
                    (`PrimitiveComponent.SetMaterial` _mesh _index "/Game/Test/Pokemon/Capture_Mat.Capture_Mat"))))
              (`KismetSystemLibrary.Delay` 1.2)
              (`ActorComponent.K2_DestroyComponent` _returnvalue_6)
              (for (_array_element _array_index) (`self.DefaultPokemonMaterials`)
                (`PrimitiveComponent.SetMaterial` _mesh _array_index _array_element))
              (`self.SetActorHiddenInGame` _pokemon true)
              (`self.SetActorEnableCollision` _pokemon false)
              (`PrimitiveComponent.SetSimulatePhysics` (`self.Pokeball`) true)))
          (:`CastFailed`
            (set `self.CanCapture?` false)
            (`KismetSystemLibrary.Delay` 2.0)
            (`SceneComponent.SetHiddenInGame` (`self.Widget`) false false)))))))

(event `Interacting`
  ;[1 1 1] Interact
  (`|ExecutionSequence`
    (:`then_0`
      (bind _asmannequin_character (cast `/Game/AdvancedLocomotionV3/Blueprints/MannequinCharacter` (`self.GetOwner`)))
      (set `self.MainCharRef` _asmannequin_character)
      (`SceneComponent.SetVisibility` (`self.Widget`) false false))
    (:`then_1`
      (`KismetSystemLibrary.K2_SetTimerDelegate` (delegate `Spin`) 0.1 true))))

(event `Capturing Pokemon`
  (bind _returnvalue (`self.K2_GetActorLocation`))
  (bind _pokeball (`self.Pokeball`))
  (bind _pokeball_2 (`self.Pokeball`))
  (bind _pokeball_3 (`self.Pokeball`))
  (bind _pokeball_4 (`self.Pokeball`))
  (bind _pokemon (`self.Pokemon`))
  (bind _pokemon_2 (`self.Pokemon`))
  (bind _pokeball_5 (`self.Pokeball`))
  (bind _pokemon_3 (`self.Pokemon`))
  (bind _pokemon_4 (`self.Pokemon`))
  (bind _pokeball_6 (`self.Pokeball`))
  (bind _scenecapturecomponent2d (`self.SceneCaptureComponent2D`))
  (bind _returnvalue_2 (`SkeletalMeshComponent.GetAnimInstance` _pokeball_5))
  (bind _returnvalue_3 (`SkeletalMeshComponent.GetAnimInstance` _pokeball_6))
  (bind _returnvalue_4 (`SceneComponent.K2_GetComponentLocation` _pokeball_3))
  (bind _returnvalue_5 (`SkeletalMeshComponent.GetAnimInstance` _pokeball))
  (bind _returnvalue_6 (`SkeletalMeshComponent.GetAnimInstance` _pokeball_4))
  ;[1 1 1] Catching Event
  (set `SceneCaptureComponent.bCaptureOnMovement` true _scenecapturecomponent2d)
  (set `SceneCaptureComponent.bCaptureEveryFrame` true _scenecapturecomponent2d)
  (`PrimitiveComponent.SetSimulatePhysics` _pokeball_2 false)
  (`KismetSystemLibrary.MoveComponentTo` _pokeball_2 _returnvalue (`KismetMathLibrary.FindLookAtRotation` _returnvalue (`PlayerCameraManager.GetCameraLocation` (`PlayerController.PlayerCameraManager` (`self.PlayerController`)))) true true 0.3 true)
  (if (> (`KismetMathLibrary.RandomIntegerInRange` 1 100) (`self.Chance`))
    (`PrimitiveComponent.SetCollisionEnabled` _pokeball_2 "NoCollision")
    (`PrimitiveComponent.SetCollisionEnabled` (`self.Sphere`) "NoCollision")
    ;;[1 1 1] Catching Pokemon
    ;;;[0.4973 1 0.4305] 1st Wiggle
    (`self.PokeballWiggle`)
    (`KismetSystemLibrary.Delay` 2.39)
    (if (> (`KismetMathLibrary.RandomIntegerInRange` 1 100) (`self.Chance`))
      ;;;[0.5935 1 0.4692] 2nd Wiggle
      (`self.PokeballWiggle`)
      (`KismetSystemLibrary.Delay` 2.39)
      (`self.chance_multiplier`)
      (if (== (`KismetMathLibrary.RandomIntegerInRange` (`self.chance_min`) (`self.chancee_max`)) (`self.Chance`))
        ;;;[0.6172 1 0.5609] 3rd Wiggle
        (`self.PokeballWiggle`)
        (`KismetSystemLibrary.Delay` 2.39)
        (if (> (`KismetMathLibrary.RandomIntegerInRange` 1 100) (`self.Chance`))
          ;;;[1 0.955 0.5374] Caught Pokemon
          (`|ExecutionSequence`
            (:`then_0`
              (`GameplayStatics.SpawnEmitterAtLocation` "/Game/ParticleEffects/AdvancedMagicFX15/Particles/PokmonCaptured.PokmonCaptured" _returnvalue_4))
            (:`then_1`
              (`GameplayStatics.PlaySoundAtLocation` "/Game/Test/Pokeball/Sounds/Pokémon_Caught__Gotcha__.Pokémon_Caught__Gotcha__" _returnvalue_4 (struct) 1.0 1.0 0.0 null null null)))
          (`PrimitiveComponent.SetMaterial` _pokeball_3 8 "/Game/Test/Pokeball/Materials/ButtonCaptured.ButtonCaptured")
          (`KismetSystemLibrary.Delay` 1.0)
          (`PrimitiveComponent.SetMaterial` _pokeball_3 8 "/Game/Test/Pokeball/Materials/Button.Button")
          (`PrimitiveComponent.SetCollisionEnabled` (`self.Pokeball`) "QueryAndPhysics")
          (`PrimitiveComponent.SetCollisionEnabled` (`self.Sphere`) "QueryAndPhysics")
          (`SceneComponent.SetHiddenInGame` (`self.Widget`) false false)
          (`KismetSystemLibrary.PrintString` "PokemonCaptured")
          (set `self.CanCapture?` false)
          (else
            ;;[1 0.7049 0.5103] Pokemon Escaped Pokeball Try 4
            (`KismetSystemLibrary.Delay` 0.2)
            (`PrimitiveComponent.SetSimulatePhysics` _pokeball false)
            (`AnimInstance.Montage_Play` _returnvalue_5 "/Game/Test/Pokeball/Animation/Pokeball_Montage.Pokeball_Montage" 1.0 "Duration" 0.0 true)
            (`AnimInstance.Montage_JumpToSection` _returnvalue_5 "OpenSpawn" "/Game/Test/Pokeball/Animation/Pokeball_Montage.Pokeball_Montage")
            (`KismetSystemLibrary.Delay` 0.5)
            (`self.SetActorHiddenInGame` _pokemon_3 false)
            (`self.SetActorEnableCollision` _pokemon_3 true)
            (`CharacterMovementComponent.SetMovementMode` (`Character.CharacterMovement` _pokemon_3) "MOVE_Walking" 0)
            (`self.SetLifeSpan` 0.1)
            (set `self.CanCapture?` true)))
        (else
          ;;[1 0.7049 0.5103] Pokemon Escaped Pokeball Try 3
          (`KismetSystemLibrary.Delay` 0.2)
          (`PrimitiveComponent.SetSimulatePhysics` _pokeball_6 false)
          (`AnimInstance.Montage_Play` _returnvalue_3 "/Game/Test/Pokeball/Animation/Pokeball_Montage.Pokeball_Montage" 1.0 "Duration" 0.0 true)
          (`AnimInstance.Montage_JumpToSection` _returnvalue_3 "OpenSpawn" "/Game/Test/Pokeball/Animation/Pokeball_Montage.Pokeball_Montage")
          (`KismetSystemLibrary.Delay` 0.5)
          (`self.SetActorHiddenInGame` _pokemon_2 false)
          (`self.SetActorEnableCollision` _pokemon_2 true)
          (`CharacterMovementComponent.SetMovementMode` (`Character.CharacterMovement` _pokemon_2) "MOVE_Walking" 0)
          (`self.SetLifeSpan` 0.1)
          (set `self.CanCapture?` true)))
      (else
        ;;[1 0.7049 0.5103] Pokemon Escaped Pokeball Try 2
        (`KismetSystemLibrary.Delay` 0.2)
        (`PrimitiveComponent.SetSimulatePhysics` _pokeball_5 false)
        (`AnimInstance.Montage_Play` _returnvalue_2 "/Game/Test/Pokeball/Animation/Pokeball_Montage.Pokeball_Montage" 1.0 "Duration" 0.0 true)
        (`AnimInstance.Montage_JumpToSection` _returnvalue_2 "OpenSpawn" "/Game/Test/Pokeball/Animation/Pokeball_Montage.Pokeball_Montage")
        (`KismetSystemLibrary.Delay` 0.5)
        (`self.SetActorHiddenInGame` _pokemon false)
        (`self.SetActorEnableCollision` _pokemon true)
        (`CharacterMovementComponent.SetMovementMode` (`Character.CharacterMovement` _pokemon) "MOVE_Walking" 0)
        (`self.SetLifeSpan` 0.1)
        (set `self.CanCapture?` true)))
    (else
      ;;[1 0.7049 0.5103] Pokemon Escaped Pokeball Try 1
      (`KismetSystemLibrary.Delay` 1.0)
      (`PrimitiveComponent.SetSimulatePhysics` _pokeball_4 false)
      (`AnimInstance.Montage_Play` _returnvalue_6 "/Game/Test/Pokeball/Animation/Pokeball_Montage.Pokeball_Montage" 1.0 "Duration" 0.0 true)
      (`AnimInstance.Montage_JumpToSection` _returnvalue_6 "OpenSpawn" "/Game/Test/Pokeball/Animation/Pokeball_Montage.Pokeball_Montage")
      (`KismetSystemLibrary.Delay` 0.5)
      (`self.SetActorHiddenInGame` _pokemon_4 false)
      (`self.SetActorEnableCollision` _pokemon_4 true)
      (`CharacterMovementComponent.SetMovementMode` (`Character.CharacterMovement` _pokemon_4) "MOVE_Walking" 0)
      (`self.SetLifeSpan` 0.1)
      (set `self.CanCapture?` true))))

(event `Spin`
  (bind _widget (`self.Widget`))
  (bind (_returnvalue_roll _returnvalue_pitch _returnvalue_yaw) (`KismetMathLibrary.BreakRotator` (`KismetMathLibrary.FindLookAtRotation` (`SceneComponent.K2_GetComponentLocation` _widget) (`SceneComponent.K2_GetComponentLocation` (`/Game/AdvancedLocomotionV3/Blueprints/ALS_BaseCharacter.TP_Camera` (`self.MainCharRef`))))))
  ;[1 1 1] Interact
  (`SceneComponent.K2_SetWorldRotation` _widget (`KismetMathLibrary.MakeRotator` 0.0 10.0 _returnvalue_yaw) false false))

(event `self.Sphere.OnComponentBeginOverlap`
  (params (OverlappedComponent :type "PrimitiveComponent Object Reference") (OtherActor :type "Actor Object Reference") (OtherComp :type "PrimitiveComponent Object Reference") (OtherBodyIndex :type Integer) (bFromSweep :type Boolean) (SweepResult :type "HitResult Structure (by ref)"))
  (bind _maincharref (`self.MainCharRef`))
  ;[1 1 1] Interact
  ;;[0.6032 1 0.5318] Icon Visibility
  (if (== OtherActor _maincharref)
    (set `/Game/AdvancedLocomotionV3/Blueprints/ALS_BaseCharacter.Interact Actor` self _maincharref)
    (`SceneComponent.SetVisibility` (`self.Widget`) true false)))

(event `self.Sphere.OnComponentEndOverlap`
  (params (OverlappedComponent :type "PrimitiveComponent Object Reference") (OtherActor :type "Actor Object Reference") (OtherComp :type "PrimitiveComponent Object Reference") (OtherBodyIndex :type Integer))
  (bind _maincharref (`self.MainCharRef`))
  ;[1 1 1] Interact
  ;;[0.6032 1 0.5318] Icon Visibility
  (if (== _maincharref OtherActor)
    (set `/Game/AdvancedLocomotionV3/Blueprints/ALS_BaseCharacter.Interact Actor` null _maincharref)
    (`SceneComponent.SetVisibility` (`self.Widget`) false false)))

(event `self.ReceiveTick`
  (params (DeltaSeconds :type "Float (single-precision)"))
  (bind _maincharref (`self.MainCharRef`))
  (bind _returnvalue (`SceneComponent.GetSocketLocation` (`Character.Mesh` _maincharref) "Hand_R"))
  (bind _returnvalue_2 (`KismetMathLibrary.VInterpTo_Constant` (`self.K2_GetActorLocation`) _returnvalue DeltaSeconds 1000.0))
  ;[1 1 1] Catching Pokeball From Spawn
  (if (`self.IsMovingToHand?`)
    (`self.K2_SetActorLocation` _returnvalue_2 true)
    (`self.SetActorEnableCollision` false)
    (if (== _returnvalue_2 _returnvalue :`ErrorTolerance` 0.1)
      (`/Game/AdvancedLocomotionV3/Blueprints/MannequinCharacter.PokeballCaught` _maincharref))))

(fn `chance_multiplier`
  (bind _pokemon (`self.Pokemon`))
  (bind (_pokemon_type _pokemon_type2 _pokemon_image _pokemon_class _pokemon_speed _pokemon_hp _pokemonatk1_dmg _pokemonatk2_dmg _pokemonatk3_dmg _pokemonatk4_dmg _pokemonatk_vfx _pokemonatk_sfx _pokemon_number _pokemon_index _pokemon_level _pokemoncurrent_xp _pokmonneeded_xp _pokemon_name _captured_ _maxhp) (break `/Game/Test/Details/PokeDetails_St` (`/Game/Test/Pokemon/BasePokemon.PokemonDetails` _pokemon)))
  (`/Engine/EditorBlueprintResources/StandardMacros.IsValid` _pokemon
    (:`Is Valid`
      (bind _output_get (set `self.chancee_max` (* _pokemon_level (`self.chancee_max`))))
      (`KismetSystemLibrary.PrintString` (`KismetStringLibrary.Conv_IntToString` _output_get) true true (struct :`R` 1.0 :`G` 0.240347 :`A` 1.0))
      (if (< (/ _pokemon_hp _maxhp) 0.3)
        (bind _output_get_2 (set `self.chancee_max` (/ (`self.chancee_max`) _pokemon_level)))
        (`KismetSystemLibrary.PrintString` (`KismetStringLibrary.Conv_IntToString` _output_get_2))))))

(fn `CreatePokeCaptureWidget`
  (bind _returnvalue (`|CreateWidget` "/Game/Test/UI/PokemonCapture_Wid/PokeBallCapture_Wid.PokeBallCapture_Wid_C"))
  (bind _output_get (set `self.PokeballCapture_Wid` _returnvalue))
  (`UserWidget.AddToViewport` _output_get 0)
  (`Widget.SetVisibility` _output_get "Visible"))

(fn `Interact`
  (returns (Result :type Boolean))
  (bind _maincharref (`self.MainCharRef`))
  (`/Game/AdvancedLocomotionV3/Blueprints/MannequinCharacter.PickUpAnim` _maincharref)
  (`/Game/AdvancedLocomotionV3/Blueprints/MannequinCharacter.AddPokemonToParty` _maincharref (`self.Pokemon`))
  (`self.SetLifeSpan` 1.25)
  (return false))

(fn `PlayHitSound`
  (params (ImpactStrength :type "Vector Structure"))
  (bind _audio (`self.Audio`))
  (if (and (not (`AudioComponent.IsPlaying` (`self.Audio`))) (> (`KismetMathLibrary.VSize` ImpactStrength) 20.0))
    (`AudioComponent.SetSound` _audio "/Game/Test/Pokeball/Sounds/PokeballBounce.PokeballBounce")
    (`AudioComponent.Play` _audio 0.0)))

(fn `PokeballWiggle`
  (bind _pokeball (`self.Pokeball`))
  (bind _returnvalue (`SkeletalMeshComponent.GetAnimInstance` _pokeball))
  (`|ExecutionSequence`
    (:`then_0`
      (`AnimInstance.Montage_Play` _returnvalue "/Game/Test/Pokeball/Animation/Pokeball_Montage.Pokeball_Montage" 1.0 "Duration" 0.0 true)
      (`AnimInstance.Montage_JumpToSection` _returnvalue "Catching" "/Game/Test/Pokeball/Animation/Pokeball_Montage.Pokeball_Montage")
      (`PrimitiveComponent.SetMaterial` _pokeball 8 "/Game/Test/Pokeball/Materials/ButtonW.ButtonW"))
    (:`then_1`
      (`GameplayStatics.PlaySoundAtLocation` "/Game/Test/Pokeball/Sounds/Pokéball_Wiggle.Pokéball_Wiggle" (`SceneComponent.K2_GetComponentLocation` _pokeball) (struct) 2.0 1.0 0.0 null null null))))

(fn `UserConstructionScript`)