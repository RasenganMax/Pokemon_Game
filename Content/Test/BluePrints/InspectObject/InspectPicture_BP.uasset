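; Inspectable picture actor that the player can pull up to the camera, rotate and read about.
; Box overlap registers it as the player's InteractActor, while timelines show its prompt widget at close range and yaw it toward the camera.
; Interact attaches it to the camera manager, eases it into view, switches input to the actor, enables post-process depth blur and opens a details widget.
; Pressing Interact again restores transform, input, HUD and focus.
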(event `self.ReceiveBeginPlay`
  (bind _asals_base_character (cast `/Game/AdvancedLocomotionV3/Blueprints/ALS_BaseCharacter` (`GameplayStatics.GetPlayerCharacter` 0)))
  (set `self.PlayerRef` _asals_base_character)
  (bind _asmannequin_character (cast `/Game/AdvancedLocomotionV3/Blueprints/MannequinCharacter` (`GameplayStatics.GetPlayerCharacter` 0)))
  (set `self.MainChar` _asmannequin_character)
  (`self.Widget Distance`)
  (`self.Widget Rotation`))

(event `self.Box.OnComponentBeginOverlap`
  (params (OverlappedComponent :type "PrimitiveComponent Object Reference") (OtherActor :type "Actor Object Reference") (OtherComp :type "PrimitiveComponent Object Reference") (OtherBodyIndex :type Integer) (bFromSweep :type Boolean) (SweepResult :type "HitResult Structure (by ref)"))
  (bind _playerref (`self.PlayerRef`))
  ;[1 1 1] Sphere Overlap
  (if (== OtherActor _playerref)
    (set `/Game/AdvancedLocomotionV3/Blueprints/ALS_BaseCharacter.Interact Actor` self _playerref)))

(event `Widget Rotation`
  (bind (_returnvalue_roll _returnvalue_pitch _returnvalue_yaw) (`KismetMathLibrary.BreakRotator` (`KismetMathLibrary.FindLookAtRotation` (`self.K2_GetActorLocation`) (`SceneComponent.K2_GetComponentLocation` (`/Game/AdvancedLocomotionV3/Blueprints/ALS_BaseCharacter.TP_Camera` (`self.PlayerRef`))))))
  ;[1 1 1] Widget Rotation
  (`Timeline|Timeline_1`
    (:`Update`
      (`SceneComponent.K2_SetWorldRotation` (`self.Widget1`) (`KismetMathLibrary.MakeRotator` 0.0 0.0 _returnvalue_yaw) true false))))

(event `Widget Distance`
  (bind _widget1 (`self.Widget1`))
  ;[1 1 1] Distance From Player For Widget Visibility
  (`Timeline|Timeline_0`
    (:`Update`
      (if (< (`KismetMathLibrary.VSize` (- (`self.K2_GetActorLocation`) (`self.K2_GetActorLocation` (`GameplayStatics.GetPlayerCharacter` 0)))) 100.0)
        (`SceneComponent.SetVisibility` _widget1 true false)
        (else
          (`SceneComponent.SetVisibility` _widget1 false false))))))

(event `self.Box.OnComponentEndOverlap`
  (params (OverlappedComponent :type "PrimitiveComponent Object Reference") (OtherActor :type "Actor Object Reference") (OtherComp :type "PrimitiveComponent Object Reference") (OtherBodyIndex :type Integer))
  (bind _playerref (`self.PlayerRef`))
  ;[1 1 1] Sphere Overlap
  (if (== OtherActor _playerref)
    (set `/Game/AdvancedLocomotionV3/Blueprints/ALS_BaseCharacter.Interact Actor` null _playerref)))

(event `Inspect`
  (bind (_returnvalue_location _returnvalue_rotation) (`KismetMathLibrary.BreakTransform` (`self.GetTransform`)))
  (bind _defaultsceneroot (`self.DefaultSceneRoot`))
  (set `self.Original Loc` _returnvalue_location)
  (set `self.Original Rot` _returnvalue_rotation)
  (`SceneComponent.SetHiddenInGame` (`self.Widget1`) true false)
  (`Widget.SetVisibility` (`/Game/AdvancedLocomotionV3/Blueprints/MannequinCharacter.MasterHUD` (`self.MainChar`)) "Hidden")
  (`PrimitiveComponent.SetCollisionEnabled` (`self.StaticMesh`) "NoCollision")
  (`self.DisableInput` (`self.PlayerRef`) (`GameplayStatics.GetPlayerController` 0))
  (`self.K2_AttachToComponent` self (`PlayerCameraManager.TransformComponent` (`GameplayStatics.GetPlayerCameraManager` 0)) "None" "KeepWorld" "KeepWorld" "KeepWorld" true)
  (`KismetSystemLibrary.MoveComponentTo` _defaultsceneroot (25.0 0.0 -5.0) (`SceneComponent.RelativeRotation` _defaultsceneroot) true true 0.5)
  (set `PlayerController.bShowMouseCursor` true (`GameplayStatics.GetPlayerController` 0))
  (`self.EnableInput` (`GameplayStatics.GetPlayerController` 0))
  (`self.ToggleDOF` true)
  (`self.ObjectDetails` true))

(event `InputAction|Interact`
  (params (Key :type "Key Structure"))
  (:`Pressed`
    (`self.K2_DetachFromActor` self "KeepWorld" "KeepWorld" "KeepWorld")
    (`KismetSystemLibrary.MoveComponentTo` (`self.DefaultSceneRoot`) (`self.Original Loc`) (`self.Original Rot`) true true 0.5 true)
    (`PrimitiveComponent.SetCollisionEnabled` (`self.StaticMesh`) "QueryAndPhysics")
    (`self.DisableInput` (`GameplayStatics.GetPlayerController` 0))
    (`self.EnableInput` (`self.PlayerRef`) (`GameplayStatics.GetPlayerController` 0))
    (`Widget.SetVisibility` (`/Game/AdvancedLocomotionV3/Blueprints/MannequinCharacter.MasterHUD` (`self.MainChar`)) "Visible")
    (`self.ToggleDOF` false)
    (`self.ObjectDetails` false)
    (`SceneComponent.SetHiddenInGame` (`self.Widget1`) false false)
    (set `PlayerController.bShowMouseCursor` false (`GameplayStatics.GetPlayerController` 0))))

(event `InputAxis|LookUp/Down`
  (params (AxisValue :type "Float (single-precision)"))
  (`SceneComponent.K2_AddLocalRotation` (`self.DefaultSceneRoot`) (`KismetMathLibrary.MakeRotator` AxisValue) false false))

(event `InputAxis|LookLeft/Right`
  (params (AxisValue :type "Float (single-precision)"))
  (`SceneComponent.K2_AddLocalRotation` (`self.DefaultSceneRoot`) (`KismetMathLibrary.MakeRotator` 0.0 0.0 AxisValue) false false))

(fn `Interact`
  (returns (Result :type Boolean))
  (`self.Inspect`)
  (return false))

(fn `ObjectDetails`
  (params (`Enable/Disable` :type Boolean))
  (bind _inspectwidget (`self.InspectWidget`))
  (if `Enable/Disable`
    (`/Engine/EditorBlueprintResources/StandardMacros.IsValid` _inspectwidget
      (:`Is Valid`
        _)
      (:`Is Not Valid`
        (bind _returnvalue (`|CreateWidget` "/Game/Test/BluePrints/InspectObject/InspectableObject2_Widget.InspectableObject2_Widget_C" (`GameplayStatics.GetPlayerController` 0)))
        (bind _output_get (set `self.InspectWidget` _returnvalue))))
    (`/Game/Test/BluePrints/InspectObject/InspectableObject2_Widget.InspectionDetails` _output_get (`self.ObjectName`) (`self.ObjectInfo`))
    (`UserWidget.AddToViewport` _output_get 0)
    (else
      (`/Engine/EditorBlueprintResources/StandardMacros.IsValid` _inspectwidget
        (:`Is Valid`
          (`Widget.RemoveFromParent` _inspectwidget))))))

(fn `ToggleDOF`
  (params (`Enable/Disable` :type Boolean))
  (bind _postprocess_vol (`self.PostProcess_vol`))
  (bind _settings (`PostProcessVolume.Settings` _postprocess_vol))
  (if `Enable/Disable`
    (bind _structout (setmembers `PostProcessSettings` :`StructRef` _settings :`ColorGain` (1.0 1.0 1.0 1.0) :`DepthOfFieldFocalDistance` 30.0 :`DepthOfFieldDepthBlurAmount` 0.03 :`DepthOfFieldDepthBlurRadius` 100.0))
    (set `PostProcessVolume.Settings` _structout _postprocess_vol)
    (else
      (bind _structout_2 (setmembers `PostProcessSettings` :`StructRef` _settings :`ColorGain` (1.0 1.0 1.0 1.0) :`DepthOfFieldFocalDistance` 0.0 :`DepthOfFieldDepthBlurAmount` 1.0 :`DepthOfFieldDepthBlurRadius` 0.0))
      (set `PostProcessVolume.Settings` _structout_2 _postprocess_vol))))

(fn `UserConstructionScript`)