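; Test spawner actor that populates the bounds of its Spawn component with Charmander actors.
; BeginPlay spawns SpawnAmount of them, then starts a looping SpawnTimer that calls Re-Spawn.
; SpawnPokemon traces down from random raised points against WorldStatic, spawns at the hit location and records each in ActivePawns.
; Re-Spawn adds one whenever that array is below SpawnAmount; nothing here removes entries.
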(event `self.ReceiveBeginPlay`
  (for _ (range 1 (+ (`self.SpawnAmount`) 1))
    (`self.SpawnPokemon`))
  (`KismetSystemLibrary.K2_SetTimer` null "Re-Spawn" (`self.SpawnTimer`) true))

(fn `Re-Spawn`
  (if (< (`KismetArrayLibrary.Array_Length` (`self.ActivePawns`)) (`self.SpawnAmount`))
    (`self.SpawnPokemon`)))

(fn `SpawnPokemon`
  (bind (_origin _boxextent) (`KismetSystemLibrary.GetComponentBounds` (`self.Spawn`)))
  (bind _returnvalue (`KismetMathLibrary.MakeVector` (.x (`KismetMathLibrary.RandomPointInBoundingBox` _origin _boxextent)) (.y (`KismetMathLibrary.RandomPointInBoundingBox` _origin _boxextent)) (+ (.z (`KismetMathLibrary.RandomPointInBoundingBox` _origin _boxextent)) 600.0)))
  (bind _outhit (`KismetSystemLibrary.LineTraceSingleForObjects` _returnvalue (+ _returnvalue (* (* (`self.GetActorUpVector`) -1) 1200.0)) (`|MakeArray` "ObjectTypeQuery1" :!type "EObjectTypeQuery Enum")))
  (bind _returnvalue_2 (`|SpawnActorFromClass` "/Game/Test/Pokemon/Charmander/Blueprint/Charmander.Charmander_C" (`KismetMathLibrary.MakeTransform` (`KismetMathLibrary.MakeVector` (.x (`.Location` (`GameplayStatics.BreakHitResult` _outhit))) (.y (`.Location` (`GameplayStatics.BreakHitResult` _outhit))) (+ (.z (`.Location` (`GameplayStatics.BreakHitResult` _outhit))) 0.0)) (`KismetMathLibrary.MakeRotator` 0.0 0.0 (`KismetMathLibrary.RandomFloat`))) "AdjustIfPossibleButAlwaysSpawn" "OverrideRootScale" null null))
  (`KismetArrayLibrary.Array_Add` (`self.ActivePawns`) _returnvalue_2))

(fn `UserConstructionScript`)