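; Inspectable spot actor that shows a named object's details to the player on interaction.
; Entering the Sphere reveals a marker widget, which a timeline turns toward the player's third-person camera.
; Interaction flip-flops between a lazily created, reused details widget and the master HUD.
; Leaving the Sphere closes the details without resetting the flip-flop; Box overlaps only cast and do nothing further.
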(event `self.ReceiveBeginPlay`
  (bind _asmannequin_character (cast `/Game/AdvancedLocomotionV3/Blueprints/MannequinCharacter` (`GameplayStatics.GetPlayerCharacter` 0)))
  (set `self.MainChar` _asmannequin_character))

(event `self.ReceiveTick`
  (params (DeltaSeconds :type "Float (single-precision)")))

(event `self.Box.OnComponentBeginOverlap`
  (params (OverlappedComponent :type "PrimitiveComponent Object Reference") (OtherActor :type "Actor Object Reference") (OtherComp :type "PrimitiveComponent Object Reference") (OtherBodyIndex :type Integer) (bFromSweep :type Boolean) (SweepResult :type "HitResult Structure (by ref)"))
  ;[1 1 1] Sphere Overlap
  (cast `/Game/AdvancedLocomotionV3/Blueprints/MannequinCharacter` OtherActor))

(event `Widget Rotation`
  (bind (_returnvalue_roll _returnvalue_pitch _returnvalue_yaw) (`KismetMathLibrary.BreakRotator` (`KismetMathLibrary.FindLookAtRotation` (`self.K2_GetActorLocation`) (`SceneComponent.K2_GetComponentLocation` (`/Game/AdvancedLocomotionV3/Blueprints/ALS_BaseCharacter.TP_Camera` (`self.MainChar`))))))
  ;[1 0.7962 0.4576] Widget Rotation
  (`Timeline|Timeline_1`
    (:`Update`
      (`SceneComponent.K2_SetWorldRotation` (`self.Inspect_Wid`) (`KismetMathLibrary.MakeRotator` 0.0 _returnvalue_pitch _returnvalue_yaw) true false))))

(event `self.Sphere.OnComponentBeginOverlap`
  (params (OverlappedComponent :type "PrimitiveComponent Object Reference") (OtherActor :type "Actor Object Reference") (OtherComp :type "PrimitiveComponent Object Reference") (OtherBodyIndex :type Integer) (bFromSweep :type Boolean) (SweepResult :type "HitResult Structure (by ref)"))
  ;[1 1 1] Distance From Player For Widget Visibility
  (cast `/Game/AdvancedLocomotionV3/Blueprints/MannequinCharacter` OtherActor)
  (`SceneComponent.SetVisibility` (`self.Inspect_Wid`) true false)
  (`self.Widget Rotation`))

(event `self.Box.OnComponentEndOverlap`
  (params (OverlappedComponent :type "PrimitiveComponent Object Reference") (OtherActor :type "Actor Object Reference") (OtherComp :type "PrimitiveComponent Object Reference") (OtherBodyIndex :type Integer))
  ;[1 1 1] Sphere Overlap
  (cast `/Game/AdvancedLocomotionV3/Blueprints/MannequinCharacter` OtherActor))

(event `self.Sphere.OnComponentEndOverlap`
  (params (OverlappedComponent :type "PrimitiveComponent Object Reference") (OtherActor :type "Actor Object Reference") (OtherComp :type "PrimitiveComponent Object Reference") (OtherBodyIndex :type Integer))
  ;[1 1 1] Distance From Player For Widget Visibility
  (cast `/Game/AdvancedLocomotionV3/Blueprints/MannequinCharacter` OtherActor)
  (`Widget.SetVisibility` (`/Game/AdvancedLocomotionV3/Blueprints/MannequinCharacter.MasterHUD` (`self.MainChar`)) "Visible")
  (`self.SpotDetails` false)
  (`SceneComponent.SetVisibility` (`self.Inspect_Wid`) false false))

(event `InspectSpot`
  ;[1 1 1] Interaction
  (`SceneComponent.SetVisibility` (`self.Inspect_Wid`) false false)
  (`Widget.SetVisibility` (`/Game/AdvancedLocomotionV3/Blueprints/MannequinCharacter.MasterHUD` (`self.MainChar`)) "Hidden")
  (`self.SpotDetails` true))

(event `/Game/Test/BluePrints/Interact/Interact_Interface.Interaction`
  (`/Engine/EditorBlueprintResources/StandardMacros.FlipFlop`
    (:`A`
      (`self.InspectSpot`))
    (:`B`
      (`self.SpotDetails` false)
      (`Widget.SetVisibility` (`/Game/AdvancedLocomotionV3/Blueprints/MannequinCharacter.MasterHUD` (`self.MainChar`)) "Visible"))))

(fn `SpotDetails`
  (params (`Enable/Disable` :type Boolean))
  (bind _widget (`self.widget`))
  (bind _widget_2 (`self.widget`))
  (if `Enable/Disable`
    (`/Engine/EditorBlueprintResources/StandardMacros.IsValid` _widget_2
      (:`Is Valid`
        _)
      (:`Is Not Valid`
        (bind _returnvalue (`|CreateWidget` "/Game/Test/BluePrints/InspectSpot/InspectableSpot_Widget.InspectableSpot_Widget_C" (`GameplayStatics.GetPlayerController` 0)))
        (set `self.widget` _returnvalue)))
    (`/Game/Test/BluePrints/InspectSpot/InspectableSpot_Widget.InspectionDetails` _widget (`self.ObjectName`) (`self.ObjectInfo`))
    (`UserWidget.AddToViewport` _widget 0)
    (else
      (`/Engine/EditorBlueprintResources/StandardMacros.IsValid` _widget_2
        (:`Is Valid`
          (`Widget.RemoveFromParent` _widget_2))))))

(fn `UserConstructionScript`)