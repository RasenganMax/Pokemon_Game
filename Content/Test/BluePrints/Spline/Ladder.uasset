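; Ladder actor that builds itself from a Height and crossbar gap and notifies actors entering its trigger.
; InitiLadder runs at construction and BeginPlay, placing LadderTop, then stretching and centering both side bars and the LadderStart volume to that height.
; It refills an instanced static mesh with evenly spaced rungs.
; LadderStart overlaps send SetLadderMessage to the other actor, passing the ladder on entry and nothing on exit.
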(event `self.ReceiveBeginPlay`
  (`self.Initi Ladder`))

(event `Initi Ladder`
  (bind _ism_crossbar (`self.ISM_CrossBar`))
  (bind _temp_height (`self.Temp_Height`))
  (bind (_relativelocation_x _relativelocation_y _relativelocation_z) (`KismetMathLibrary.BreakVector` (`SceneComponent.RelativeLocation` (`self.LadderTop`))))
  (`SceneComponent.K2_SetRelativeLocation` (`self.LadderTop`) (`KismetMathLibrary.MakeVector` 0.0 0.0 (`self.Height`)) false false)
  (`self.AdjustSideBar` (`self.Ladder_L`))
  (`self.AdjustSideBar` (`self.Ladder_R`))
  (`self.AdjustSideBar` (`self.LadderStart`))
  (set `self.Temp_Height` 0.0)
  (`InstancedStaticMeshComponent.ClearInstances` _ism_crossbar)
  (while (< _temp_height _relativelocation_z)
    (`InstancedStaticMeshComponent.AddInstance` _ism_crossbar (`KismetMathLibrary.MakeTransform` (`KismetMathLibrary.MakeVector` 0.0 0.0 _temp_height) (struct) (0.05 0.6 0.05)))
    (set `self.Temp_Height` (+ _temp_height (`self.CrossBar_Gap`)))))

(event `self.LadderStart.OnComponentBeginOverlap`
  (params (OverlappedComponent :type "PrimitiveComponent Object Reference") (OtherActor :type "Actor Object Reference") (OtherComp :type "PrimitiveComponent Object Reference") (OtherBodyIndex :type Integer) (bFromSweep :type Boolean) (SweepResult :type "HitResult Structure (by ref)"))
  (message `/Game/Test/BluePrints/InterFace/Ladder_BPI.SetLadder` OtherActor self))

(event `self.LadderStart.OnComponentEndOverlap`
  (params (OverlappedComponent :type "PrimitiveComponent Object Reference") (OtherActor :type "Actor Object Reference") (OtherComp :type "PrimitiveComponent Object Reference") (OtherBodyIndex :type Integer))
  (message `/Game/Test/BluePrints/InterFace/Ladder_BPI.SetLadder` OtherActor null))

(fn `UserConstructionScript`
  (`self.Initi Ladder`))