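; BP_ky_beam12 is a beam effect Blueprint that exposes color controls for its Fx component.
; The construction script passes SpiralColor to the "colorDeco" effect parameter.
; It also creates a dynamic material instance on element 1 and sets its highlight and sub colors from HilightColor and SubColor.
; The event graph holds only disabled stub events, so the Blueprint runs no gameplay logic.
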(fn `UserConstructionScript`
  (`parent.UserConstructionScript`)
  ;[1 1 1] setting spiral color
  (`ParticleSystemComponent.SetVectorParameter` (`self.fx`) "colorDeco" (`KismetMathLibrary.Conv_LinearColorToVector` (`self.spiralColor`)))
  ;[1 1 1] get effect material instance
  (bind _returnvalue (`PrimitiveComponent.CreateDynamicMaterialInstance` (`self.fx`) 1 null "None"))
  ;[1 1 1] setting hilight color
  (`MaterialInstanceDynamic.SetVectorParameterValue` _returnvalue "hilightColor" (`self.hilightColor`))
  ;[1 1 1] setting sub color
  (`MaterialInstanceDynamic.SetVectorParameterValue` _returnvalue "subColor" (`self.subColor`)))