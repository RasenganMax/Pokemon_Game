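; Scene capture cube actor that defines a reflection box for volumetric glass materials on selected static mesh actors.
; The construction script sizes the box component from the reflection extent and passes a hidden-actor list to the cube capture.
; It creates dynamic instances of materials based on M_GlassShape on the affected meshes and writes the box's location and extent into them.
; All setup happens at construction, with no runtime event logic.
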(fn `UserConstructionScript`
  (set `self.ReflectionBoxLocation` (`self.K2_GetActorLocation`))
  (`BoxComponent.SetBoxExtent` (`self.Box`) (`self.ReflectionBoxExtend`) true)
  (`SceneComponent.SetWorldScale3D` (`self.Box`) (1.0 1.0 1.0))
  (set `SceneCaptureComponent.HiddenActors` (`self.HiddenActors`) (`self.CaptureComponentCube`))
  (for _array_element (`self.AffectedStaticMeshes`)
    (`/Engine/EditorBlueprintResources/StandardMacros.IsValid` _array_element
      (:`Is Valid`
        (bind _staticmeshcomponent (`StaticMeshActor.StaticMeshComponent` _array_element))
        (`/Engine/EditorBlueprintResources/StandardMacros.IsValid` _staticmeshcomponent
          (:`Is Valid`
            (for (_array_element_2 _array_index) (`MeshComponent.GetMaterials` _staticmeshcomponent)
              (bind _returnvalue (`MaterialInterface.GetBaseMaterial` _array_element_2))
              (if (== _returnvalue "/Game/Materials/VolumetricGlass/Materials/M_GlassShape.M_GlassShape")
                (bind _returnvalue_2 (`PrimitiveComponent.CreateDynamicMaterialInstance` _staticmeshcomponent _array_index _array_element_2 "None"))
                (`MaterialInstanceDynamic.SetVectorParameterValue` _returnvalue_2 "ReflectionBoxExtend" (`KismetMathLibrary.Conv_VectorToLinearColor` (`self.ReflectionBoxExtend`)))
                (`MaterialInstanceDynamic.SetVectorParameterValue` _returnvalue_2 "ReflectionBoxLocation" (`KismetMathLibrary.Conv_VectorToLinearColor` (`self.ReflectionBoxLocation`)))))))))))