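; Short-lived physics debris actor for the tree creator, flung out with a given impulse and removed after it settles.
; Construction applies the supplied mesh and damping, enables physics, and copies the source material's parameters onto a dynamic TreeDebris_M instance so it can fade.
; BeginPlay adds linear and random angular impulses, then after a delay turns off physics and collision responses to save performance.
; A later timeline drives the material's Fade parameter, then destroys the actor.
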(event `self.ReceiveBeginPlay`
  ;[0 0 0] Add initial impulses for the mesh. After X seconds, stop simulating physics to minimize performance hit. After another delay, fade out the mesh by smoothly adjusting dither material parameter.
  (`KismetSystemLibrary.Delay` 0.1)
  (`PrimitiveComponent.AddImpulse` (`self.StaticMesh`) (`self.initialImpulse`) "None" true)
  (`PrimitiveComponent.AddAngularImpulseInRadians` (`self.StaticMesh`) (`KismetMathLibrary.RandomUnitVector`) "None" true)
  (`KismetSystemLibrary.Delay` 5.0)
  (`PrimitiveComponent.SetSimulatePhysics` (`self.StaticMesh`) false)
  (`PrimitiveComponent.SetCollisionResponseToAllChannels` (`self.StaticMesh`) "ECR_Ignore")
  (`KismetSystemLibrary.Delay` 10.0)
  (bind (_direction _fade) (`Timeline|FadeOut` :!via `PlayFromStart`)
    (:`Update`
      (`MaterialInstanceDynamic.SetScalarParameterValue` (`self.dynMaterial`) "Fade" (* _fade 100.0)))
    (:`Finished`
      (`self.K2_DestroyActor`))))

(fn `UserConstructionScript`
  ;[0.005 0.005 0.005] Assign all the parameters for debris and turn on physics simulation.
  (`StaticMeshComponent.SetStaticMesh` (`self.StaticMesh`) (`self.Mesh`))
  (bind _returnvalue (`KismetMaterialLibrary.CreateDynamicMaterialInstance` "/Game/Landscape/InTreeCreator/Materials/Misc/TreeDebris_M.TreeDebris_M"))
  (set `self.dynMaterial` _returnvalue)
  (`MaterialInstanceDynamic.K2_CopyMaterialInstanceParameters` (`self.dynMaterial`) (`self.Material`) false)
  (`PrimitiveComponent.SetMaterial` (`self.StaticMesh`) 0 (`self.dynMaterial`))
  (`PrimitiveComponent.SetSimulatePhysics` (`self.StaticMesh`) true)
  (`PrimitiveComponent.SetLinearDamping` (`self.StaticMesh`) (`self.Damping`)))