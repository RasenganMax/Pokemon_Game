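; Stump actor that stands in for the base of a ChoppableTree once it is fully chopped.
; Its construction script rebuilds the stump from mesh components passed in by that tree, setting the static mesh and adding a spline mesh for the chopped section.
; The spline mesh copies the source's shape, scales and bark and interior materials.
; The event graph holds no active logic.
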(fn `UserConstructionScript`
  (bind _stumpsplinechopmesh (`self.stumpSplineChopMesh`))
  ;[0.02 0.02 0.02] Set static mesh and spline mesh part for fully chopped stump. The mesh info is passed from ChoppableTree blueprint, upon fully chopping.
  (`StaticMeshComponent.SetStaticMesh` (`self.Mesh`) (`StaticMeshComponent.StaticMesh` (`self.stumpMesh`)))
  (bind _returnvalue (`AddComponent|NODE_AddSplineMeshComponent-0`))
  (`StaticMeshComponent.SetStaticMesh` _returnvalue (`StaticMeshComponent.StaticMesh` _stumpsplinechopmesh))
  (`SplineMeshComponent.SetStartAndEnd` _returnvalue (`SplineMeshComponent.GetStartPosition` _stumpsplinechopmesh) (`SplineMeshComponent.GetStartTangent` _stumpsplinechopmesh) (`SplineMeshComponent.GetEndPosition` _stumpsplinechopmesh) (`SplineMeshComponent.GetEndTangent` _stumpsplinechopmesh) false)
  (`SplineMeshComponent.SetStartScale` _returnvalue (`SplineMeshComponent.GetStartScale` (`self.stumpSplineChopMesh`)) false)
  (`SplineMeshComponent.SetEndScale` _returnvalue (`SplineMeshComponent.GetEndScale` (`self.stumpSplineChopMesh`)) true)
  ;[0.02 0.02 0.02] Set materials for interior and bark
  (`PrimitiveComponent.SetMaterial` _returnvalue 1 (`PrimitiveComponent.GetMaterial` (`self.stumpSplineChopMesh`) 1))
  (`PrimitiveComponent.SetMaterial` _returnvalue 0 (`PrimitiveComponent.GetMaterial` (`self.stumpSplineChopMesh`) 0)))