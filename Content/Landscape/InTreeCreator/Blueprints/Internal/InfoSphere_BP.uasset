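; InfoSphere_BP is a helper actor for the InTreeCreator tree generator that previews wind and displays debug text.
; Its construction script, with WindPreview on, writes the actor's forward vector and preview strength to the WindParameters collection and re-centres its height on TreeGen's bounds.
; Otherwise it hides the wind-direction meshes.
; Both paths offset the sphere by the tree's extent to avoid overlap and update the text, noting hidden splines.
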(fn `AdjustLocationToCurrentTreeSize`
  (locals (infoText :type String))
  ;[0.005 0.005 0.005] Adjusts the info sphere location based on current tree bounds. This prevents it from overlapping the tree. Also add some debug info for user - might add more info later.
  (`SceneComponent.K2_SetWorldTransform` (`self.Sphere`) (`KismetMathLibrary.MakeTransform` (`KismetMathLibrary.MakeVector` (* (.x (`.BoxExtent` (`self.GetActorBounds` (`self.treeGen`) false))) 1.2)) (struct :`Yaw` 90.0)) false false)
  (if (`/Game/Landscape/InTreeCreator/Blueprints/TreeGenerator_BP.HIDE_ALL_SPLINES` (`self.treeGen`))
    (set `local.infoText` (`KismetStringLibrary.Concat_StrStr` (`local.infoText`) "All splines hidden")))
  (`TextRenderComponent.K2_SetText` (`self.Info1`) (`KismetSystemLibrary.MakeLiteralText` (`KismetTextLibrary.Conv_StringToText` (`local.infoText`)))))

(fn `UserConstructionScript`
  (if (`self.WindPreview`)
    (`|ExecutionSequence`
      (:`then_0`
        ;[0.005 0.005 0.005] Set wind parameters based on the actor rotation & WindStrength value.
        (`KismetMaterialLibrary.SetVectorParameterValue` "/Game/Landscape/InTreeCreator/Materials/WindParameters.WindParameters" "WindDirection" (`KismetMathLibrary.Conv_VectorToLinearColor` (`self.GetActorForwardVector`)))
        (`KismetMaterialLibrary.SetScalarParameterValue` "/Game/Landscape/InTreeCreator/Materials/WindParameters.WindParameters" "WindStrength" (`self.WindPreviewStrength`)))
      (:`then_1`
        ;[0.005 0.005 0.005] Set the location to around the center of tree generator to achieve better visualization preview
        (`self.K2_SetActorLocation` (`KismetMathLibrary.MakeVector` 0.0 0.0 (* (.z (`self.GetActorBounds` (`self.treeGen`) false)) 1.3))))
      (:`then_2`
        (`self.AdjustLocationToCurrentTreeSize` :!label _label)))
    (else
      ;[0.08767 0.16 0.0288] Show/hide the wind direction visualiation meshes.
      (`SceneComponent.SetVisibility` (`self.Arrow`) false false)
      (`SceneComponent.SetVisibility` (`self.Cube`) false false)
      (`SceneComponent.SetVisibility` (`self.StaticMesh`) false false)
      (goto _label))))