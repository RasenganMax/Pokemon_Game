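; BillboardPlaneForMerge_V2_BP is an InTreeCreator actor that assembles tree billboard planes, apparently for merging into one mesh.
; Its construction script vertex-paints the non-trunk planes opaque black so the billboard material can tell the trunk plane from the rest.
; It then applies the billboard material, if valid, to all four planes and destroys both cross planes when CROSSPLANES is off.
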(fn `UserConstructionScript`
  ;[0.1165 0.245 0.01241] Paint these planes with vertex color to make them work properly with billboard material, because it uses vertex color to distinguish trunk plane from the rest.
  (`MeshVertexPainterKismetLibrary.PaintVerticesSingleColor` (`self.PlaneForTheRest`) (make `LinearColor` 0.0 0.0 0.0 1.0))
  (`MeshVertexPainterKismetLibrary.PaintVerticesSingleColor` (`self.PlaneForTheRest_Cross`) (make `LinearColor` 0.0 0.0 0.0 1.0))
  ;[0.0613 0.2 0.01102] If billboard material is valid, assign it to all the plane meshes. Finally, if user doesn't want cross planes for billboard, destroy the cross planes.
  (`/Engine/EditorBlueprintResources/StandardMacros.IsValid` (`self.BillboardMaterial`)
    (:`Is Valid`
      (`PrimitiveComponent.SetMaterial` (`self.PlaneForTrunk`) 0 (`self.BillboardMaterial`))
      (`PrimitiveComponent.SetMaterial` (`self.PlaneForTheRest`) 0 (`self.BillboardMaterial`))
      (`PrimitiveComponent.SetMaterial` (`self.PlaneForTrunk_Cross`) 0 (`self.BillboardMaterial`))
      (`PrimitiveComponent.SetMaterial` (`self.PlaneForTheRest_Cross`) 0 (`self.BillboardMaterial`))
      (if (not (`self.CROSS_PLANES`))
        (`ActorComponent.K2_DestroyComponent` (`self.PlaneForTheRest_Cross`))
        (`ActorComponent.K2_DestroyComponent` (`self.PlaneForTrunk_Cross`))))))