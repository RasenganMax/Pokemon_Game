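; Choppable tree actor that takes hit damage and shows progressive chop damage until it is felled.
; ReacttoChoppingHit maps lost HP to four stages, rebuilding two spline meshes from ChopInfo with bark parameters copied from the material named "bark".
; Each hit emits splinters and may drop random debris.
; At the final stage, it spawns separate stump and chopped tree actors, passing on meshes and fall settings, then destroys itself.
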(event `/Game/Landscape/InTreeCreator/Blueprints/Internal/Choppable_BP.ReactToChoppingHit`
  (params (HitStrength :type "Float (single-precision)") (`'HitItem'` :type Integer))
  (bind _chopinfo (`self.chopInfo`))
  (bind _chopinfo_2 (`self.chopInfo`))
  (bind _addedsplinemesh_bottom (`self.addedSplineMesh_Bottom`))
  (bind _addedsplinemesh_top (`self.addedSplineMesh_Top`))
  (bind ((`MidSplineLoc_10_4FD1D683443C0DB542DF97ACE94E1B04` _midsplineloc) (`MidSplineTangent_12_2BDAA5A04D634E445EE75DA21E6EA30C` _midsplinetangent)) (break `/Game/Landscape/InTreeCreator/Blueprints/Internal/Misc/UnivChopPartInfo` _chopinfo))
  (bind ((`BottomSplineLoc_16_4D5395644CAE3955514F39A4EF21FFAE` _bottomsplineloc) (`BottomSplineTangent_18_C0FBC8304DB933E7754CE7BE9217DCEB` _bottomsplinetangent)) (break `/Game/Landscape/InTreeCreator/Blueprints/Internal/Misc/UnivChopPartInfo` _chopinfo_2))
  (bind ((`TopSplineLoc_5_EF40C68C4612F890D5028DAF224670A2` _topsplineloc) (`TopSplineTangent_6_62A0D1424E96B368C2AEF782C366A8BB` _topsplinetangent) (`TopSplineScale_21_1833EB81447B7BC61E36A6835B278B5A` _topsplinescale) (`MidSplineScale_22_2728E77B46A0F74BFAEAE086C0B4A07B` _midsplinescale)) (break `/Game/Landscape/InTreeCreator/Blueprints/Internal/Misc/UnivChopPartInfo` _chopinfo))
  (bind ((`MidSplineLoc_10_4FD1D683443C0DB542DF97ACE94E1B04` _midsplineloc_2) (`MidSplineTangent_12_2BDAA5A04D634E445EE75DA21E6EA30C` _midsplinetangent_2) (`MidSplineScale_22_2728E77B46A0F74BFAEAE086C0B4A07B` _midsplinescale_2) (`BottomSplineScale_23_3225188E4CC0C5C4EA7E04AAA7EFA705` _bottomsplinescale)) (break `/Game/Landscape/InTreeCreator/Blueprints/Internal/Misc/UnivChopPartInfo` _chopinfo_2))
  (set `self.hitStrength` HitStrength)
  (`|ExecutionSequence`
    (:`then_0`
      ;[0.1403 0.185 0.1165] Calculate current tree HP
      (set `self.currentHP` (- (`self.currentHP`) (`self.hitStrength`)))
      ;[0.01805 0.05761 0.06] By default there are 4 chop stages (4 different universal spline mesh variations)
      (bind _output_get (set `self.chopStagesCount` 4))
      (set `self.chopStageProgressStep` (/ 100.0 (`KismetMathLibrary.Conv_IntToDouble` _output_get)))
      ;[0.08261 0.17 0.01215] Calculate current missing % of tree HP and based on that, calculate current chop stage.
      (set `self.currentMissingHP_Percent` (* (- 1.0 (/ (`self.currentHP`) (`self.HP`))) 100.0))
      (set `self.calculatedChopStage` (`KismetMathLibrary.Clamp` (/ (`KismetMathLibrary.FCeil` (`self.currentMissingHP_Percent`)) (`KismetMathLibrary.FCeil` (`self.chopStageProgressStep`))) 0 (`self.chopStagesCount`)))
      ;[0.01 0.01 0.01] Check if initial chop (the first chopping hit) is already done, then assign previously calculated chop stage to the variable to use it i further calculations.
      (if (`self.initialChopDone`)
        (if (!= (`self.calculatedChopStage`) (`self.currentChopStage`))
          (bind _output_get_2 (set `self.currentChopStage` (`self.calculatedChopStage`) :!label _label))
          (if (>= _output_get_2 (`self.chopStagesCount`))
            ;[0.01 0.01 0.01] Spawn separate 'chopped' tree parts to be able to distinguish them as chopped stump and chopped tree, for example for gameplay purposes.
            ; Finally, destroy this 'choppable' version of tree.
            (`|SpawnActorFromClass` "/Game/Landscape/InTreeCreator/Blueprints/Internal/ChoppedTreeStump_BP.ChoppedTreeStump_BP_C" (`self.GetTransform`) "AlwaysSpawn" "OverrideRootScale" null (`self.choppedBottomMesh`) (`self.addedSplineMesh_Bottom`) null)
            (`|SpawnActorFromClass` "/Game/Landscape/InTreeCreator/Blueprints/Internal/ChoppedTree_BP.ChoppedTree_BP_C" (`self.GetTransform`) "AlwaysSpawn" "OverrideRootScale" null (`self.choppedTopMesh`) (`self.addedSplineMesh_Top`) (`self.fallingDebris`) (`self.fullChopImpactParticles`) (`self.hasFruits`) (`self.fruits`) (`self.FallingFruits_Height`) (`self.FallingFruits_AreaScale`) (`self.fallShakeStrength`) null)
            (`self.K2_DestroyActor`)
            (else
              (`|ExecutionSequence`
                (:`then_0`
                  ;[0.015 0.015 0.015] Destroy previously added spline meshes to make room for new chopped version.
                  (`|ExecutionSequence`
                    (:`then_0`
                      (`/Engine/EditorBlueprintResources/StandardMacros.IsValid` _addedsplinemesh_bottom
                        (:`Is Valid`
                          (`ActorComponent.K2_DestroyComponent` _addedsplinemesh_bottom))))
                    (:`then_1`
                      (`/Engine/EditorBlueprintResources/StandardMacros.IsValid` _addedsplinemesh_top
                        (:`Is Valid`
                          (`ActorComponent.K2_DestroyComponent` _addedsplinemesh_top))))))
                (:`then_1`
                  ;[0.015 0.015 0.015] Detect material assignment from the mesh by checking material name. User should name any custom materials accordingly, as stated in the documentation.
                  ; Then create dynamic material using parameters from detected bark material.
                  (for _array_element (`MeshComponent.GetMaterials` (`self.choppedTopMesh`))
                    (if (`KismetStringLibrary.Contains` (`KismetSystemLibrary.GetDisplayName` _array_element) "bark")
                      (set `self.detectedBarkMaterial` _array_element)))
                  (bind _returnvalue (`KismetMaterialLibrary.CreateDynamicMaterialInstance` "/Game/Landscape/InTreeCreator/Materials/Masters/BarkForChopParts_M.BarkForChopParts_M"))
                  (bind _output_get_3 (set `self.dynMatForChoppedParts` _returnvalue))
                  (`MaterialInstanceDynamic.CopyParameterOverrides` _output_get_3 (cast `MaterialInstance` (`self.detectedBarkMaterial`) :!pure true)))
                (:`then_2`
                  ;[0.01 0.01 0.01] Add universal chopped modular mesh for top chopped part. Set its properties by using the Chop Info that user should paste in (more info in the documentation)
                  (bind _returnvalue_2 (`AddComponent|NODE_AddSplineMeshComponent-0`))
                  (bind _output_get_4 (set `self.addedSplineMesh_Bottom` _returnvalue_2))
                  (`StaticMeshComponent.SetStaticMesh` _output_get_4 (select `int` (`self.currentChopStage`) :`0` "/Game/Landscape/InTreeCreator/Meshes/ModularParts/univChopPart_Bottom_1_SM.univChopPart_Bottom_1_SM" :`1` "/Game/Landscape/InTreeCreator/Meshes/ModularParts/univChopPart_Bottom_2_SM.univChopPart_Bottom_2_SM" :`2` "/Game/Landscape/InTreeCreator/Meshes/ModularParts/univChopPart_Bottom_3_SM.univChopPart_Bottom_3_SM" :`3` "/Game/Landscape/InTreeCreator/Meshes/ModularParts/univChopPart_Bottom_4_SM.univChopPart_Bottom_4_SM" :!type "StaticMesh Object Reference"))
                  (`SplineMeshComponent.SetStartAndEnd` (`self.addedSplineMesh_Bottom`) _bottomsplineloc _bottomsplinetangent _midsplineloc_2 _midsplinetangent_2 false)
                  (`SplineMeshComponent.SetStartScale` (`self.addedSplineMesh_Bottom`) _bottomsplinescale false)
                  (`SplineMeshComponent.SetEndScale` (`self.addedSplineMesh_Bottom`) _midsplinescale_2 true)
                  ;;[0.04088 0.175 0.1055] Set material for interior
                  (`PrimitiveComponent.SetMaterial` (`self.addedSplineMesh_Bottom`) 1 (`self.interiorMaterial`))
                  (`PrimitiveComponent.SetMaterial` (`self.addedSplineMesh_Bottom`) 0 (`self.dynMatForChoppedParts`)))
                (:`then_3`
                  ;[0 0 0] Add universal chopped modular mesh for bottom chopped part. Set its properties by using the Chop Info that user should paste in (more info in the documentation)
                  (bind _returnvalue_3 (`AddComponent|NODE_AddSplineMeshComponent-1`))
                  (bind _output_get_5 (set `self.addedSplineMesh_Top` _returnvalue_3))
                  (`StaticMeshComponent.SetStaticMesh` _output_get_5 (select `int` (`self.currentChopStage`) :`0` "/Game/Landscape/InTreeCreator/Meshes/ModularParts/univChopPart_Top_1_SM.univChopPart_Top_1_SM" :`1` "/Game/Landscape/InTreeCreator/Meshes/ModularParts/univChopPart_Top_2_SM.univChopPart_Top_2_SM" :`2` "/Game/Landscape/InTreeCreator/Meshes/ModularParts/univChopPart_Top_3_SM.univChopPart_Top_3_SM" :`3` "/Game/Landscape/InTreeCreator/Meshes/ModularParts/univChopPart_Top_4_SM.univChopPart_Top_4_SM" :!type "StaticMesh Object Reference"))
                  (`SplineMeshComponent.SetStartAndEnd` (`self.addedSplineMesh_Top`) _midsplineloc _midsplinetangent _topsplineloc _topsplinetangent false)
                  (`SplineMeshComponent.SetStartScale` (`self.addedSplineMesh_Top`) _midsplinescale false)
                  (`SplineMeshComponent.SetEndScale` (`self.addedSplineMesh_Top`) _topsplinescale true)
                  ;;[0.03922 0.1725 0.1059] Set material for interior
                  (`PrimitiveComponent.SetMaterial` (`self.addedSplineMesh_Top`) 1 (`self.interiorMaterial`))
                  (`PrimitiveComponent.SetMaterial` (`self.addedSplineMesh_Top`) 0 (`self.dynMatForChoppedParts`)))))))
        (else
          (set `self.initialChopDone` true)
          (goto _label))))
    (:`then_1`
      ;[0.375 0.288 0.1631] Splinters: Falling particles
      (`GameplayStatics.SpawnEmitterAtLocation` "/Game/Landscape/InTreeCreator/Particles/Misc/ChopEffect1_PS.ChopEffect1_PS" (`KismetMathLibrary.TransformLocation` (`self.GetTransform`) (`.MidSplineLoc_10_4FD1D683443C0DB542DF97ACE94E1B04` (break `/Game/Landscape/InTreeCreator/Blueprints/Internal/Misc/UnivChopPartInfo` (`self.chopInfo`)))))
      ;[0 0.149 1] Spawn falling debris from chopping hit. It uses the user-specified parameters for debris spawn height & area size.
      (if (`KismetMathLibrary.RandomBoolWithWeight` (`self.chopping_FallingDebris_ChancePerHit`))
        (set `self.baseSpawnLocation` (`KismetMathLibrary.MakeVector` (.x (`self.K2_GetActorLocation`)) (.y (`self.K2_GetActorLocation`)) (+ (.z (`self.K2_GetActorLocation`)) (* (* (.z (`.BoxExtent` (`self.GetActorBounds` false))) 2.0) (`self.FallingDebris_Height`)))))
        (for _array_element_2 (`self.fallingDebris`)
          (bind (_minamountfromimpulse _maxamountfromimpulse _minamountfromtreefall _maxamountfromtreefall _mesh _scale_min _scale_max _gettexturesfrom _damping) (break `/Game/Landscape/InTreeCreator/Blueprints/Internal/Misc/TreeDebris` _array_element_2))
          (for _ (range 1 (+ (`KismetMathLibrary.RandomIntegerInRange` _minamountfromimpulse _maxamountfromimpulse) 1))
            (`|SpawnActorFromClass` "/Game/Landscape/InTreeCreator/Blueprints/Internal/TreeDebris_BP.TreeDebris_BP_C" (`KismetMathLibrary.MakeTransform` (`KismetMathLibrary.RandomPointInBoundingBox` (`self.baseSpawnLocation`) (* (`.BoxExtent` (`self.GetActorBounds` false)) (`self.FallingDebris_AreaScale`))) (struct) (`KismetMathLibrary.Conv_DoubleToVector` (`KismetMathLibrary.RandomFloatInRange` _scale_min _scale_max))) "AlwaysSpawn" "OverrideRootScale" null _mesh (`self.dynMatForChoppedParts`) (0.0 0.0 0.0) _damping null)))))))

(fn `UserConstructionScript`
  ;[0.1883 0.49 0.04351] Set the user-specified mesh for chopped top & bottom parts + tree chopping HP.
  (`StaticMeshComponent.SetStaticMesh` (`self.choppedTopMesh`) (`self.ChoppedTop`))
  (`StaticMeshComponent.SetStaticMesh` (`self.choppedBottomMesh`) (`self.ChoppedBottom`))
  (set `self.currentHP` (`self.HP`)))