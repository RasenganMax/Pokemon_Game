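; TreeFruit_BP is a short-lived physics fruit for the InTreeCreator tree tool.
; Its construction script applies the mesh, two materials and damping from its variables and enables physics simulation.
; Shortly after BeginPlay it gets an initial impulse and random spin.
; To limit performance cost, it later stops simulating and ignores all collision, then destroys itself after a further delay.
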(event `self.ReceiveBeginPlay`
  ;[0.015 0.015 0.015] Add initial impulse force for the fruit. After X seconds turn off physics simulation to minimize performance hit. After another delay, destroy the fruit, for similar reasons.
  (`KismetSystemLibrary.Delay` 0.1)
  (`PrimitiveComponent.AddImpulse` (`self.StaticMesh`) (`self.initialImpulse`) "None" true)
  (`PrimitiveComponent.AddAngularImpulseInRadians` (`self.StaticMesh`) (`KismetMathLibrary.RandomUnitVector`) "None" true)
  (`KismetSystemLibrary.Delay` 7.0)
  (`PrimitiveComponent.SetSimulatePhysics` (`self.StaticMesh`) false)
  (`PrimitiveComponent.SetCollisionResponseToAllChannels` (`self.StaticMesh`) "ECR_Ignore")
  (`KismetSystemLibrary.Delay` 30.0)
  (`self.K2_DestroyActor`))

(fn `UserConstructionScript`
  (locals (dynMaterial :type "MaterialInstanceDynamic Object Reference"))
  ;[0.01 0.01 0.01] Assign all the fruit parameters and turn on physics simulation.
  (`StaticMeshComponent.SetStaticMesh` (`self.StaticMesh`) (`self.Mesh`))
  (`PrimitiveComponent.SetMaterial` (`self.StaticMesh`) 0 (`self.Material`))
  (`PrimitiveComponent.SetMaterial` (`self.StaticMesh`) 1 (`self.Material2`))
  (`PrimitiveComponent.SetSimulatePhysics` (`self.StaticMesh`) true)
  (`PrimitiveComponent.SetLinearDamping` (`self.StaticMesh`) (`self.Damping`))
  (`PrimitiveComponent.SetAngularDamping` (`self.StaticMesh`) 5.0))