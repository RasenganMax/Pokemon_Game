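; Example flying actor for InTreeCreator that moves in a straight line along its initial facing.
; BeginPlay caches the forward vector scaled by Speed and, if DestroyAfterSeconds is non-zero, destroys the actor after that delay.
; Tick adds the cached vector as an unswept world offset without delta-time scaling, so travel speed depends on frame rate.
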(event `self.ReceiveBeginPlay`
  ;[0 0.2373 1] Set flying direction at Begin Play, using current actor orientation.
  (set `self.Dir` (* (`self.GetActorForwardVector`) (`self.speed`)))
  ;[1 1 1] Destroy after X seconds.
  (if (!= (`self.destroyAfterSeconds`) 0.0)
    (`KismetSystemLibrary.Delay` (`self.destroyAfterSeconds`))
    (`self.K2_DestroyActor`)))

(event `self.ReceiveTick`
  (params (DeltaSeconds :type "Float (single-precision)"))
  ;[0 0.4104 1] SImple flying movement in previously set direction by adding the vector every tick as location offset.
  (`self.K2_AddActorWorldOffset` (`self.Dir`)))

(fn `UserConstructionScript`)