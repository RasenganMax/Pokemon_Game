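; Physics actor for a felled tree, built from the mesh and spline chop part passed by ChoppableTree.
; A timer temporarily caps horizontal velocity to stop collision launches, and physics switches off later.
; Name-matched bark, leaf and fruit materials become dynamic instances, with timelines driving wind fade and shake.
; Polling detects impact from sudden speed loss, then spawns particles, debris and fruit and makes the tree pickable after a delay.
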(event `LimitVelocityIfNeeded`
  (bind _returnvalue (`SceneComponent.GetComponentVelocity` (`self.Mesh`)))
  ;[0.025 0.025 0.025] Fixes UE physics throwing trees far away when it's colliding with other trees. It will limit its velocity as soon as it detects a sudden speed increase.
  (if (> (`KismetMathLibrary.Sqrt` (+ (`KismetMathLibrary.Square` (.x _returnvalue)) (`KismetMathLibrary.Square` (.y _returnvalue)))) (`self.maxVelocity`))
    (`PrimitiveComponent.SetAllPhysicsLinearVelocity` (`self.Mesh`) (`KismetMathLibrary.MakeVector` (.x (* (`KismetMathLibrary.Normal` (`KismetMathLibrary.MakeVector` (.x _returnvalue) (.y _returnvalue))) (`self.maxVelocity`))) (.y (* (`KismetMathLibrary.Normal` (`KismetMathLibrary.MakeVector` (.x _returnvalue) (.y _returnvalue))) (`self.maxVelocity`))) (.z _returnvalue)) false)))

(event `self.ReceiveBeginPlay`
  (bind _returnvalue (`KismetMathLibrary.RandomFloatInRange` -100.0 100.0))
  (bind _returnvalue_2 (`KismetMathLibrary.RandomFloatInRange` -100.0 100.0))
  (bind _detectedleafmaterials (`self.detectedLeafMaterials`))
  (bind _detectedbarkmaterials (`self.detectedBarkMaterials`))
  (bind _mesh (`self.Mesh`))
  (bind _mesh_2 (`self.Mesh`))
  (bind _dynmatforchopped_bark (`self.dynMatForChopped_Bark`))
  (bind _dynmatforchopped_leaves (`self.dynMatForChopped_Leaves`))
  (bind _dynmatforchopped_fruits (`self.dynMatForChopped_Fruits`))
  (bind (_origin _boxextent) (`KismetSystemLibrary.GetComponentBounds` (`self.Mesh`)))
  (bind _returnvalue_3 (`KismetSystemLibrary.GetDisplayName` (`self.mat`)))
  (`|ExecutionSequence`
    (:`then_0`
      ;[0.005 0.005 0.005] Attach the universal spline part to the main mesh, set its mass scale and finally simulate physics.
      (`SceneComponent.K2_AttachToComponent` (`self.splineMeshChop`) (`self.Mesh`) "None" "KeepWorld" "KeepWorld" "KeepWorld" true)
      (`PrimitiveComponent.SetAllMassScale` (`self.Mesh`) 20.0)
      (`KismetSystemLibrary.Delay` 0.1)
      (`PrimitiveComponent.SetSimulatePhysics` (`self.Mesh`) true)
      ;[0.025 0.025 0.025] Fixes UE physics throwing trees far away when it's colliding with other trees. It will limit its velocity as soon as it detects a sudden speed increase.
      (`PrimitiveComponent.SetPhysicsMaxAngularVelocityInDegrees` (`self.Mesh`) 200.0 false "None")
      (bind _returnvalue_4 (`KismetSystemLibrary.K2_SetTimerDelegate` (delegate `LimitVelocityIfNeeded`) 0.04 true))
      (set `self.limitVelocityTimer` _returnvalue_4))
    (:`then_1`
      ;[0.005 0.005 0.005] Turn off physics simulation after X (10 -> 10 by default) seconds.
      ; Also disable the velocity limiter, to save CPU.
      (`KismetSystemLibrary.Delay` 10.0)
      (`KismetSystemLibrary.K2_ClearAndInvalidateTimerHandle` (`self.limitVelocityTimer`))
      (`KismetSystemLibrary.Delay` 10.0)
      (`PrimitiveComponent.SetSimulatePhysics` (`self.Mesh`) false))
    (:`then_2`
      (`|ExecutionSequence`
        (:`then_0`
          ;[0.015 0.015 0.015] Detect bark/leaf/fruit material from the mesh by checking material name. User should name any custom materials accordingly, as stated in the documentation.
          (for _array_element (`MeshComponent.GetMaterials` (`self.Mesh`))
            (set `self.mat` _array_element)
            (if (`KismetStringLibrary.Contains` _returnvalue_3 "bark")
              (`KismetArrayLibrary.Array_Add` (`self.detectedBarkMaterials`) (`self.mat`))
              (elif (`KismetStringLibrary.Contains` _returnvalue_3 "leaves")
                (`KismetArrayLibrary.Array_Add` (`self.detectedLeafMaterials`) (`self.mat`))
                (elif (`KismetStringLibrary.Contains` _returnvalue_3 "fruit")
                  (`KismetArrayLibrary.Array_Add` (`self.detectedFruitMaterials`) (`self.mat`))))))
          (`|ExecutionSequence`
            (:`then_0`
              ;[0.005 0.005 0.005] Create & set dynamic materials for chopped tree mesh. Used to fade the wind out and play shake effect.
              (for _array_element_2 (`self.detectedLeafMaterials`)
                (bind _returnvalue_5 (`KismetMaterialLibrary.CreateDynamicMaterialInstance` "/Game/Landscape/InTreeCreator/Materials/Masters/Leaf_ForChopped_M.Leaf_ForChopped_M"))
                (bind _output_get (set `self.dynMatForChopped_Leaves` _returnvalue_5))
                (`MaterialInstanceDynamic.K2_CopyMaterialInstanceParameters` _output_get _array_element_2 false)
                (`PrimitiveComponent.SetMaterial` (`self.Mesh`) (`KismetArrayLibrary.Array_Find` (`MeshComponent.GetMaterials` (`self.Mesh`)) _array_element_2) _dynmatforchopped_leaves)
                (`KismetArrayLibrary.Array_Add` (`self.dynMatsForChopped_Leaves`) _dynmatforchopped_leaves)))
            (:`then_1`
              (for _array_element_3 (`self.detectedBarkMaterials`)
                (bind _returnvalue_6 (`KismetMaterialLibrary.CreateDynamicMaterialInstance` "/Game/Landscape/InTreeCreator/Materials/Masters/Bark_ForChopped_M.Bark_ForChopped_M"))
                (bind _output_get_2 (set `self.dynMatForChopped_Bark` _returnvalue_6))
                (`MaterialInstanceDynamic.K2_CopyMaterialInstanceParameters` _output_get_2 _array_element_3 false)
                (`PrimitiveComponent.SetMaterial` (`self.Mesh`) (`KismetArrayLibrary.Array_Find` (`MeshComponent.GetMaterials` (`self.Mesh`)) _array_element_3) _dynmatforchopped_bark)
                (`KismetArrayLibrary.Array_Add` (`self.dynMatsForChopped_Bark`) _dynmatforchopped_bark)))
            (:`then_2`
              (if (`self.hasFruits`)
                (for _array_element_4 (`self.detectedFruitMaterials`)
                  (bind _returnvalue_7 (`KismetMaterialLibrary.CreateDynamicMaterialInstance` "/Game/Landscape/InTreeCreator/Materials/Masters/TreeFruit_ForChopped_M.TreeFruit_ForChopped_M"))
                  (bind _output_get_3 (set `self.dynMatForChopped_Fruits` _returnvalue_7))
                  (`MaterialInstanceDynamic.K2_CopyMaterialInstanceParameters` _output_get_3 _array_element_4 false)
                  (`PrimitiveComponent.SetMaterial` (`self.Mesh`) (`KismetArrayLibrary.Array_Find` (`MeshComponent.GetMaterials` (`self.Mesh`)) _array_element_4) _dynmatforchopped_fruits)
                  (`KismetArrayLibrary.Array_Add` (`self.dynMatsForChopped_Fruits`) _dynmatforchopped_fruits))))))
        (:`then_1`
          ;[0.01 0.01 0.01] To avoid fast micro leaf noise jitter due to tree movement + throw some life into leaves when falling
          (bind (_direction _alphamicroleaves) (`Timeline|FadeTimeline` :!via `PlayFromStart`)
            (:`Update`
              (`MaterialInstanceDynamic.SetScalarParameterValue` (`self.dynMatsForChopped_Leaves`) "LeafMicroWindFadeOut" _alphamicroleaves)
              (if (`self.hasFruits`)
                (bind _returnvalue_8 (* _alphamicroleaves (`self.FallShakeStrength`)))
                (`MaterialInstanceDynamic.SetScalarParameterValue` (`self.dynMatsForChopped_Leaves`) "FallShake" _returnvalue_8)
                (`MaterialInstanceDynamic.SetScalarParameterValue` (`self.dynMatsForChopped_Bark`) "FallShake" _returnvalue_8)
                (`MaterialInstanceDynamic.SetScalarParameterValue` (`self.dynMatsForChopped_Fruits`) "FallShake" _returnvalue_8)
                (else
                  (`MaterialInstanceDynamic.SetScalarParameterValue` (`self.dynMatsForChopped_Leaves`) "FallShake" _returnvalue_8)
                  (`MaterialInstanceDynamic.SetScalarParameterValue` (`self.dynMatsForChopped_Bark`) "FallShake" _returnvalue_8))))))))
    (:`then_3`
      ;[0.01 0.01 0.01] Detect if broken tree part hit a ground (sudden velocity decrease)
      (bind _returnvalue_9 (`PrimitiveComponent.GetPhysicsLinearVelocity` (`self.Mesh`) "None" :!label _label))
      (bind _returnvalue_10 (`KismetMathLibrary.VSize` _returnvalue_9))
      (if (and (< _returnvalue_10 (`self.previousVelocity`)) (> (`KismetMathLibrary.Abs` (- _returnvalue_10 (`self.previousVelocity`))) 100.0))
        (`|ExecutionSequence`
          (:`then_0`
            ;[0.01 0.01 0.01] Make it pickable after specified amount of seconds.
            (`KismetSystemLibrary.Delay` (`self.pickableAfterXFromFall`))
            (set `self.alreadyPickable` true))
          (:`then_1`
            ;[0.01 0.01 0.01] Adjust material parameters to achieve shake effect
            (`MaterialInstanceDynamic.SetScalarParameterValue` (`self.dynMatsForChopped_Leaves`) "rotMotion_speed" 3.0)
            (`MaterialInstanceDynamic.SetScalarParameterValue` (`self.dynMatsForChopped_Leaves`) "upDown_speed" 2.0)
            (`MaterialInstanceDynamic.SetScalarParameterValue` (`self.dynMatsForChopped_Leaves`) "rotMotion_Elasticity" 0.01)
            (`MaterialInstanceDynamic.SetScalarParameterValue` (`self.dynMatsForChopped_Leaves`) "elasticity_UpDownMovement" 0.15)
            ;[0.01 0.01 0.01] Play shake effect by smoothly adjusting material parameters. It results in fall impact shake effect and calms down main wind after fully chopped.
            (bind (_direction_2 _windout _microleaffadeout _updownshake) (`Timeline|ShakeAlpha` :!via `PlayFromStart`)
              (:`Update`
                (`MaterialInstanceDynamic.SetScalarParameterValue` (`self.dynMatsForChopped_Leaves`) "LeafMicroWindFadeOut" _microleaffadeout)
                (if (`self.hasFruits`)
                  (`MaterialInstanceDynamic.SetScalarParameterValue` (`self.dynMatsForChopped_Leaves`) "BranchWindFadeOut" _windout)
                  (`MaterialInstanceDynamic.SetScalarParameterValue` (`self.dynMatsForChopped_Bark`) "BranchWindFadeOut" _windout)
                  (`MaterialInstanceDynamic.SetScalarParameterValue` (`self.dynMatsForChopped_Fruits`) "BranchWindFadeOut" _windout)
                  (`MaterialInstanceDynamic.SetScalarParameterValue` (`self.dynMatsForChopped_Leaves`) "MainWindFadeOut" _windout)
                  (`MaterialInstanceDynamic.SetScalarParameterValue` (`self.dynMatsForChopped_Bark`) "MainWindFadeOut" _windout)
                  (`MaterialInstanceDynamic.SetScalarParameterValue` (`self.dynMatsForChopped_Fruits`) "MainWindFadeOut" _windout)
                  (bind _returnvalue_11 (* _updownshake (`self.FallShakeStrength`)))
                  (`MaterialInstanceDynamic.SetScalarParameterValue` (`self.dynMatsForChopped_Leaves`) "FallShake" _returnvalue_11)
                  (`MaterialInstanceDynamic.SetScalarParameterValue` (`self.dynMatsForChopped_Bark`) "FallShake" _returnvalue_11)
                  (`MaterialInstanceDynamic.SetScalarParameterValue` (`self.dynMatsForChopped_Fruits`) "FallShake" _returnvalue_11)
                  (else
                    (`MaterialInstanceDynamic.SetScalarParameterValue` (`self.dynMatsForChopped_Leaves`) "BranchWindFadeOut" _windout)
                    (`MaterialInstanceDynamic.SetScalarParameterValue` (`self.dynMatsForChopped_Bark`) "BranchWindFadeOut" _windout)
                    (`MaterialInstanceDynamic.SetScalarParameterValue` (`self.dynMatsForChopped_Leaves`) "MainWindFadeOut" _windout)
                    (`MaterialInstanceDynamic.SetScalarParameterValue` (`self.dynMatsForChopped_Bark`) "MainWindFadeOut" _windout)
                    (`MaterialInstanceDynamic.SetScalarParameterValue` (`self.dynMatsForChopped_Leaves`) "FallShake" _returnvalue_11)
                    (`MaterialInstanceDynamic.SetScalarParameterValue` (`self.dynMatsForChopped_Bark`) "FallShake" _returnvalue_11))))))
          (:`then_2`
            ;[0.01 0.01 0.01] Spawn assigned particles from fall impact
            (for _array_element_5 (`self.fallImpactParticles`)
              (`GameplayStatics.SpawnEmitterAtLocation` _array_element_5 (`KismetSystemLibrary.GetComponentBounds` _mesh) (`KismetMathLibrary.Conv_VectorToRotator` (`SceneComponent.GetUpVector` _mesh)))))
          (:`then_3`
            ;[0.01 0.01 0.01] Spawn assigned debris from fall impact
            (for _array_element_6 (`self.fallImpactDebris`)
              (`|ExecutionSequence`
                (:`then_0`
                  ;[0.005 0.005 0.005] Detect material assignment from the mesh by checking material name. User should name any custom materials accordingly, as stated in the documentation.
                  (switch `/Game/Landscape/InTreeCreator/Blueprints/Internal/Misc/Bark_or_Leaves` (`.GetTexturesFrom_27_3714FF7D4E17CC99ED6E8BB0C5106141` (break `/Game/Landscape/InTreeCreator/Blueprints/Internal/Misc/TreeDebris` _array_element_6))
                    (:`NewEnumerator0`
                      (for _array_element_7 (`MeshComponent.GetMaterials` (`self.Mesh`))
                        (if (`KismetStringLibrary.Contains` (`KismetSystemLibrary.GetDisplayName` _array_element_7) "bark")
                          (`KismetArrayLibrary.Array_Add` (`self.detectedBarkMaterials`) _array_element_7)))
                      (set `self.materialForDebris` (`|GetArrayItem` _detectedbarkmaterials (`KismetMathLibrary.RandomInteger` (`KismetArrayLibrary.Array_Length` _detectedbarkmaterials)))))
                    (:`NewEnumerator1`
                      (for _array_element_8 (`MeshComponent.GetMaterials` (`self.Mesh`))
                        (if (`KismetStringLibrary.Contains` (`KismetSystemLibrary.GetDisplayName` _array_element_8) "leaves")
                          (`KismetArrayLibrary.Array_Add` (`self.detectedLeafMaterials`) _array_element_8)))
                      (set `self.materialForDebris` (`|GetArrayItem` _detectedleafmaterials (`KismetMathLibrary.RandomInteger` (`KismetArrayLibrary.Array_Length` _detectedleafmaterials)))))))
                (:`then_1`
                  (bind (_minamountfromimpulse _maxamountfromimpulse _minamountfromtreefall _maxamountfromtreefall _mesh_3 _scale_min _scale_max _gettexturesfrom _damping) (break `/Game/Landscape/InTreeCreator/Blueprints/Internal/Misc/TreeDebris` _array_element_6))
                  (for _ (range 1 (+ (`KismetMathLibrary.RandomIntegerInRange` _minamountfromtreefall _maxamountfromtreefall) 1))
                    (`|SpawnActorFromClass` "/Game/Landscape/InTreeCreator/Blueprints/Internal/TreeDebris_BP.TreeDebris_BP_C" (`KismetMathLibrary.MakeTransform` (`KismetMathLibrary.RandomPointInBoundingBox` _origin (* _boxextent 0.7)) (struct) (`KismetMathLibrary.Conv_DoubleToVector` (* (`KismetMathLibrary.RandomFloatInRange` _scale_min _scale_max) 1.5))) "AlwaysSpawn" "OverrideRootScale" null _mesh_3 (`self.materialForDebris`) (`KismetMathLibrary.MakeVector` _returnvalue_2 _returnvalue_2 (`KismetMathLibrary.RandomFloatInRange` 300.0 700.0)) _damping null))))))
          (:`then_4`
            (if (`self.hasFruits`)
              ;[0.01 0.01 0.01] Spawn assigned fruits from fall impact
              (for _array_element_9 (`self.fruits`)
                (bind (_fruittype _minfallwith1impulse _maxfallwith1impulse _minfallaftertreefall _maxfallaftertreefall _minimumimpulsestrengthtofall _scalemin _scalemax _damping_2) (break `/Game/Landscape/InTreeCreator/Blueprints/Internal/Misc/TreeFruits` _array_element_9))
                (for _ (range 1 (+ (`KismetMathLibrary.RandomIntegerInRange` _minfallaftertreefall _maxfallaftertreefall) 1))
                  (`|SpawnActorFromClass` _fruittype (`KismetMathLibrary.MakeTransform` (`KismetMathLibrary.RandomPointInBoundingBox` (+ (* (`SceneComponent.GetUpVector` _mesh_2) (* (`self.FallingFruitsHeight`) (.z (`.Max` (`StaticMeshComponent.GetLocalBounds` _mesh_2))))) (`SceneComponent.K2_GetComponentLocation` _mesh_2)) (* (`.BoxExtent` (`KismetSystemLibrary.GetComponentBounds` (`self.Mesh`))) (`self.FallingFruitsAreaScale`))) (struct) (`KismetMathLibrary.Conv_DoubleToVector` (`KismetMathLibrary.RandomFloatInRange` _scalemin _scalemax))) "AdjustIfPossibleButAlwaysSpawn" "OverrideRootScale" null (`KismetMathLibrary.MakeVector` _returnvalue _returnvalue (`KismetMathLibrary.RandomFloatInRange` 300.0 700.0)) _damping_2 null))))))
        (else
          (set `self.previousVelocity` _returnvalue_10)
          (`KismetSystemLibrary.Delay` 0.05)
          (goto _label))))))

(fn `UserConstructionScript`
  (bind _splinemeshchoppart (`self.splineMeshChopPart`))
  ;[0.015 0.015 0.015] Set static mesh and spline mesh part for fully chopped stump. The mesh info is passed from ChoppableTree blueprint, upon fully chopping.
  (`StaticMeshComponent.SetStaticMesh` (`self.Mesh`) (`StaticMeshComponent.StaticMesh` (`self.choppedTreeMesh`)))
  (bind _returnvalue (`AddComponent|NODE_AddSplineMeshComponent-0`))
  (bind _output_get (set `self.splineMeshChop` _returnvalue))
  (`StaticMeshComponent.SetStaticMesh` _output_get (`StaticMeshComponent.StaticMesh` _splinemeshchoppart))
  (`SplineMeshComponent.SetStartAndEnd` _output_get (`SplineMeshComponent.GetStartPosition` _splinemeshchoppart) (`SplineMeshComponent.GetStartTangent` _splinemeshchoppart) (`SplineMeshComponent.GetEndPosition` _splinemeshchoppart) (`SplineMeshComponent.GetEndTangent` _splinemeshchoppart) false)
  (`SplineMeshComponent.SetStartScale` _output_get (`SplineMeshComponent.GetStartScale` (`self.splineMeshChopPart`)) false)
  (`SplineMeshComponent.SetEndScale` _output_get (`SplineMeshComponent.GetEndScale` (`self.splineMeshChopPart`)) true)
  ;[0.015 0.015 0.015] Set materials for interior and bark
  (`PrimitiveComponent.SetMaterial` _output_get 1 (`PrimitiveComponent.GetMaterial` (`self.splineMeshChopPart`) 1))
  (`PrimitiveComponent.SetMaterial` _output_get 0 (`PrimitiveComponent.GetMaterial` (`self.splineMeshChopPart`) 0)))