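; Foliage instance component for trees that adds falling leaves, debris, fruit drops and chopping to instanced meshes.
; Randomized looping timers spawn wind-aligned idle leaf emitters on instances near the camera and forget expired ones.
; Impulse functions spawn leaves, plus debris and fruits scaled by distance, matching debris materials by name and tracking fruit depletion per instance.
; A chopping hit swaps the instance for a ChoppableTree_BP actor and forwards the hit.
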(event `self.ReceiveBeginPlay`
  ;[0.12 0.1054 0.0786] Get player camera and set timers for updating idle falling leaves.
  (set `self.PlayerCameraManager` (`GameplayStatics.GetPlayerCameraManager` 0))
  (if (`self.FallingLeaves_Idle_ON`)
    (`KismetSystemLibrary.K2_SetTimerDelegate` (delegate `UpdateFallingLeavesAroundPlayer`) (`KismetMathLibrary.RandomFloatInRange` 1.5 2.0) true)
    (`KismetSystemLibrary.K2_SetTimerDelegate` (delegate `CheckIfCullIdleParticles`) (`KismetMathLibrary.RandomFloatInRange` 1.0 1.5) true)))

(event `UpdateFallingLeavesAroundPlayer`
  ;[0.12 0.1054 0.0786] Check for instances near camera and spawn idle falling leaves if it's close enough and if it's not already spawned.
  (for _array_element (`self.GetInstancesOverlappingSphere` (`PlayerCameraManager.GetCameraLocation` (`self.PlayerCameraManager`)) (`self.FallingLeaves_MaxDistanceFromCamera`))
    (if (not (`KismetArrayLibrary.Array_Contains` (`self.instancesWithActiveFallingLeaves`) _array_element))
      (`self.SpawnFallingLeaves_Idle` _array_element))))

(event `CheckIfCullIdleParticles`
  (bind _indexestoremove (`self.indexesToRemove`))
  ;[0.12 0.1054 0.0786] Check active idle falling leaf particles. If they're auto-self-destroyed already (it happens after X loops set in particle system), remove their indexes from the list. This way the next sphere check around camera will know that these instances don't have active particles anymore.
  (for (_array_element _array_index) (`self.ActiveFallingLeaves`)
    (`/Engine/EditorBlueprintResources/StandardMacros.IsValid` _array_element
      (:`Is Not Valid`
        (`KismetArrayLibrary.Array_Add` (`self.indexesToRemove`) _array_index))))
  (for _array_element_2 _indexestoremove
    (`KismetArrayLibrary.Array_Remove` (`self.ActiveFallingLeaves`) _array_element_2)
    (`KismetArrayLibrary.Array_Remove` (`self.instancesWithActiveFallingLeaves`) _array_element_2))
  (`KismetArrayLibrary.Array_Clear` _indexestoremove))

(event `/Game/Landscape/InTreeCreator/Blueprints/Internal/Choppable_BP.ReactToChoppingHit`
  (params (HitStrength :type "Float (single-precision)") (`'HitItem'` :type Integer))
  ;[0.07613 0.2 0.008186] Implementation of the chopping reaction function. In this case, turn a simple mesh instance into choppable tree blueprint.
  (if (`self.isChoppable`)
    (`self.TurnIntoChoppableBlueprint` HitStrength `'HitItem'`)))

(fn `SpawnDebrisFromImpulse`
  (params (InstanceIndex :type Integer) (ImpulseLocation :type "Vector Structure") (ImpulseStrength :type "Float (double-precision)") (ImpulseRadius :type "Float (double-precision)"))
  (locals (baseSpawnLocation :type "Vector Structure") (impulseInfluence :type "Float (double-precision)") (materialForDebris :type "MaterialInterface Object Reference") (detectedBarkMaterials :type "Array of MaterialInterface Object Reference") (detectedLeafMaterials :type "Array of MaterialInterface Object Reference"))
  (bind _detectedleafmaterials (`local.detectedLeafMaterials`))
  (bind _detectedbarkmaterials (`local.detectedBarkMaterials`))
  (bind (_returnvalue_origin _returnvalue_boxextent) (`KismetMathLibrary.BreakBoxSphereBounds` (`StaticMesh.GetBounds` (`self.StaticMesh`))))
  (bind (_returnvalue_origin_2 _returnvalue_boxextent_2) (`KismetMathLibrary.BreakBoxSphereBounds` (`StaticMesh.GetBounds` (`self.StaticMesh`))))
  ;[0 0 0] Calculate main location for debris spawn
  (if (`self.FallingDebris_Impulse_ON`)
    (set `local.baseSpawnLocation` (`KismetMathLibrary.MakeVector` (.x (.location (`self.GetInstanceTransform` (`local.InstanceIndex`) true))) (.y (.location (`self.GetInstanceTransform` (`local.InstanceIndex`) true))) (+ (.z (.location (`self.GetInstanceTransform` (`local.InstanceIndex`) true))) (* (* (.z (.scale (`self.GetInstanceTransform` (`local.InstanceIndex`) true))) 2.0 (.z _returnvalue_boxextent_2)) (`self.FallingDebris_Height`)))))
    ;[0.01 0.01 0.01] Calculate impulse influence on this particular instance.
    (set `local.impulseInfluence` (- 1.0 (/ (`KismetMathLibrary.VSize` (- (.location (`self.GetInstanceTransform` (`local.InstanceIndex`) true)) (`local.ImpulseLocation`))) (`local.ImpulseRadius`))))
    ;[0 0 0] Spawn assigned debris type.
    (for _array_element (`self.Debris`)
      (if (> (* (`local.ImpulseStrength`) 100.0 (`local.impulseInfluence`)) (`.MinimumImpulseStrengthToFall_24_E8128E614368B8C8F0F00B8186A73498` (break `/Game/Landscape/InTreeCreator/Blueprints/Internal/Misc/TreeDebris` _array_element)))
        (`|ExecutionSequence`
          (:`then_0`
            ;[0.005 0.005 0.005] Detect material assignment from the mesh by checking material name. User should name any custom materials accordingly, as stated in the documentation.
            (switch `/Game/Landscape/InTreeCreator/Blueprints/Internal/Misc/Bark_or_Leaves` (`.GetTexturesFrom_27_3714FF7D4E17CC99ED6E8BB0C5106141` (break `/Game/Landscape/InTreeCreator/Blueprints/Internal/Misc/TreeDebris` _array_element))
              (:`NewEnumerator0`
                (for _array_element_2 (`self.GetMaterials`)
                  (if (`KismetStringLibrary.Contains` (`KismetSystemLibrary.GetDisplayName` _array_element_2) "bark")
                    (`KismetArrayLibrary.Array_Add` (`local.detectedBarkMaterials`) _array_element_2)))
                (set `local.materialForDebris` (`|GetArrayItem` _detectedbarkmaterials (`KismetMathLibrary.RandomInteger` (`KismetArrayLibrary.Array_Length` _detectedbarkmaterials)))))
              (:`NewEnumerator1`
                (for _array_element_3 (`self.GetMaterials`)
                  (if (`KismetStringLibrary.Contains` (`KismetSystemLibrary.GetDisplayName` _array_element_3) "leaves")
                    (`KismetArrayLibrary.Array_Add` (`local.detectedLeafMaterials`) _array_element_3)))
                (set `local.materialForDebris` (`|GetArrayItem` _detectedleafmaterials (`KismetMathLibrary.RandomInteger` (`KismetArrayLibrary.Array_Length` _detectedleafmaterials)))))))
          (:`then_1`
            (bind ((`MinAmountFromImpulse_28_6DB3AC0440FDE171F2846A9B31ED7E60` _minamountfromimpulse) (`MaxAmountFromImpulse_29_D47D4A6643F4AE867D6C728C45C90585` _maxamountfromimpulse) (`MinAmountFromTreeFall_32_B3A2EA6C4CD7DB47DFC5ED8ABB860AF4` _minamountfromtreefall) (`MaxAmountFromTreeFall_34_613A4BDC4F63CD727E4B6EBBAE69D42C` _maxamountfromtreefall) (`Mesh_2_C8810A4845544D30D0BFF794769C1543` _mesh) (`Scale_Min_16_1965CF0A49A1287288DCDE85F06C78E1` _scale_min) (`Scale_Max_17_456C121441E1FF1FC0CB399CE083EBBE` _scale_max) (`Damping_20_487587934775CE17943BEFB9E5E0E927` _damping)) (break `/Game/Landscape/InTreeCreator/Blueprints/Internal/Misc/TreeDebris` _array_element))
            (for _ (range 1 (+ (`KismetMathLibrary.RandomIntegerInRange` _minamountfromimpulse _maxamountfromimpulse) 1))
              (`|SpawnActorFromClass` "/Game/Landscape/InTreeCreator/Blueprints/Internal/TreeDebris_BP.TreeDebris_BP_C" (`KismetMathLibrary.MakeTransform` (`KismetMathLibrary.RandomPointInBoundingBox` (`local.baseSpawnLocation`) (* _returnvalue_boxextent (`self.FallingDebris_AreaScale`))) (struct) (`KismetMathLibrary.Conv_DoubleToVector` (`KismetMathLibrary.RandomFloatInRange` _scale_min _scale_max))) "AlwaysSpawn" "OverrideRootScale" null _mesh (`local.materialForDebris`) (* (`KismetMathLibrary.Conv_RotatorToVector` (`KismetMathLibrary.FindLookAtRotation` (`local.ImpulseLocation`) (`local.baseSpawnLocation`))) (+ (* (`local.ImpulseStrength`) 10000.0 (`local.impulseInfluence`)) 100.0)) _damping null))))))))

(fn `SpawnFallingLeaves_Idle`
  (params (InstanceIndex :type Integer))
  (bind (_returnvalue_origin _returnvalue_boxextent) (`KismetMathLibrary.BreakBoxSphereBounds` (`StaticMesh.GetBounds` (`self.StaticMesh`))))
  ;[0.04678 0.1 0.028] Spawn falling leaf particles (idle version) in instance's location. For rotation, get current wind direction - this way the falling leaves will match current wind direction. Finally, add it to the array to be able to control it later.
  (bind _returnvalue (`KismetMaterialLibrary.GetVectorParameterValue` "/Game/Landscape/InTreeCreator/Materials/WindParameters.WindParameters" "WindDirection"))
  (bind _returnvalue_2 (`GameplayStatics.SpawnEmitterAtLocation` (`self.FallingLeaves_Idle`) (`KismetMathLibrary.MakeVector` (.x (.location (`self.GetInstanceTransform` (`local.InstanceIndex`) true))) (.y (.location (`self.GetInstanceTransform` (`local.InstanceIndex`) true))) (+ (.z (.location (`self.GetInstanceTransform` (`local.InstanceIndex`) true))) (* (* (.z (.scale (`self.GetInstanceTransform` (`local.InstanceIndex`) true))) 2.0 (.z _returnvalue_boxextent)) (`self.FallingLeaves_Height`)))) (`KismetMathLibrary.Conv_VectorToRotator` (`KismetMathLibrary.Conv_LinearColorToVector` _returnvalue))))
  (`KismetArrayLibrary.Array_Add` (`self.ActiveFallingLeaves`) _returnvalue_2)
  (`KismetArrayLibrary.Array_Add` (`self.instancesWithActiveFallingLeaves`) (`local.InstanceIndex`)))

(fn `SpawnFruitsFromImpulse`
  (params (InstanceIndex :type Integer) (ImpulseLocation :type "Vector Structure") (ImpulseStrength :type "Float (double-precision)") (ImpulseRadius :type "Float (double-precision)"))
  (locals (baseSpawnLocation :type "Vector Structure") (impulseInfluence :type "Float (double-precision)"))
  (bind (_value _returnvalue) (`BlueprintMapLibrary.Map_Find` (`self.instancesAndFallenFruitAmounts`) (`local.InstanceIndex`)))
  (bind (_returnvalue_origin _returnvalue_boxextent) (`KismetMathLibrary.BreakBoxSphereBounds` (`StaticMesh.GetBounds` (`self.StaticMesh`))))
  (bind (_returnvalue_origin_2 _returnvalue_boxextent_2) (`KismetMathLibrary.BreakBoxSphereBounds` (`StaticMesh.GetBounds` (`self.StaticMesh`))))
  (bind _returnvalue_2 (+ _value 1))
  ;[0 0 0] Check if the instance isn't depleted yet (out of fruits available to fall) - if not, calculate main location for fruit spawn
  (if (`self.hasFruits`)
    (if (not (`KismetArrayLibrary.Array_Contains` (`self.instancesWithDepletedFruits`) (`local.InstanceIndex`)))
      (set `local.baseSpawnLocation` (`KismetMathLibrary.MakeVector` (.x (.location (`self.GetInstanceTransform` (`local.InstanceIndex`) true))) (.y (.location (`self.GetInstanceTransform` (`local.InstanceIndex`) true))) (+ (.z (.location (`self.GetInstanceTransform` (`local.InstanceIndex`) true))) (* (* (.z (.scale (`self.GetInstanceTransform` (`local.InstanceIndex`) true))) 2.0 (.z _returnvalue_boxextent_2)) (`self.FallingFruits_Height`)))))
      ;[0.0239 0.04 0.0172] Calculate impulse force influence on this instance, based on location (distance)
      (set `local.impulseInfluence` (- 1.0 (/ (`KismetMathLibrary.VSize` (- (.location (`self.GetInstanceTransform` (`local.InstanceIndex`) true)) (`local.ImpulseLocation`))) (`local.ImpulseRadius`))))
      ;[0.01622 0.02 0.0111] For every assigned fruit type, spawn the right amount (random from user-specified range) with previously calculated spawn attributes.
      (for _array_element (`self.Fruits`)
        (if (> (* (`local.ImpulseStrength`) 100.0 (`local.impulseInfluence`)) (`.MinimumImpulseStrengthToFall_14_783AB18F40E1B59EC44985BCB5566C38` (break `/Game/Landscape/InTreeCreator/Blueprints/Internal/Misc/TreeFruits` _array_element)))
          (bind ((`FruitType_3_5BCD957F40EBABC216EDACBD6F230DDE` _fruittype) (`MinFallWith1Impulse_25_4640BF534AEF550DA74024A062F02B0D` _minfallwith1impulse) (`MaxFallWith1Impulse_23_0CD5084E4BA17F2A2A80669A5A286EB0` _maxfallwith1impulse) (`MinFallAfterTreeFall_29_BBBDAF29470C4FFA30E3FB9A50E35B76` _minfallaftertreefall) (`MaxFallAfterTreeFall_31_10BC133A42D98553A33AF6A68C2A4ECB` _maxfallaftertreefall) (`ScaleMin_17_9EE2CDB44A6FEBB39FB2228A5CE7AA98` _scalemin) (`ScaleMax_18_474A649249F62F449D2838BBFB6E09A5` _scalemax) (`Damping_20_9E9E0D6145B254CF2A2593B057088750` _damping)) (break `/Game/Landscape/InTreeCreator/Blueprints/Internal/Misc/TreeFruits` _array_element))
          (for _ (range 1 (+ (`KismetMathLibrary.RandomIntegerInRange` _minfallwith1impulse _maxfallwith1impulse) 1))
            (`|SpawnActorFromClass` _fruittype (`KismetMathLibrary.MakeTransform` (`KismetMathLibrary.RandomPointInBoundingBox` (`local.baseSpawnLocation`) (* _returnvalue_boxextent (`self.FallingFruits_AreaScale`))) (struct) (`KismetMathLibrary.Conv_DoubleToVector` (`KismetMathLibrary.RandomFloatInRange` _scalemin _scalemax))) "AlwaysSpawn" "OverrideRootScale" null (* (`KismetMathLibrary.Conv_RotatorToVector` (`KismetMathLibrary.FindLookAtRotation` (`local.ImpulseLocation`) (`local.baseSpawnLocation`))) (+ (* (`local.ImpulseStrength`) 10000.0 (`local.impulseInfluence`)) 100.0)) _damping null)
            ;[0.01 0.01 0.01] Using the Map variable type, find this instance in it and add the amount of spawned (fallen) fruits to it, to be able to track already fallen fruits for every instance.
            (if _returnvalue
              (`BlueprintMapLibrary.Map_Add` (`self.instancesAndFallenFruitAmounts`) (`local.InstanceIndex`) _returnvalue_2) ; Same key == overrides the previous value.
              (if (> _returnvalue_2 (`self.TotalLooseFruitsAmount`))
                (`KismetArrayLibrary.Array_AddUnique` (`self.instancesWithDepletedFruits`) (`local.InstanceIndex`)))
              (else
                (`BlueprintMapLibrary.Map_Add` (`self.instancesAndFallenFruitAmounts`) (`local.InstanceIndex`) 1) ; Same key == overrides the previous value.
              ))))))))

(fn `SpawnLeavesFromImpulse`
  (params (InstanceIndex :type Integer) (ImpulseLocation :type "Vector Structure"))
  (bind (_returnvalue_origin _returnvalue_boxextent) (`KismetMathLibrary.BreakBoxSphereBounds` (`StaticMesh.GetBounds` (`self.StaticMesh`))))
  (bind _location (.location (`self.GetInstanceTransform` (`local.InstanceIndex`) true)))
  ;[0.005 0.005 0.005] Spawn leaf particles at instance's location, with rotation that matches force direction.
  (if (`self.FallingLeaves_Impulse_ON`)
    (`GameplayStatics.SpawnEmitterAtLocation` (`self.FallingLeaves_Impulse`) (`KismetMathLibrary.MakeVector` (.x _location) (.y _location) (+ (.z _location) (* (* (.z _returnvalue_boxextent) 2.0 (.z (.scale (`self.GetInstanceTransform` (`local.InstanceIndex`) true)))) (`self.FallingLeaves_Height`)))) (`KismetMathLibrary.FindLookAtRotation` (`local.ImpulseLocation`) _location))))

(fn `TurnIntoChoppableBlueprint`
  (params (hitStrength :type "Float (double-precision)") (InstanceIndex :type Integer))
  (locals (transformOfOriginalInstance :type "Transform Structure"))
  ;[0.05523 0.15 0] Turn the instance into a choppable tree version by removing it and replacing with a blueprint. All the previously prepared properties are passed to it. After that, inform the choppable tree that it needs to react to the first chopping hit with certain strength.
  (set `local.transformOfOriginalInstance` (`self.GetInstanceTransform` InstanceIndex true))
  (`self.RemoveInstance` (`local.InstanceIndex`))
  (bind _returnvalue (`|SpawnActorFromClass` "/Game/Landscape/InTreeCreator/Blueprints/Internal/ChoppableTree_BP.ChoppableTree_BP_C" (`local.transformOfOriginalInstance`) "AlwaysSpawn" "OverrideRootScale" null (`self.choppedTopMesh`) (`self.choppedBottomMesh`) (`self.chopInfo`) (`self.chopHP`) (`self.InteriorMaterial`) (`self.chopping_FallingDebris`) (`self.chopping_FallingDebris_ChancePerHit`) (`self.FallingDebris_Height`) (`self.FallingDebris_AreaScale`) (`self.fullChopImpactParticles`) (`self.hasFruits`) (`self.Fruits`) (`self.FallingFruits_Height`) (`self.FallingFruits_AreaScale`) (`self.fallShakeStrength`) null))
  (`/Game/Landscape/InTreeCreator/Blueprints/Internal/ChoppableTree_BP.ReactToChoppingHit` _returnvalue (`local.hitStrength`) 0))