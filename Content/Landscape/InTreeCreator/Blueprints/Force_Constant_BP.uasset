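; Force_Constant_BP is a placeable actor that applies a constant force through the level's TreeManager_BP.
; On BeginPlay it finds the manager and registers itself with strength, radius and startup speed, saving the returned channel index.
; It destroys itself if registration fails, and prints a warning if no manager exists.
; TurnOff frees the channel through the manager, either when called or automatically after an optional delay.
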(event `self.ReceiveBeginPlay`
  ;[0.01 0.01 0.01] Find tree manager an assign it to a variable, to access it later. If not found, display a proper message.
  (bind _outactors (`GameplayStatics.GetAllActorsOfClass` "/Game/Landscape/InTreeCreator/Blueprints/TreeManager_BP.TreeManager_BP_C"))
  (bind _output_get (set `self.treeManager` (`|GetArrayItem` _outactors)))
  (`/Engine/EditorBlueprintResources/StandardMacros.IsValid` _output_get
    (:`Is Valid`
      ;[0.01 0.01 0.01] Using the previously detected tree manager, register this constant force.
      ; Then save the channel index to be able to free it up after it's turned off.
      (bind (_success _usedchannel) (`/Game/Landscape/InTreeCreator/Blueprints/TreeManager_BP.AddConstantForce` (`self.treeManager`) self (`self.Strength`) (`self.Radius`) (`self.StartupSpeed`)))
      (if _success
        (set `self.channelIndex` _usedchannel)
        ;[0.01 0.01 0.01] If this force should be turned off after X seconds, do it after X second delay.
        (if (!= (`self.TurnOffAfterSeconds`) 0.0)
          (`KismetSystemLibrary.Delay` (`self.TurnOffAfterSeconds`))
          (`self.TurnOff`))
        (else
          (`self.K2_DestroyActor`))))
    (:`Is Not Valid`
      (`KismetSystemLibrary.PrintString` "Tree Manager not found. Please add Tree Manager to your scene." true true (struct :`R` 0.55 :`G` 0.105488 :`A` 1.0) 15.0))))

(event `TurnOff`
  ;[0.005 0.005 0.005] Turn off this force by registering this event in the tree manager. Pass the saved channel index to free up this channel via tree manager.
  (`/Game/Landscape/InTreeCreator/Blueprints/TreeManager_BP.TurnOffConstantForce` (`self.treeManager`) (`self.channelIndex`)))

(fn `UserConstructionScript`)