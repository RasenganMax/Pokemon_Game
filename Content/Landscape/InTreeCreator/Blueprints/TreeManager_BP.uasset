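; TreeManager feeds impulse and constant forces to tree bark and leaf materials through the ForceParameters material parameter collection.
; AddImpulse and AddConstantForce each reserve one of three shared channels, failing if none is free.
; Impulses animate strength with a timeline curve, then free their channel.
; Constant forces track an actor by looping timer and ramp strength; turning one off ramps again, frees the channel and destroys that actor.
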(event `Play Impulse`
  (params (atChannel :type Integer))
  (switch `int` atChannel
    (:`0`
      ;[0.005 0.005 0.005] Impulse animation - channel 1
      (`TimelineComponent.SetPlayRate` (`self.ImpulseAnim_Channel1`) 0.25)
      (`TimelineComponent.SetFloatCurve` (`self.ImpulseAnim_Channel1`) "/Game/Landscape/InTreeCreator/Blueprints/Internal/Misc/ImpulseCurve4.ImpulseCurve4" "Anim")
      (`KismetMaterialLibrary.SetVectorParameterValue` "/Game/Landscape/InTreeCreator/Materials/ForceParameters.ForceParameters" "Force1_Loc" (`KismetMathLibrary.Conv_VectorToLinearColor` (`self.force1_Loc`)))
      (`KismetMaterialLibrary.SetScalarParameterValue` "/Game/Landscape/InTreeCreator/Materials/ForceParameters.ForceParameters" "Force1_Radius" (`self.force1_Radius`))
      (bind (_direction _anim _radiusgrowth) (`Timeline|ImpulseAnim_Channel1` :!via `PlayFromStart`)
        (:`Update`
          (`KismetMaterialLibrary.SetScalarParameterValue` "/Game/Landscape/InTreeCreator/Materials/ForceParameters.ForceParameters" "Force1_Strength" (* _anim (`self.force1_Strength`))))
        (:`Finished`
          (`self.MarkForceChannelAsFree` 0))))
    (:`1`
      ;[0.005 0.005 0.005] Impulse animation - channel 2
      (`TimelineComponent.SetPlayRate` (`self.ImpulseAnim_Channel2`) 0.25)
      (`TimelineComponent.SetFloatCurve` (`self.ImpulseAnim_Channel2`) "/Game/Landscape/InTreeCreator/Blueprints/Internal/Misc/ImpulseCurve4.ImpulseCurve4" "Anim")
      (`KismetMaterialLibrary.SetVectorParameterValue` "/Game/Landscape/InTreeCreator/Materials/ForceParameters.ForceParameters" "Force2_Loc" (`KismetMathLibrary.Conv_VectorToLinearColor` (`self.force2_Loc`)))
      (`KismetMaterialLibrary.SetScalarParameterValue` "/Game/Landscape/InTreeCreator/Materials/ForceParameters.ForceParameters" "Force2_Radius" (`self.force2_Radius`))
      (bind (_direction_2 _anim_2 _radiusgrowth_2) (`Timeline|ImpulseAnim_Channel2` :!via `PlayFromStart`)
        (:`Update`
          (`KismetMaterialLibrary.SetScalarParameterValue` "/Game/Landscape/InTreeCreator/Materials/ForceParameters.ForceParameters" "Force2_Strength" (* _anim_2 (`self.force2_Strength`))))
        (:`Finished`
          (`self.MarkForceChannelAsFree` 1))))
    (:`2`
      ;[0.005 0.005 0.005] Impulse animation - channel 3
      (`TimelineComponent.SetPlayRate` (`self.ImpulseAnim_Channel3`) 0.25)
      (`TimelineComponent.SetFloatCurve` (`self.ImpulseAnim_Channel3`) "/Game/Landscape/InTreeCreator/Blueprints/Internal/Misc/ImpulseCurve4.ImpulseCurve4" "Anim")
      (`KismetMaterialLibrary.SetVectorParameterValue` "/Game/Landscape/InTreeCreator/Materials/ForceParameters.ForceParameters" "Force3_Loc" (`KismetMathLibrary.Conv_VectorToLinearColor` (`self.force3_Loc`)))
      (`KismetMaterialLibrary.SetScalarParameterValue` "/Game/Landscape/InTreeCreator/Materials/ForceParameters.ForceParameters" "Force3_Radius" (`self.force3_Radius`))
      (bind (_direction_3 _anim_3 _radiusgrowth_3) (`Timeline|ImpulseAnim_Channel3` :!via `PlayFromStart`)
        (:`Update`
          (`KismetMaterialLibrary.SetScalarParameterValue` "/Game/Landscape/InTreeCreator/Materials/ForceParameters.ForceParameters" "Force3_Strength" (* _anim_3 (`self.force3_Strength`))))
        (:`Finished`
          (`self.MarkForceChannelAsFree` 2))))))

(event `UpdateConstForceLoc_Channel1`
  ;[0.005 0.005 0.005] Constant force - channel 1
  (`KismetMaterialLibrary.SetVectorParameterValue` "/Game/Landscape/InTreeCreator/Materials/ForceParameters.ForceParameters" "Force1_Loc" (`KismetMathLibrary.Conv_VectorToLinearColor` (`self.K2_GetActorLocation` (`self.constForce1_Actor`)))))

(event `UpdateForceLocation`
  ;[0.03257 0.26 0.02613] Optional - Smoothly changing force location to prevent unnatural immediate bend direction snap for trees.
  (set `self.currentLoc` (`self.K2_GetActorLocation`))
  (bind (_direction _alpha) (`Timeline|Lerp` :!via `PlayFromStart`)
    (:`Update`
      (bind _returnvalue (`KismetMathLibrary.VLerp` (`self.lastLoc`) (`self.currentLoc`) _alpha))
      (`KismetMaterialLibrary.SetVectorParameterValue` "/Game/Landscape/InTreeCreator/Materials/ForceParameters.ForceParameters" "Force1_Loc" (`KismetMathLibrary.Conv_VectorToLinearColor` _returnvalue)))
    (:`Finished`
      (set `self.lastLoc` _returnvalue))))

(event `StartConstantForce`
  (params (atChannel :type Integer))
  (switch `int` atChannel
    (:`0`
      ;[0.005 0.005 0.005] Constant force - channel 1
      (`KismetMaterialLibrary.SetScalarParameterValue` "/Game/Landscape/InTreeCreator/Materials/ForceParameters.ForceParameters" "Force1_Radius" (`self.constForce1_Radius`))
      (`|ExecutionSequence`
        (:`then_0`
          (bind _returnvalue (`KismetSystemLibrary.K2_SetTimerDelegate` (delegate `UpdateConstForceLoc_Channel1`) 0.02 true))
          (set `self.timer_UpdateConstForceLoc1` _returnvalue))
        (:`then_1`
          (`TimelineComponent.SetPlayRate` (`self.ConstForce1_TurnOn`) (`self.constForce1_StartSpeed`))
          (bind (_direction _alpha) (`Timeline|ConstForce1_TurnOn` :!via `PlayFromStart`)
            (:`Update`
              (`KismetMaterialLibrary.SetScalarParameterValue` "/Game/Landscape/InTreeCreator/Materials/ForceParameters.ForceParameters" "Force1_Strength" (* _alpha (`self.constForce1_Strength`))))))))
    (:`1`
      ;[0.005 0.005 0.005] Constant force - channel 2
      (`KismetMaterialLibrary.SetScalarParameterValue` "/Game/Landscape/InTreeCreator/Materials/ForceParameters.ForceParameters" "Force2_Radius" (`self.constForce2_Radius`))
      (`|ExecutionSequence`
        (:`then_0`
          (bind _returnvalue_2 (`KismetSystemLibrary.K2_SetTimerDelegate` (delegate `UpdateConstForceLoc_Channel2`) 0.02 true))
          (set `self.timer_UpdateConstForceLoc2` _returnvalue_2))
        (:`then_1`
          (`TimelineComponent.SetPlayRate` (`self.ConstForce2_TurnOn`) (`self.constForce2_StartSpeed`))
          (bind (_direction_2 _alpha_2) (`Timeline|ConstForce2_TurnOn` :!via `PlayFromStart`)
            (:`Update`
              (`KismetMaterialLibrary.SetScalarParameterValue` "/Game/Landscape/InTreeCreator/Materials/ForceParameters.ForceParameters" "Force2_Strength" (* _alpha_2 (`self.constForce2_Strength`))))))))
    (:`2`
      ;[0.005 0.005 0.005] Constant force - channel 3
      (`KismetMaterialLibrary.SetScalarParameterValue` "/Game/Landscape/InTreeCreator/Materials/ForceParameters.ForceParameters" "Force3_Radius" (`self.constForce3_Radius`))
      (`|ExecutionSequence`
        (:`then_0`
          (bind _returnvalue_3 (`KismetSystemLibrary.K2_SetTimerDelegate` (delegate `UpdateConstForceLoc_Channel3`) 0.02 true))
          (set `self.timer_UpdateConstForceLoc3` _returnvalue_3))
        (:`then_1`
          (`TimelineComponent.SetPlayRate` (`self.ConstForce3_TurnOn`) (`self.constForce3_StartSpeed`))
          (bind (_direction_3 _alpha_3) (`Timeline|ConstForce3_TurnOn` :!via `PlayFromStart`)
            (:`Update`
              (`KismetMaterialLibrary.SetScalarParameterValue` "/Game/Landscape/InTreeCreator/Materials/ForceParameters.ForceParameters" "Force3_Strength" (* _alpha_3 (`self.constForce3_Strength`))))))))))

(event `UpdateConstForceLoc_Channel2`
  ;[0.005 0.005 0.005] Constant force - channel 2
  (`KismetMaterialLibrary.SetVectorParameterValue` "/Game/Landscape/InTreeCreator/Materials/ForceParameters.ForceParameters" "Force2_Loc" (`KismetMathLibrary.Conv_VectorToLinearColor` (`self.K2_GetActorLocation` (`self.constForce2_Actor`)))))

(event `UpdateConstForceLoc_Channel3`
  ;[0.005 0.005 0.005] Constant force - channel 3
  (`KismetMaterialLibrary.SetVectorParameterValue` "/Game/Landscape/InTreeCreator/Materials/ForceParameters.ForceParameters" "Force3_Loc" (`KismetMathLibrary.Conv_VectorToLinearColor` (`self.K2_GetActorLocation` (`self.constForce3_Actor`)))))

(event `TurnOffConstantForce`
  (params (channelIndex :type Integer))
  (switch `int` channelIndex
    (:`0`
      ;[0.005 0.005 0.005] Constant force OFF - channel 1
      (`KismetSystemLibrary.K2_ClearAndInvalidateTimerHandle` (`self.timer_UpdateConstForceLoc1`))
      (`TimelineComponent.SetPlayRate` (`self.ConstForce1_TurnOff`) (`self.constForce1_StartSpeed`))
      (bind (_direction _alpha) (`Timeline|ConstForce1_TurnOff` :!via `PlayFromStart`)
        (:`Update`
          (`KismetMaterialLibrary.SetScalarParameterValue` "/Game/Landscape/InTreeCreator/Materials/ForceParameters.ForceParameters" "Force1_Strength" (* _alpha (`self.constForce1_Strength`))))
        (:`Finished`
          (`self.MarkForceChannelAsFree` 0)
          (`self.K2_DestroyActor` (`self.constForce1_Actor`)))))
    (:`1`
      ;[0.005 0.005 0.005] Constant force OFF - channel 2
      (`KismetSystemLibrary.K2_ClearAndInvalidateTimerHandle` (`self.timer_UpdateConstForceLoc2`))
      (`TimelineComponent.SetPlayRate` (`self.ConstForce2_TurnOff`) (`self.constForce2_StartSpeed`))
      (bind (_direction_2 _alpha_2) (`Timeline|ConstForce2_TurnOff` :!via `PlayFromStart`)
        (:`Update`
          (`KismetMaterialLibrary.SetScalarParameterValue` "/Game/Landscape/InTreeCreator/Materials/ForceParameters.ForceParameters" "Force2_Strength" (* _alpha_2 (`self.constForce2_Strength`))))
        (:`Finished`
          (`self.MarkForceChannelAsFree` 1)
          (`self.K2_DestroyActor` (`self.constForce2_Actor`)))))
    (:`2`
      ;[0.005 0.005 0.005] Constant force OFF - channel 3
      (`KismetSystemLibrary.K2_ClearAndInvalidateTimerHandle` (`self.timer_UpdateConstForceLoc3`))
      (`TimelineComponent.SetPlayRate` (`self.ConstForce3_TurnOff`) (`self.constForce3_StartSpeed`))
      (bind (_direction_3 _alpha_3) (`Timeline|ConstForce3_TurnOff` :!via `PlayFromStart`)
        (:`Update`
          (`KismetMaterialLibrary.SetScalarParameterValue` "/Game/Landscape/InTreeCreator/Materials/ForceParameters.ForceParameters" "Force3_Strength" (* _alpha_3 (`self.constForce3_Strength`))))
        (:`Finished`
          (`self.MarkForceChannelAsFree` 2)
          (`self.K2_DestroyActor` (`self.constForce3_Actor`)))))))

(fn `AddConstantForce`
  (params (AtActor :type "Actor Object Reference") (Strength :type "Float (double-precision)") (Radius :type "Float (double-precision)") (StartupSpeed :type "Float (double-precision)"))
  (returns (Success :type Boolean) (usedChannel :type Integer))
  ;[0.015 0.015 0.015] First, get free force channel. If found, register the new force into the proper variables, taking into account also its strength, radius and start speed.
  (bind (_found _indexofchannel) (`self.GetFreeForceChannel`))
  (if _found
    (switch `int` _indexofchannel
      (:`0`
        (set `self.constForce1_Actor` (`local.AtActor`))
        (set `self.constForce1_Strength` (`local.Strength`))
        (set `self.constForce1_Radius` (`local.Radius`))
        (set `self.constForce1_StartSpeed` (`local.StartupSpeed`))
        (`self.StartConstantForce` 0)
        (return true 0))
      (:`1`
        (set `self.constForce2_Actor` (`local.AtActor`))
        (set `self.constForce2_Strength` (`local.Strength`))
        (set `self.constForce2_Radius` (`local.Radius`))
        (set `self.constForce2_StartSpeed` (`local.StartupSpeed`))
        (`self.StartConstantForce` 1)
        (return true 1))
      (:`2`
        (set `self.constForce3_Actor` (`local.AtActor`))
        (set `self.constForce3_Strength` (`local.Strength`))
        (set `self.constForce3_Radius` (`local.Radius`))
        (set `self.constForce3_StartSpeed` (`local.StartupSpeed`))
        (`self.StartConstantForce` 2)
        (return true 2)))
    (else
      (return false 0))))

(fn `AddImpulse`
  (params (Location :type "Vector Structure") (Strength :type "Float (double-precision)") (Radius :type "Float (double-precision)"))
  (returns (Success :type Boolean) (usedChannel :type Integer))
  ;[0.03246 0.06585 0.11] First, get free force channel. If found, register the new force into the proper variables, taking into account also its strength & radius.
  (bind (_found _indexofchannel) (`self.GetFreeForceChannel`))
  (if _found
    (switch `int` _indexofchannel
      (:`0`
        (set `self.force1_Loc` (`local.Location`))
        (set `self.force1_Strength` (`local.Strength`))
        (set `self.force1_Radius` (`local.Radius`))
        (`self.Play Impulse` 0)
        (return true 0))
      (:`1`
        (set `self.force2_Loc` (`local.Location`))
        (set `self.force2_Strength` (`local.Strength`))
        (set `self.force2_Radius` (`local.Radius`))
        (`self.Play Impulse` 1)
        (return true 1))
      (:`2`
        (set `self.force3_Loc` (`local.Location`))
        (set `self.force3_Strength` (`local.Strength`))
        (set `self.force3_Radius` (`local.Radius`))
        (`self.Play Impulse` 2)
        (return true 2)))
    (else
      (return false 0))))

(fn `GetFreeForceChannel`
  (returns (Found :type Boolean) (indexOfChannel :type Integer))
  (locals (indexOfFoundChannel :type Integer))
  ;[0.0612 0.1183 0.255] Gets free force channel to 'reserve' it for newly registered force. If there's no free channel, return a proper warning to user. If found, return index of found channel to be able to free it up later.
  (bind _output_get (set `local.indexOfFoundChannel` (`KismetArrayLibrary.Array_Find` (`self.freeForceChannels`) true)))
  (if (!= _output_get -1)
    (`KismetArrayLibrary.Array_Set` (`self.freeForceChannels`) (`local.indexOfFoundChannel`))
    (return true (`local.indexOfFoundChannel`))
    (else
      (`KismetSystemLibrary.PrintString` "Couldn't find a free force channel. If you want to have more forces \nworking simultaneously, please add more channels in TreeManager \nblueprint and in the main materials for bark and leaves. \nYou can find more info in the starter guide. \nIf you have problems with setting this up, please contact me  \non the support email or in the forum thread." true true (struct :`R` 0.54 :`G` 0.034075 :`A` 1.0) 20.0)
      (return false -1))))

(fn `MarkForceChannelAsFree`
  (params (indexOfChannel :type Integer))
  ;[0.05476 0.245 0.01888] Marking force channel as free allows other forces to register themselves as active.
  (`KismetArrayLibrary.Array_Set` (`self.freeForceChannels`) indexOfChannel true))

(fn `UserConstructionScript`)