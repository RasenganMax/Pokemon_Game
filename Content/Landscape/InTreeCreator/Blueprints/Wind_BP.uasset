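; Wind actor that drives global wind direction and strength through the WindParameters material parameter collection.
; Construction script and BeginPlay write the Strength property and the actor's forward vector into the collection, so editor placement and rotation set the wind.
; ChangeDirection and ChangeStrength events read the current value, then use duration-scaled timelines to lerp smoothly to a new one.
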(event `ChangeDirection`
  (params (newDirection :type "Vector Structure") (changeDuration :type "Float (double-precision)" :default 3.0))
  ;[0 0.3173 1] Smoothly change wind direction, with user specified duration & new direction.
  (set `self.newDirection_` (`KismetMathLibrary.Conv_VectorToLinearColor` newDirection))
  (set `self.directionChangeDuration` changeDuration)
  (bind _returnvalue (`KismetMaterialLibrary.GetVectorParameterValue` "/Game/Landscape/InTreeCreator/Materials/WindParameters.WindParameters" "WindDirection"))
  (set `self.oldDirection` _returnvalue)
  (`TimelineComponent.SetPlayRate` (`self.DirectionChange`) (/ 1.0 (`self.directionChangeDuration`)))
  (bind (_direction _alpha) (`Timeline|DirectionChange` :!via `PlayFromStart`)
    (:`Update`
      (`KismetMaterialLibrary.SetVectorParameterValue` "/Game/Landscape/InTreeCreator/Materials/WindParameters.WindParameters" "WindDirection" (`KismetMathLibrary.LinearColorLerp` (`self.oldDirection`) (`self.newDirection_`) _alpha)))))

(event `ChangeStrength`
  (params (newStrength :type "Float (double-precision)" :default 0.7) (changeDuration :type "Float (double-precision)" :default 3.0))
  ;[0 0.3173 1] Smoothly change wind strength, with user specified duration & new strength.
  (set `self.newStrength` newStrength)
  (set `self.strengthChangeDuration` changeDuration)
  (bind _returnvalue (`KismetMaterialLibrary.GetScalarParameterValue` "/Game/Landscape/InTreeCreator/Materials/WindParameters.WindParameters" "WindStrength"))
  (set `self.oldStrength` _returnvalue)
  (`TimelineComponent.SetPlayRate` (`self.StrengthChange`) (/ 1.0 (`self.strengthChangeDuration`)))
  (bind (_direction _alpha) (`Timeline|StrengthChange` :!via `PlayFromStart`)
    (:`Update`
      (`KismetMaterialLibrary.SetScalarParameterValue` "/Game/Landscape/InTreeCreator/Materials/WindParameters.WindParameters" "WindStrength" (`KismetMathLibrary.Lerp` (`self.oldStrength`) (`self.newStrength`) _alpha)))))

(event `self.ReceiveBeginPlay`
  ;[0.1876 0.447 1] At game begin, set strength and direction by using current wind actor rotation and strength property.
  (`KismetMaterialLibrary.SetScalarParameterValue` "/Game/Landscape/InTreeCreator/Materials/WindParameters.WindParameters" "WindStrength" (`self.Strength`))
  (`KismetMaterialLibrary.SetVectorParameterValue` "/Game/Landscape/InTreeCreator/Materials/WindParameters.WindParameters" "WindDirection" (`KismetMathLibrary.Conv_VectorToLinearColor` (`self.GetActorForwardVector`))))

(fn `UserConstructionScript`
  ;[0.1876 0.447 1] Useful for in-editor wind manipulation. Set strength and direction by using current wind actor rotation and strength property.
  (`KismetMaterialLibrary.SetScalarParameterValue` "/Game/Landscape/InTreeCreator/Materials/WindParameters.WindParameters" "WindStrength" (`self.Strength`))
  (`KismetMaterialLibrary.SetVectorParameterValue` "/Game/Landscape/InTreeCreator/Materials/WindParameters.WindParameters" "WindDirection" (`KismetMathLibrary.Conv_VectorToLinearColor` (`self.GetActorForwardVector`))))