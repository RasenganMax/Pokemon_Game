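; Force_Impulse_BP is a one-shot impulse actor that disturbs interactive foliage trees around its location.
; On BeginPlay it registers location, strength and radius with the level's TreeManager_BP, printing a warning if none exists.
; A multi sphere trace finds FoliageComp_Tree_BP instances, each spawning leaves, debris and fruits once, deduplicated by component and instance index.
; The actor then destroys itself.
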(event `self.ReceiveBeginPlay`
  (bind _returnvalue (`self.K2_GetActorLocation`))
  (`|ExecutionSequence`
    (:`then_0`
      ;[0.01 0.01 0.01] Find tree manager an assign it to a variable, to access it later. If not found, display a proper message.
      (bind _outactors (`GameplayStatics.GetAllActorsOfClass` "/Game/Landscape/InTreeCreator/Blueprints/TreeManager_BP.TreeManager_BP_C"))
      (bind _output_get (set `self.treeManager` (`|GetArrayItem` _outactors)))
      (`/Engine/EditorBlueprintResources/StandardMacros.IsValid` _output_get
        (:`Is Valid`
          ;[0.01 0.01 0.01] Using the previously detected tree manager, register this force.
          (`/Game/Landscape/InTreeCreator/Blueprints/TreeManager_BP.AddImpulse` (`self.treeManager`) (`self.K2_GetActorLocation`) (`self.Strength`) (`self.Radius`)))
        (:`Is Not Valid`
          (`KismetSystemLibrary.PrintString` "Tree Manager not found. Please add Tree Manager to your scene." true true (struct :`R` 0.55 :`G` 0.105488 :`A` 1.0) 15.0))))
    (:`then_1`
      ;[0.005 0.005 0.005] Detect any interactive trees by multi sphere trace. 'Already Detected Instances' array is used to prevent multi-detecting the same instance more than once.
      (bind _outhits (`KismetSystemLibrary.SphereTraceMulti` _returnvalue (+ _returnvalue (0.0 0.0 1.0)) (`self.Radius`) "TraceTypeQuery1"))
      (for _array_element _outhits
        (bind (_bblockinghit _binitialoverlap _time _distance _location _impactpoint _normal _impactnormal _physmat _hitactor _hitcomponent _hitbonename _hititem) (`GameplayStatics.BreakHitResult` _array_element))
        (bind _asfoliage_comp_tree_bp (cast `/Game/Landscape/InTreeCreator/Blueprints/Internal/FoliageComp_Tree_BP` _hitcomponent)
          (:`then`
            (set `self.detectedTreeComp` _asfoliage_comp_tree_bp)
            (set `self.hitItem` _hititem)
            (if (not (`KismetArrayLibrary.Array_Contains` (`self.alreadyDetectedInstances_`) (make `/Game/Landscape/InTreeCreator/Blueprints/Internal/Misc/FoliageCompAndInstanceIndex` (`self.detectedTreeComp`) (`self.hitItem`))))
              ;[0.005 0.005 0.005] Spawn leaves, debris and fruits from the detected tree instance, using the assigned force location, strength and radius.
              (`/Game/Landscape/InTreeCreator/Blueprints/Internal/FoliageComp_Tree_BP.SpawnLeavesFromImpulse` (`self.detectedTreeComp`) (`self.hitItem`) (`self.K2_GetActorLocation`))
              (`/Game/Landscape/InTreeCreator/Blueprints/Internal/FoliageComp_Tree_BP.SpawnDebrisFromImpulse` (`self.detectedTreeComp`) (`self.hitItem`) (`self.K2_GetActorLocation`) (`self.Strength`) (`self.Radius`))
              (`/Game/Landscape/InTreeCreator/Blueprints/Internal/FoliageComp_Tree_BP.SpawnFruitsFromImpulse` (`self.detectedTreeComp`) (`self.hitItem`) (`self.K2_GetActorLocation`) (`self.Strength`) (`self.Radius`))
              ;[0.15 0.127 0.093] Add the detected tree instance to the array. It is used to prevent multi-detecting the same instance many times.
              (`KismetArrayLibrary.Array_Add` (`self.alreadyDetectedInstances_`) (make `/Game/Landscape/InTreeCreator/Blueprints/Internal/Misc/FoliageCompAndInstanceIndex` (`self.detectedTreeComp`) (`self.hitItem`)))))
          (:`CastFailed`
            (`KismetSystemLibrary.PrintString` "Marketplace guidelines." false false (struct :`G` 0.66 :`B` 1.0 :`A` 1.0) 1.0) ; Not needed, but required.
          ))))
    (:`then_2`
      (`self.K2_DestroyActor`) ; Destroy it after it's no longer needed.
    )))

(fn `UserConstructionScript`)