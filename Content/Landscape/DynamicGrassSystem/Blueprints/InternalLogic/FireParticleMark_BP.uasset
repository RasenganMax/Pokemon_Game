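; FireParticleMark_BP is a marker actor in the dynamic grass system that limits how densely fire particle marks cluster.
; The construction script sizes its collider sphere from CheckRadius.
; CheckDensity counts overlapping marks of the same class, returning whether the count stays within MaxDensity.
; The same check schedules self-destruction: accepted marks persist for a while before cleanup, while excess marks are removed almost immediately.
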(event `DestroyAfterDelay`
  (params (Delay :type "Float (double-precision)"))
  ;[1 1 1] Destroy the mark after delay, to prevent leaving many unused marks.
  (`KismetSystemLibrary.Delay` Delay)
  (`self.K2_DestroyActor`))

(fn `CheckDensity`
  (returns (OK_ToSpawn :type Boolean))
  (bind _returnvalue (<= (`KismetArrayLibrary.Array_Length` (`PrimitiveComponent.GetOverlappingActors` (`self.Collider`) "FireParticleMark_BP_C")) (`self.maxDensity`)))
  ;[1 1 1] Check how many other marks it overlaps and compare it with the 'Max Density' value.
  (`self.DestroyAfterDelay` (`KismetMathLibrary.SelectFloat` 30.0 0.01 _returnvalue))
  (return _returnvalue))

(fn `UserConstructionScript`
  ;[1 1 1] Set the mark radius.
  (`SphereComponent.SetSphereRadius` (`self.Collider`) (`self.checkRadius`) false))