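; Temporary actor for one burning foliage instance in the dynamic grass system, handling its burn effects and fire propagation.
; Spawns wind-driven fire and smoke plus a burnt-ground decal, each optionally density-limited by mark actors.
; Timelines drive a dissolve or shrink burn with lean, sampled on a timer slowed by camera distance.
; After a random delay it spawns a FireStarter within propagation limits, then self-destructs, optionally leaving an instanced burnt mesh.
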(event `self.ReceiveBeginPlay`
  (bind _manager (`self.manager`))
  (bind _manager_2 (`self.manager`))
  (bind _ownercomponent (`self.ownerComponent`))
  (bind _manager_3 (`self.manager`))
  (bind _ownercomponent_2 (`self.ownerComponent`))
  (bind _ownercomponent_3 (`self.ownerComponent`))
  (bind _ownercomponent_4 (`self.ownerComponent`))
  (bind _ownercomponent_5 (`self.ownerComponent`))
  (bind _manager_4 (`self.manager`))
  (bind _manager_5 (`self.manager`))
  (bind _manager_6 (`self.manager`))
  (bind _burntgroundmaterial__materialinstance (break `/Game/Landscape/DynamicGrassSystem/Blueprints/InternalLogic/MaterialInstance_Struct` (`/Game/Landscape/DynamicGrassSystem/Blueprints/InternalLogic/INTERACTIVE_FoliageComp_BP.burntGroundMaterial_` _ownercomponent_2)))
  (bind _dissolvemask__texture (break `/Game/Landscape/DynamicGrassSystem/Blueprints/InternalLogic/Texture2D_Struct` (`/Game/Landscape/DynamicGrassSystem/Blueprints/InternalLogic/INTERACTIVE_FoliageComp_BP.dissolveMask_` (`self.ownerComponent`))))
  (bind _firescale (`/Game/Landscape/DynamicGrassSystem/Blueprints/InternalLogic/INTERACTIVE_FoliageComp_BP.fireScale` _ownercomponent_4))
  (bind _returnvalue (`KismetMathLibrary.FClamp` (* (`/Game/Landscape/DynamicGrassSystem/Blueprints/InteractiveGrassManager_BP.BurnUpdateInterval` _manager_3) (* (`/Game/Landscape/DynamicGrassSystem/Blueprints/InternalLogic/INTERACTIVE_FoliageComp_BP.BurnDuration` (`self.ownerComponent`)) 0.1)) 0.04))
  (`|ExecutionSequence`
    (:`then_0`
      ;[1 1 1] Spawn burnt ground decal - and if optimization is enabled, first check if it's ok to spawn it (if it's not too dense)
      (if (`/Game/Landscape/DynamicGrassSystem/Blueprints/InternalLogic/INTERACTIVE_FoliageComp_BP.leaveBurntGround` (`self.ownerComponent`))
        (if (`/Game/Landscape/DynamicGrassSystem/Blueprints/InteractiveGrassManager_BP.OptimizeBurntGround` _manager_2)
          (bind _returnvalue_2 (`|SpawnActorFromClass` "/Game/Landscape/DynamicGrassSystem/Blueprints/InternalLogic/BurntGroundMark_BP.BurntGroundMark_BP_C" (`self.GetTransform`) "AlwaysSpawn" "OverrideRootScale" null (`/Game/Landscape/DynamicGrassSystem/Blueprints/InteractiveGrassManager_BP.OptimizeBurntGround_CheckRadius` _manager_2) (`/Game/Landscape/DynamicGrassSystem/Blueprints/InteractiveGrassManager_BP.OptimizeBurntGround_maxOverlapping` _manager_2) null))
          (bind _ok_tospawn (`/Game/Landscape/DynamicGrassSystem/Blueprints/InternalLogic/BurntGroundMark_BP.CheckDensity` _returnvalue_2))
          (if _ok_tospawn
            (`|SpawnActorFromClass` "/Game/Landscape/DynamicGrassSystem/Blueprints/InternalLogic/BurntGround_DECAL_BP.BurntGround_DECAL_BP_C" (`KismetMathLibrary.Conv_VectorToTransform` (`self.K2_GetActorLocation`)) "AlwaysSpawn" "OverrideRootScale" null (`/Game/Landscape/DynamicGrassSystem/Blueprints/InternalLogic/INTERACTIVE_FoliageComp_BP.BurnDuration` (`self.ownerComponent`)) (`self.manager`) (`/Game/Landscape/DynamicGrassSystem/Blueprints/InternalLogic/INTERACTIVE_FoliageComp_BP.burntGround_Scale` _ownercomponent_2) (`/Game/Landscape/DynamicGrassSystem/Blueprints/InternalLogic/INTERACTIVE_FoliageComp_BP.burntGround_ScaleRandomization` _ownercomponent_2) _burntgroundmaterial__materialinstance null :!label _label))
          (else
            (goto _label)))))
    (:`then_1`
      ;[1 1 1] Spawn smoke particle - and if optimization is enabled, first check if it's ok to spawn it (if it's not too dense) - Then, set necessary particle parameters.
      (if (`/Game/Landscape/DynamicGrassSystem/Blueprints/InternalLogic/INTERACTIVE_FoliageComp_BP.enableSmoke` (`self.ownerComponent`))
        (if (`/Game/Landscape/DynamicGrassSystem/Blueprints/InteractiveGrassManager_BP.OptimizeSmoke` _manager)
          (bind _returnvalue_3 (`|SpawnActorFromClass` "/Game/Landscape/DynamicGrassSystem/Blueprints/InternalLogic/SmokeParticleMark_BP.SmokeParticleMark_BP_C" (`self.GetTransform`) "AlwaysSpawn" "OverrideRootScale" null (`/Game/Landscape/DynamicGrassSystem/Blueprints/InteractiveGrassManager_BP.OptimizeSmoke_CheckRadius` _manager) (`/Game/Landscape/DynamicGrassSystem/Blueprints/InteractiveGrassManager_BP.OptimizeSmoke_maxOverlapping` _manager) null))
          (bind _ok_tospawn_2 (`/Game/Landscape/DynamicGrassSystem/Blueprints/InternalLogic/SmokeParticleMark_BP.CheckDensity` _returnvalue_3))
          (if _ok_tospawn_2
            (bind _returnvalue_4 (`|SpawnActorFromClass` "/Game/Landscape/DynamicGrassSystem/Blueprints/InternalLogic/Smoke_BP.Smoke_BP_C" (`self.GetTransform`) "AlwaysSpawn" "OverrideRootScale" null (`/Game/Landscape/DynamicGrassSystem/Blueprints/InternalLogic/INTERACTIVE_FoliageComp_BP.smokeSpawnHeight` _ownercomponent_5) (`/Game/Landscape/DynamicGrassSystem/Blueprints/InternalLogic/INTERACTIVE_FoliageComp_BP.smokeScale` _ownercomponent_5) (`/Game/Landscape/DynamicGrassSystem/Blueprints/InternalLogic/INTERACTIVE_FoliageComp_BP.smokeParticleLifetime` _ownercomponent_5) (`/Game/Landscape/DynamicGrassSystem/Blueprints/InternalLogic/INTERACTIVE_FoliageComp_BP.BurnDuration` _ownercomponent_5) null :!label _label_2))
            (bind _smokeparticles (`/Game/Landscape/DynamicGrassSystem/Blueprints/InternalLogic/Smoke_BP.SmokeParticles` _returnvalue_4))
            (`ParticleSystemComponent.SetVectorParameter` _smokeparticles "InitialVelocity" (* (`/Game/Landscape/DynamicGrassSystem/Blueprints/InteractiveGrassManager_BP.WindDirection` _manager_6) (* (`/Game/Landscape/DynamicGrassSystem/Blueprints/InteractiveGrassManager_BP.WindStrength` _manager_6) (`/Game/Landscape/DynamicGrassSystem/Blueprints/InteractiveGrassManager_BP.WindStrength_SmokeMultiplier` _manager_6))))
            (bind _returnvalue_5 (`KismetMaterialLibrary.CreateDynamicMaterialInstance` "/Game/Landscape/DynamicGrassSystem/Materials/Misc/ExampleSmoke_M.ExampleSmoke_M"))
            (`MaterialInstanceDynamic.SetVectorParameterValue` _returnvalue_5 "StartColor" (`/Game/Landscape/DynamicGrassSystem/Blueprints/InternalLogic/INTERACTIVE_FoliageComp_BP.smokeStartColor` (`self.ownerComponent`)))
            (`MaterialInstanceDynamic.SetVectorParameterValue` _returnvalue_5 "EndColor" (`/Game/Landscape/DynamicGrassSystem/Blueprints/InternalLogic/INTERACTIVE_FoliageComp_BP.smokeEndColor` (`self.ownerComponent`)))
            (`MaterialInstanceDynamic.SetScalarParameterValue` _returnvalue_5 "StartColorIntensity" (`/Game/Landscape/DynamicGrassSystem/Blueprints/InternalLogic/INTERACTIVE_FoliageComp_BP.smokeStartColor_Intensity` (`self.ownerComponent`)))
            (`MaterialInstanceDynamic.SetScalarParameterValue` _returnvalue_5 "EndColorAppearSpeed" (`/Game/Landscape/DynamicGrassSystem/Blueprints/InternalLogic/INTERACTIVE_FoliageComp_BP.smokeEndColor_AppearSpeed` (`self.ownerComponent`)))
            (`PrimitiveComponent.SetMaterial` _smokeparticles 0 _returnvalue_5))
          (else
            (goto _label_2)))))
    (:`then_2`
      ;[1 1 1] Spawn fire particle - and if optimization is enabled, first check if it's ok to spawn it (if it's not too dense) - Then, set necessary particle parameters.
      (if (`/Game/Landscape/DynamicGrassSystem/Blueprints/InternalLogic/INTERACTIVE_FoliageComp_BP.enableFire` _ownercomponent_4)
        (if (`/Game/Landscape/DynamicGrassSystem/Blueprints/InteractiveGrassManager_BP.OptimizeFire` _manager_4)
          (bind _returnvalue_6 (`|SpawnActorFromClass` "/Game/Landscape/DynamicGrassSystem/Blueprints/InternalLogic/FireParticleMark_BP.FireParticleMark_BP_C" (`self.GetTransform`) "AlwaysSpawn" "OverrideRootScale" null (`/Game/Landscape/DynamicGrassSystem/Blueprints/InteractiveGrassManager_BP.OptimizeFire_CheckRadius` _manager_4) (`/Game/Landscape/DynamicGrassSystem/Blueprints/InteractiveGrassManager_BP.OptimizeFire_maxOverlapping` _manager_4) null))
          (bind _ok_tospawn_3 (`/Game/Landscape/DynamicGrassSystem/Blueprints/InternalLogic/FireParticleMark_BP.CheckDensity` _returnvalue_6))
          (if _ok_tospawn_3
            (bind _returnvalue_7 (`|SpawnActorFromClass` "/Game/Landscape/DynamicGrassSystem/Blueprints/InternalLogic/Fire_BP.Fire_BP_C" (`self.GetTransform`) "AlwaysSpawn" "OverrideRootScale" null (`/Game/Landscape/DynamicGrassSystem/Blueprints/InternalLogic/INTERACTIVE_FoliageComp_BP.fireSpawnHeight` (`self.ownerComponent`)) (`KismetMathLibrary.RandomFloatInRange` _firescale (* _firescale 1.5)) (`/Game/Landscape/DynamicGrassSystem/Blueprints/InternalLogic/INTERACTIVE_FoliageComp_BP.BurnDuration` (`self.ownerComponent`)) null :!label _label_3))
            (bind _fireparticles (`/Game/Landscape/DynamicGrassSystem/Blueprints/InternalLogic/Fire_BP.FireParticles` _returnvalue_7))
            (`ParticleSystemComponent.SetVectorParameter` _fireparticles "InitialVelocity" (* (`/Game/Landscape/DynamicGrassSystem/Blueprints/InteractiveGrassManager_BP.WindDirection` _manager_5) (* (`/Game/Landscape/DynamicGrassSystem/Blueprints/InteractiveGrassManager_BP.WindStrength` _manager_5) (`/Game/Landscape/DynamicGrassSystem/Blueprints/InteractiveGrassManager_BP.WindStrength_FireMultiplier` _manager_5))))
            (bind _returnvalue_8 (`KismetMaterialLibrary.CreateDynamicMaterialInstance` "/Game/Landscape/DynamicGrassSystem/Materials/Misc/ExampleFire_M.ExampleFire_M"))
            (`MaterialInstanceDynamic.SetVectorParameterValue` _returnvalue_8 "StartColor" (`/Game/Landscape/DynamicGrassSystem/Blueprints/InternalLogic/INTERACTIVE_FoliageComp_BP.flameStartColor` (`self.ownerComponent`)))
            (`MaterialInstanceDynamic.SetVectorParameterValue` _returnvalue_8 "EndColor" (`/Game/Landscape/DynamicGrassSystem/Blueprints/InternalLogic/INTERACTIVE_FoliageComp_BP.flameEndColor` (`self.ownerComponent`)))
            (`MaterialInstanceDynamic.SetScalarParameterValue` _returnvalue_8 "StartColorIntensity" (`/Game/Landscape/DynamicGrassSystem/Blueprints/InternalLogic/INTERACTIVE_FoliageComp_BP.flameStartColor_Intensity` (`self.ownerComponent`)))
            (`MaterialInstanceDynamic.SetScalarParameterValue` _returnvalue_8 "EndColorIntensity" (`/Game/Landscape/DynamicGrassSystem/Blueprints/InternalLogic/INTERACTIVE_FoliageComp_BP.flameEndColor_Intensity` (`self.ownerComponent`)))
            (`PrimitiveComponent.SetMaterial` _fireparticles 0 _returnvalue_8) ; Index 0 == emitter nr 1 [flames]
            (bind _returnvalue_9 (`KismetMaterialLibrary.CreateDynamicMaterialInstance` "/Game/Landscape/DynamicGrassSystem/Materials/Misc/FireSpark_M.FireSpark_M"))
            (`MaterialInstanceDynamic.SetVectorParameterValue` _returnvalue_9 "StartColor" (`/Game/Landscape/DynamicGrassSystem/Blueprints/InternalLogic/INTERACTIVE_FoliageComp_BP.sparkStartColor` (`self.ownerComponent`)))
            (`MaterialInstanceDynamic.SetVectorParameterValue` _returnvalue_9 "EndColor" (`/Game/Landscape/DynamicGrassSystem/Blueprints/InternalLogic/INTERACTIVE_FoliageComp_BP.sparkEndColor` (`self.ownerComponent`)))
            (`MaterialInstanceDynamic.SetScalarParameterValue` _returnvalue_9 "StartColorIntensity" (`/Game/Landscape/DynamicGrassSystem/Blueprints/InternalLogic/INTERACTIVE_FoliageComp_BP.sparkColor_Intensity` (`self.ownerComponent`))) ; ... End intensity should always be '1' anyway, because otherwise it destroys smooth fade out by alpha.
            (`PrimitiveComponent.SetMaterial` _fireparticles 1 _returnvalue_9) ; Index 1 == emitter nr 2 [embers]
          )
          (else
            (goto _label_3)))))
    (:`then_3`
      ;[1 1 1] Create dynamic material for burning effect and set its parameters to match corresponding foliage material.
      (bind _returnvalue_10 (`KismetMaterialLibrary.CreateDynamicMaterialInstance` (select `bool` (`/Game/Landscape/DynamicGrassSystem/Blueprints/InternalLogic/INTERACTIVE_FoliageComp_BP.useDissolveBurnEffect` (`self.ownerComponent`)) :`false` "/Game/Landscape/DynamicGrassSystem/Materials/Grass/GrassBurnFade_M.GrassBurnFade_M" :`true` "/Game/Landscape/DynamicGrassSystem/Materials/Grass/GrassBurnDissolveFade_M.GrassBurnDissolveFade_M" :!type "MaterialInterface Object Reference")))
      (bind _output_get (set `self.dynFadeBurnMat` _returnvalue_10))
      (`MaterialInstanceDynamic.K2_CopyMaterialInstanceParameters` _output_get (`PrimitiveComponent.GetMaterial` (`self.ownerComponent`) 0) false)
      (`MaterialInstanceDynamic.SetScalarParameterValue` (`self.dynFadeBurnMat`) "BurnProgress" 0.0) ; To prevent blinking at start
      ;;[1 1 1] Ember color & intensity for e.g. grass blades
      (`MaterialInstanceDynamic.SetVectorParameterValue` (`self.dynFadeBurnMat`) "EmberColor" (`/Game/Landscape/DynamicGrassSystem/Blueprints/InternalLogic/INTERACTIVE_FoliageComp_BP.emberColor` (`self.ownerComponent`)))
      (`MaterialInstanceDynamic.SetScalarParameterValue` (`self.dynFadeBurnMat`) "EmberIntensity" (`/Game/Landscape/DynamicGrassSystem/Blueprints/InternalLogic/INTERACTIVE_FoliageComp_BP.emberColor_Intensity` (`self.ownerComponent`)))
      (`PrimitiveComponent.SetMaterial` (`self.TempBurndownGrassMesh`) 0 (`self.dynFadeBurnMat`))
      ;[1 1 1] Set start & target rotation for burning effect.
      (bind _output_get_2 (set `self.startRotation` (`SceneComponent.RelativeRotation` (`self.TempBurndownGrassMesh`))))
      (set `self.targetRotation` (`KismetMathLibrary.MakeRotator` (.roll _output_get_2) (+ (.pitch _output_get_2) (`/Game/Landscape/DynamicGrassSystem/Blueprints/InternalLogic/INTERACTIVE_FoliageComp_BP.LeanAmountWhenBurning` (`self.ownerComponent`))) (.yaw _output_get_2)))
      ;[1 1 1] If detected foliage uses dissolve burn effect, set the corresponding material parameter for this. If not, set start & end scale for another, non-dissolve effect.
      (if (`/Game/Landscape/DynamicGrassSystem/Blueprints/InternalLogic/INTERACTIVE_FoliageComp_BP.useDissolveBurnEffect` (`self.ownerComponent`))
        (`MaterialInstanceDynamic.SetTextureParameterValue` (`self.dynFadeBurnMat`) "BurnDissolveMask" _dissolvemask__texture)
        (else
          (bind _output_get_3 (set `self.startScale` (`SceneComponent.RelativeScale3D` (`self.TempBurndownGrassMesh`))))
          (set `self.targetScale` (`KismetMathLibrary.MakeVector` (.x _output_get_3) (.y _output_get_3) (`KismetMathLibrary.SelectFloat` (* (.z _output_get_3) 0.3) 0.0 (`/Game/Landscape/DynamicGrassSystem/Blueprints/InternalLogic/INTERACTIVE_FoliageComp_BP.leaveBurntGrass` (`self.ownerComponent`)))))))
      ;[1 1 1] Set burn duration. (The timeline has default 1.0 s. duration)
      (`TimelineComponent.SetPlayRate` (select `bool` (`/Game/Landscape/DynamicGrassSystem/Blueprints/InternalLogic/INTERACTIVE_FoliageComp_BP.useDissolveBurnEffect` (`self.ownerComponent`)) :`false` (`self.Timeline_Update4TopDownMat`) :`true` (`self.Timeline_Update4DissolveMat`)) (/ 1.0 (`/Game/Landscape/DynamicGrassSystem/Blueprints/InternalLogic/INTERACTIVE_FoliageComp_BP.BurnDuration` (`self.ownerComponent`))))
      (`|ExecutionSequence`
        (:`then_0`
          (`|ExecutionSequence`
            (:`then_0`
              ;[1 1 1] Optimization: The further from camera, the less frequent updates. It scales depending on values that can be set in the Manager.
              ; Also, if burn speed is slower, it also updates it less frequently. Fast updates are required only on faster burn speeds, to aboid 'choppy' mesh updates.
              (set `self.usesOptimizedUpdateInterval` (> (`self.DistanceToViewTarget`) (`/Game/Landscape/DynamicGrassSystem/Blueprints/InteractiveGrassManager_BP.BurnUpdateInterval_OptimizationStartRadius` (`self.manager`))))
              (set `self.currentUpdateInterval` (`KismetMathLibrary.SelectFloat` (* (`KismetMathLibrary.MapRangeClamped` (`self.DistanceToViewTarget`) (`/Game/Landscape/DynamicGrassSystem/Blueprints/InteractiveGrassManager_BP.BurnUpdateInterval_OptimizationStartRadius` _manager_3) 10000.0 1.0 (`/Game/Landscape/DynamicGrassSystem/Blueprints/InteractiveGrassManager_BP.BurnUpdateInterval_OptimizationFactor` _manager_3)) _returnvalue) _returnvalue (`self.usesOptimizedUpdateInterval`)) :!label _label_4)
              ;[1 1 1] Timer that updates burn progress. If current update interval is optimized (less frequent due to camera distance), it will check again after ~0.7s to avoid problems where player quickly runs into burning meshes that are still updating on optimized, less frequent intervals, resulting in 'choppy' motion.
              (bind _returnvalue_11 (`KismetSystemLibrary.K2_SetTimerDelegate` (select `bool` (`/Game/Landscape/DynamicGrassSystem/Blueprints/InternalLogic/INTERACTIVE_FoliageComp_BP.useDissolveBurnEffect` (`self.ownerComponent`)) :`false` (`|CreateDelegate` :!event `Update_4UpDownMat`) :`true` (`|CreateDelegate` :!event `Update_4DissolveMat`)) (`self.currentUpdateInterval`) true))
              (set `self.timer_UpdateBurningGrass` _returnvalue_11)
              (if (`self.usesOptimizedUpdateInterval`)
                (`KismetSystemLibrary.Delay` 1.0)
                (`self.CheckIfStillOptimizeInterval`)))
            (:`then_1`
              ;[1 1 1] Change different parameters depending on chosen burn effect
              (if (`/Game/Landscape/DynamicGrassSystem/Blueprints/InternalLogic/INTERACTIVE_FoliageComp_BP.useDissolveBurnEffect` (`self.ownerComponent`))
                ;[1 1 1] Set parameters over time - for dissolve burn effect.
                (bind (_direction _alpha _grassleanalpha _emberalpha) (`Timeline|Timeline_Update4DissolveMat` :!via `PlayFromStart`)
                  (:`Finished`
                    _))
                (else
                  ;[1 1 1] Set parameters over time - for standard burn effect.
                  (bind (_direction_2 _alpha_2 _emberalpha_2 _grassleanalpha_2 _noiseintensity) (`Timeline|Timeline_Update4TopDownMat` :!via `PlayFromStart`)
                    (:`Finished`
                      _))))
              ;[1 1 1] After completing the burn-effect parameter change, clear the update timer and if propagation process is done, destroy this temporary actor. If not, wait a little and try again.
              (`KismetSystemLibrary.K2_ClearAndInvalidateTimerHandle` (`self.timer_UpdateBurningGrass`))
              (if (`/Game/Landscape/DynamicGrassSystem/Blueprints/InternalLogic/INTERACTIVE_FoliageComp_BP.leaveBurntGrass` (`self.ownerComponent`))
                ;[0.04 0.04 0.04] Delete the actor and leave instanced, burnt grass mesh [OPTIONAL & EXPERIMENTAL - a flat, burned ground, without sticking grass is more realistic & more optimized.]
                (for _array_element (`self.K2_GetComponentsByClass` (`self.manager`) "/Script/Engine.InstancedStaticMeshComponent")
                  (if (== (`StaticMeshComponent.StaticMesh` _array_element) (`StaticMeshComponent.StaticMesh` (`self.TempBurndownGrassMesh`)))
                    (set `self.foundCompWithThisGrassMesh` true)
                    (set `self.foundCompWithGrass` _array_element)))
                (if (`self.foundCompWithThisGrassMesh`)
                  (`InstancedStaticMeshComponent.AddInstanceWorldSpace` (`self.foundCompWithGrass`) (`SceneComponent.K2_GetComponentToWorld` (`self.TempBurndownGrassMesh`)))
                  (else
                    (bind _returnvalue_12 (`AddComponent|NODE_AddInstancedStaticMeshComponent-0` :`self` (`self.manager`)))
                    (`StaticMeshComponent.SetStaticMesh` _returnvalue_12 (`StaticMeshComponent.StaticMesh` (`self.TempBurndownGrassMesh`)))
                    (bind _returnvalue_13 (`KismetMaterialLibrary.CreateDynamicMaterialInstance` "/Game/Landscape/DynamicGrassSystem/Materials/Grass/BurntGrass_M.BurntGrass_M"))
                    (bind _returnvalue_14 (`MaterialInstanceDynamic.K2_GetTextureParameterValue` (`self.dynFadeBurnMat`) "ColorTexture"))
                    (`MaterialInstanceDynamic.SetTextureParameterValue` _returnvalue_13 "ColorTexture" _returnvalue_14)
                    (bind _returnvalue_15 (`MaterialInstanceDynamic.K2_GetTextureParameterValue` (`self.dynFadeBurnMat`) "OpacityMask"))
                    (`MaterialInstanceDynamic.SetTextureParameterValue` _returnvalue_13 "OpacityMask" _returnvalue_15)
                    (bind _returnvalue_16 (`MaterialInstanceDynamic.K2_GetVectorParameterValue` (`self.dynFadeBurnMat`) "Tint2"))
                    (`MaterialInstanceDynamic.SetVectorParameterValue` _returnvalue_13 "Tint2" _returnvalue_16)
                    (`PrimitiveComponent.SetMaterial` _returnvalue_12 0 _returnvalue_13)
                    (`InstancedStaticMeshComponent.AddInstanceWorldSpace` _returnvalue_12 (`SceneComponent.K2_GetComponentToWorld` (`self.TempBurndownGrassMesh`)))))
                (`SceneComponent.SetHiddenInGame` (`self.TempBurndownGrassMesh`) true false)
                (`KismetSystemLibrary.Delay` 1.0 :!label _label_5)
                (if (or (`self.propagationDone`) (`self.reachedMaxPropagations`))
                  (`self.K2_DestroyActor`)
                  (else
                    (goto _label_5)))
                (else
                  (`KismetSystemLibrary.Delay` 1.0 :!label _label_6)
                  (if (or (`self.propagationDone`) (`self.reachedMaxPropagations`))
                    (`self.K2_DestroyActor`)
                    (else
                      (goto _label_6))))))))
        (:`then_1`
          ;[1 1 1] After delay determined by 'Propagate Duration' variables, check if this burning instance can propagate further.
          (`KismetSystemLibrary.Delay` (`KismetMathLibrary.RandomFloatInRange` (`/Game/Landscape/DynamicGrassSystem/Blueprints/InternalLogic/INTERACTIVE_FoliageComp_BP.PropagateDuration_Min` _ownercomponent_3) (`/Game/Landscape/DynamicGrassSystem/Blueprints/InternalLogic/INTERACTIVE_FoliageComp_BP.PropagateDuration_Max` _ownercomponent_3)))
          (if (`/Game/Landscape/DynamicGrassSystem/Blueprints/InteractiveGrassManager_BP.PROPAGATION_PROHIBITED` (`self.manager`))
            _
            (elif (`self.useMaxPropagations`)
              (bind __ (`/Game/Landscape/DynamicGrassSystem/Blueprints/InternalLogic/FireStarterLimiter_BP.HasReachedMaxPropagations` (`self.assignedLimiter`)))
              (if __
                (set `self.reachedMaxPropagations` true)
                (else
                  (`/Game/Landscape/DynamicGrassSystem/Blueprints/InternalLogic/FireStarterLimiter_BP.IncrementPropagationCounter` (`self.assignedLimiter`))
                  ;[1 1 1] If it can propagate further, spawn a new Fire Starter.
                  (`|SpawnActorFromClass` "/Game/Landscape/DynamicGrassSystem/Blueprints/FireStarter_BP.FireStarter_BP_C" (`self.GetTransform`) "AlwaysSpawn" "OverrideRootScale" null false (`self.useMaxPropagations`) 0 (`self.assignedLimiter`) (`/Game/Landscape/DynamicGrassSystem/Blueprints/InternalLogic/INTERACTIVE_FoliageComp_BP.propagateOnlyToSameType` _ownercomponent) _ownercomponent false null :!label _label_7)
                  (set `self.propagationDone` true)))
              (else
                (goto _label_7)))))))))

(event `CheckIfStillOptimizeInterval`
  ;[1 1 1] Optimization: The further from camera, the less frequent updates. It scales depending on values that can be set in the Manager.
  ; Also, if burn speed is slower, it also updates it less frequently. Fast updates are required only on faster burn speeds, to aboid 'choppy' mesh updates.
  (if (and (`self.usesOptimizedUpdateInterval`) (not (> (`self.DistanceToViewTarget`) (`/Game/Landscape/DynamicGrassSystem/Blueprints/InteractiveGrassManager_BP.BurnUpdateInterval_OptimizationStartRadius` (`self.manager`)))))
    (set `self.usesOptimizedUpdateInterval` false) ; FALSE
    (goto _label_4)
    (else
      (`KismetSystemLibrary.Delay` 1.0)
      (`self.CheckIfStillOptimizeInterval`))))

(event `Update_4DissolveMat`
  ;[1 1 1] Set parameters over time - for dissolve burn effect.
  (`MaterialInstanceDynamic.SetScalarParameterValue` (`self.dynFadeBurnMat`) "BurnProgress" (stale `self.ReceiveBeginPlay` _alpha))
  (`MaterialInstanceDynamic.SetScalarParameterValue` (`self.dynFadeBurnMat`) "Ember" (stale `self.ReceiveBeginPlay` _emberalpha))
  (`SceneComponent.K2_SetRelativeRotation` (`self.TempBurndownGrassMesh`) (`KismetMathLibrary.RLerp` (`self.startRotation`) (`self.targetRotation`) (stale `self.ReceiveBeginPlay` _grassleanalpha)) false false))

(event `Update_4UpDownMat`
  (bind _dynfadeburnmat (`self.dynFadeBurnMat`))
  ;[1 1 1] Set parameters over time - for standard burn effect.
  (`MaterialInstanceDynamic.SetScalarParameterValue` _dynfadeburnmat "Noise Intensity" (stale `self.ReceiveBeginPlay` _noiseintensity)) ; To eliminate displacement at the end of burning (without it, mesh visible even with 0 scale)
  (`MaterialInstanceDynamic.SetScalarParameterValue` _dynfadeburnmat "BurnProgress" (stale `self.ReceiveBeginPlay` _alpha_2))
  (`MaterialInstanceDynamic.SetScalarParameterValue` _dynfadeburnmat "Ember" (stale `self.ReceiveBeginPlay` _emberalpha_2))
  (`SceneComponent.SetRelativeScale3D` (`self.TempBurndownGrassMesh`) (`KismetMathLibrary.VLerp` (`self.startScale`) (`self.targetScale`) (stale `self.ReceiveBeginPlay` _alpha_2)))
  (`SceneComponent.K2_SetRelativeRotation` (`self.TempBurndownGrassMesh`) (`KismetMathLibrary.RLerp` (`self.startRotation`) (`self.targetRotation`) (stale `self.ReceiveBeginPlay` _grassleanalpha_2)) false false))

(fn `UserConstructionScript`
  ;[1 1 1] Set the temporary mesh to match the foliage component's mesh.
  (`StaticMeshComponent.SetStaticMesh` (`self.TempBurndownGrassMesh`) (`StaticMeshComponent.StaticMesh` (`self.ownerComponent`)))
  ;[1 1 1] Prevent auto switching to lower LOD when minimizing scale via burning
  (`StaticMeshComponent.SetForcedLodModel` (`self.TempBurndownGrassMesh`) 1))