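; Fire Blueprint for the Dynamic Grass System: a temporary fire effect that shrinks over its burn duration, then destroys itself.
; The construction script offsets the fire particles by the start height and applies the initial fire scale.
; On BeginPlay, a timeline rate-scaled to the burn duration drives an alpha.
; A looping quarter-second timer, rather than the timeline update, samples that alpha to lerp particle scale toward near zero.
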(event `self.ReceiveBeginPlay`
  ;[1 1 1] At begin, set target fire scale, scale transition duration (the timeline has default 1.0s duration) and update it via the timeline. After it's done, destroy the fire.
  (set `self.Scale` (`KismetMathLibrary.Conv_DoubleToVector` (`self.fireScale`)))
  (`TimelineComponent.SetPlayRate` (`self.Timeline`) (/ 1.0 (`self.burnDuration`)))
  (`|ExecutionSequence`
    (:`then_0`
      (`KismetSystemLibrary.K2_SetTimerDelegate` (delegate `UpdateFireParticle`) 0.25 true))
    (:`then_1`
      (bind (_direction _firealpha) (`Timeline|Timeline` :!via `PlayFromStart`)
        (:`Finished`
          (`KismetSystemLibrary.Delay` 0.1)
          (`self.K2_DestroyActor`))))))

(event `UpdateFireParticle`
  ;[1 1 1] At begin, set target fire scale, scale transition duration (the timeline has default 1.0s duration) and update it via the timeline. After it's done, destroy the fire.
  (`SceneComponent.SetRelativeScale3D` (`self.FireParticles`) (`KismetMathLibrary.VLerp` (`self.Scale`) (0.01 0.01 0.01) (stale `self.ReceiveBeginPlay` _firealpha))))

(fn `UserConstructionScript`
  (bind _firestartheight (`self.fireStartHeight`))
  ;[1 1 1] Add local offset to fire particles, based on specified height - also, set fire scale based on specified scale.
  (`SceneComponent.K2_AddLocalOffset` (`self.FireParticles`) (`KismetMathLibrary.MakeVector` _firestartheight _firestartheight) false false)
  (`SceneComponent.SetRelativeScale3D` (`self.FireParticles`) (`KismetMathLibrary.Conv_DoubleToVector` (`self.fireScale`))))