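; ExampleBomb_BP is an example thrown bomb for the Dynamic Grass System that explodes on a timer to deform and optionally ignite grass.
; On BeginPlay it launches along ThrowDirection, briefly ignoring collision before switching to blocking.
; After a fuse delay it plays a camera shake, explosion emitter and spawns Impulse_BP with optional displacement interaction.
; With FireStarting, it adds flames and waits for impulse deformation before spawning a propagating FireStarter_BP, then destroys itself.
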(event `self.ReceiveBeginPlay`
  (bind _totallyaccuratebomb (`self.TotallyAccurateBomb`))
  (bind _firestartertransform_location (`KismetMathLibrary.BreakTransform` (`self.fireStarterTransform`)))
  (bind _returnvalue (`SceneComponent.K2_GetComponentToWorld` _totallyaccuratebomb))
  (`PrimitiveComponent.SetCollisionResponseToAllChannels` (`self.TotallyAccurateBomb`) "ECR_Ignore")
  (`PrimitiveComponent.AddImpulse` (`self.TotallyAccurateBomb`) (`self.throwDirection`) "None" true)
  (`KismetSystemLibrary.Delay` 0.4)
  (`PrimitiveComponent.SetCollisionResponseToAllChannels` (`self.TotallyAccurateBomb`) "ECR_Block")
  (`KismetSystemLibrary.Delay` 2.0)
  (`GameplayStatics.PlayWorldCameraShake` "/Game/Landscape/DynamicGrassSystem/Blueprints/InternalLogic/CameraShake1_BP.CameraShake1_BP_C" (`self.K2_GetActorLocation`) 5000.0 100000.0)
  (`|SpawnActorFromClass` "/Game/Landscape/DynamicGrassSystem/Blueprints/InternalLogic/Impulse_BP.Impulse_BP_C" _returnvalue "AlwaysSpawn" "OverrideRootScale" null 350.0 20.0 0.3 (`self.useDisplacementInteraction`) true 400.0 null)
  (bind _output_get (set `self.fireStarterTransform` _returnvalue))
  (`GameplayStatics.SpawnEmitterAtLocation` "/Game/Landscape/DynamicGrassSystem/Particles/SimpleExplosion1_P.SimpleExplosion1_P" (.location _output_get))
  (if (`self.fireStarting`)
    (`ActorComponent.K2_DestroyComponent` _totallyaccuratebomb)
    (`ActorComponent.K2_DestroyComponent` (`self.PointLight`))
    (`GameplayStatics.SpawnEmitterAtLocation` "/Game/Landscape/DynamicGrassSystem/Particles/FireStart1_FlamesMore_P.FireStart1_FlamesMore_P" _firestartertransform_location)
    (`KismetSystemLibrary.Delay` 3.0) ; Wait for impulse deformation
    (`|SpawnActorFromClass` "/Game/Landscape/DynamicGrassSystem/Blueprints/FireStarter_BP.FireStarter_BP_C" (`self.fireStarterTransform`) "AlwaysSpawn" "OverrideRootScale" null true true 10 null false null false null))
  (`self.K2_DestroyActor`))

(fn `UserConstructionScript`)