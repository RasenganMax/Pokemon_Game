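; Smoke_BP is a self-cleaning smoke effect actor in the dynamic grass system that plays a particle effect for a set time.
; The construction script offsets the particles to a start height, scales them and sets a slightly randomized Lifetime parameter.
; On BeginPlay it waits for the duration, deactivates the emitter, then delays so remaining particles fade naturally before destroying the actor.
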(event `self.ReceiveBeginPlay`
  ;[1 1 1] After specified duration deactivate the smoke particles - then, after delay (to wait until any remaining particles will disappear naturally, without harsh disappearing) it destroys the actor.
  (`KismetSystemLibrary.Delay` (`self.Duration`))
  (`ActorComponent.Deactivate` (`self.SmokeParticles`))
  (`KismetSystemLibrary.Delay` 7.0)
  (`self.K2_DestroyActor`))

(fn `UserConstructionScript`
  (bind _smokelifetime (`self.smokeLifetime`))
  ;[1 1 1] Set desired smoke spawn height, its scale and lifetime.
  (`SceneComponent.K2_AddLocalOffset` (`self.SmokeParticles`) (`KismetMathLibrary.MakeVector` 0.0 0.0 (`self.smokeStartHeight`)) false false)
  (`SceneComponent.SetRelativeScale3D` (`self.SmokeParticles`) (`KismetMathLibrary.Conv_DoubleToVector` (`self.smokeScale`)))
  (`ParticleSystemComponent.SetFloatParameter` (`self.SmokeParticles`) "Lifetime" (`KismetMathLibrary.RandomFloatInRange` (* _smokelifetime 0.8) _smokelifetime)))