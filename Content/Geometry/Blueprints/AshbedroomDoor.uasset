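; Interactable hinged bedroom door that the player swings open when standing nearby and that later closes by itself.
; Box overlap registers the door as the ALS player character's InteractActor and sets NearDoor, clearing both on exit.
; Interact fires DoorOpen, which rotates the Door component with an eased MoveComponentTo over OpenCloseTime.
; Leaving the box starts a fixed delay, then eases the door back to zero relative rotation.
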(event `self.ReceiveBeginPlay`
  (bind _asals_base_character (cast `/Game/AdvancedLocomotionV3/Blueprints/ALS_BaseCharacter` (`GameplayStatics.GetPlayerCharacter` 0)))
  (set `self.Player` _asals_base_character))

(event `self.Box.OnComponentBeginOverlap`
  (params (OverlappedComponent :type "PrimitiveComponent Object Reference") (OtherActor :type "Actor Object Reference") (OtherComp :type "PrimitiveComponent Object Reference") (OtherBodyIndex :type Integer) (bFromSweep :type Boolean) (SweepResult :type "HitResult Structure (by ref)"))
  (bind _player (`self.Player`))
  (if (== OtherActor _player)
    (set `/Game/AdvancedLocomotionV3/Blueprints/ALS_BaseCharacter.Interact Actor` self _player)
    (set `self.NearDoor` true)))

(event `self.Box.OnComponentEndOverlap`
  (params (OverlappedComponent :type "PrimitiveComponent Object Reference") (OtherActor :type "Actor Object Reference") (OtherComp :type "PrimitiveComponent Object Reference") (OtherBodyIndex :type Integer))
  (bind _player (`self.Player`))
  (if (== _player OtherActor)
    (set `/Game/AdvancedLocomotionV3/Blueprints/ALS_BaseCharacter.Interact Actor` null _player)
    (set `self.NearDoor` false)
    (`KismetSystemLibrary.Delay` 10.0)
    (`KismetSystemLibrary.MoveComponentTo` (`self.Door`) (0.0 0.0 0.0) (struct) true true (`self.OpenCloseTime`) true)))

(event `DoorOpen`
  (if (`self.NearDoor`)
    (`KismetSystemLibrary.MoveComponentTo` (`self.Door`) (0.0 0.0 0.0) (struct :`Yaw` -105.0) true true (`self.OpenCloseTime`) true)))

(fn `Interact`
  (returns (Result :type Boolean))
  (`self.DoorOpen`)
  (return false))

(fn `UserConstructionScript`)