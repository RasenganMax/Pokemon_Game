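; BP_Fence_E1 is a procedural fence built along a spline in its construction script.
; Spline meshes follow the spline points, sharing one material with the pillars.
; Evenly spaced pillars become instanced meshes, while end pillars, placed only when the pillar count is positive, are separate static mesh components spread by their own count.
; Optional spline orientation rotates each end pillar, but rotates the whole instanced component rather than individual instances.
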(fn `UserConstructionScript`
  (locals (Temp_ISM :type "InstancedStaticMeshComponent Object Reference") (Local_Float :type "Float (double-precision)"))
  (bind _spline1 (`self.Spline1`))
  (bind _number_of_pillars (`self.Number of Pillars`))
  (bind _number_of_end_pillars (`self.Number of End Pillars`))
  (bind _splinemesh (`self.SplineMesh`))
  (bind _returnvalue (- _number_of_pillars 1))
  (bind _returnvalue_2 (- _number_of_end_pillars 1))
  (for _index (range (+ (- (`SplineComponent.GetNumberOfSplinePoints` (`self.Spline1`)) 2) 1))
    (bind _returnvalue_3 (+ _index 1))
    (`SplineMeshComponent.SetStartAndEnd` _splinemesh (`SplineComponent.GetLocationAtSplinePoint` _spline1 _index "Local") (`SplineComponent.GetTangentAtSplinePoint` _spline1 _index "Local") (`SplineComponent.GetLocationAtSplinePoint` _spline1 _returnvalue_3 "Local") (`SplineComponent.GetTangentAtSplinePoint` _spline1 _returnvalue_3 "Local") true)
    (`PrimitiveComponent.SetMaterial` _splinemesh 0 (`self.Element 0`)))
  (bind _returnvalue_4 (`AddComponent|NODE_AddInstancedStaticMeshComponent-0`))
  (set `local.Temp_ISM` _returnvalue_4)
  (if (> _number_of_pillars 0)
    (if (!= _returnvalue 0)
      (for _index_2 (range (+ _returnvalue 1))
        (bind _returnvalue_5 (* _index_2 (/ (`SplineComponent.GetSplineLength` (`self.Spline1`)) (`KismetMathLibrary.Conv_IntToDouble` _returnvalue))))
        (`InstancedStaticMeshComponent.AddInstance` (`local.Temp_ISM`) (`KismetMathLibrary.MakeTransform` (`KismetMathLibrary.InverseTransformLocation` (`self.GetTransform`) (`SplineComponent.GetLocationAtDistanceAlongSpline` (`self.Spline1`) _returnvalue_5 "World")) (struct) (`self.Mesh_Scale`)))
        (`PrimitiveComponent.SetMaterial` (`local.Temp_ISM`) 0 (`self.Element 0`))
        (`PrimitiveComponent.SetMaterial` (`self.Spline1`) 0 (`self.Element 0`))
        (if (`self.Orient to spline`)
          (`SceneComponent.K2_SetWorldRotation` (`local.Temp_ISM`) (`SplineComponent.GetRotationAtDistanceAlongSpline` (`self.Spline1`) _returnvalue_5 "World") false false) ; Rotate mesh to match direction of spline at its position
        )))
    (if (> _number_of_end_pillars 0)
      (if (!= _returnvalue_2 0)
        (set `local.Local_Float` (/ (`SplineComponent.GetSplineLength` (`self.Spline1`)) (`KismetMathLibrary.Conv_IntToDouble` _returnvalue_2)))
        (else
          (set `local.Local_Float` 0.0)))
      (for _index_3 (range (+ _returnvalue_2 1))
        (bind _returnvalue_6 (* _index_3 (`local.Local_Float`)))
        (bind _returnvalue_7 (`AddComponent|NODE_AddStaticMeshComponent-0` :`RelativeTransform` (`KismetMathLibrary.MakeTransform` (`KismetMathLibrary.InverseTransformLocation` (`self.GetTransform`) (`SplineComponent.GetLocationAtDistanceAlongSpline` (`self.Spline1`) _returnvalue_6 "World")) (struct) (`self.Pillar_Scale`)))) ; Add static mesh component
        (`PrimitiveComponent.SetMaterial` _returnvalue_7 0 (`self.Element 0`))
        (if (`self.Orient to spline`)
          (`SceneComponent.K2_SetWorldRotation` _returnvalue_7 (`SplineComponent.GetRotationAtDistanceAlongSpline` (`self.Spline1`) _returnvalue_6 "World") false false) ; Rotate mesh to match direction of spline at its position
        )))))