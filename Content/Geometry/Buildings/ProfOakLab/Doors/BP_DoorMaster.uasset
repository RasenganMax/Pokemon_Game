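; Master interactive door that the player can open, close or unlock with a key while inside its trigger box.
; A DoOnce-gated interaction unlocks it if the character's KeyInventory holds the required key, otherwise shows a message and plays a locked animation.
; Macros disable input and door collision, walk the player to the nearer side's anchor, rotate them by timeline and play a montage.
; When open/close montages blend out, MoveComponentTo swings the door.
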(event `self.ReceiveBeginPlay`
  (bind _returnvalue (`GameplayStatics.GetPlayerCharacter` 0))
  (bind _asals_base_character (cast `/Game/AdvancedLocomotionV3/Blueprints/ALS_BaseCharacter` _returnvalue))
  (set `self.Player` _asals_base_character)
  (bind _asmannequin_character (cast `/Game/AdvancedLocomotionV3/Blueprints/MannequinCharacter` _returnvalue))
  (set `self.Character_Ref` _asmannequin_character))

(event `/Game/Test/BluePrints/Interact/Interact_Interface.Interaction`
  ;[1 1 1] Interaction
  (`self.DoorOpen`))

(event `self.Box.OnComponentBeginOverlap`
  (params (OverlappedComponent :type "PrimitiveComponent Object Reference") (OtherActor :type "Actor Object Reference") (OtherComp :type "PrimitiveComponent Object Reference") (OtherBodyIndex :type Integer) (bFromSweep :type Boolean) (SweepResult :type "HitResult Structure (by ref)"))
  ;[1 1 1] Check if near door // Allow input
  (cast `/Game/AdvancedLocomotionV3/Blueprints/MannequinCharacter` OtherActor)
  (set `self.NearDoor` true)
  (`self.EnableInput` (`GameplayStatics.GetPlayerController` 0)))

(event `self.Box.OnComponentEndOverlap`
  (params (OverlappedComponent :type "PrimitiveComponent Object Reference") (OtherActor :type "Actor Object Reference") (OtherComp :type "PrimitiveComponent Object Reference") (OtherBodyIndex :type Integer))
  ;[1 1 1] Check if near door // Allow input
  (cast `/Game/AdvancedLocomotionV3/Blueprints/MannequinCharacter` OtherActor)
  (set `self.NearDoor` false)
  (`self.DisableInput` (`GameplayStatics.GetPlayerController` 0)))

(event `DoorOpen`
  (bind _returnvalue (`GameplayStatics.GetPlayerController` 0))
  (bind _character_ref (`self.Character_Ref`))
  (bind _character_ref_2 (`self.Character_Ref`))
  (bind _character_ref_3 (`self.Character_Ref`))
  (bind _character_ref_4 (`self.Character_Ref`))
  (bind _character_ref_5 (`self.Character_Ref`))
  (bind _mesh (`Character.Mesh` _character_ref))
  ;[1 1 1] Checks if close enough and if door is locked
  (if (`self.NearDoor`)
    (`/Engine/EditorBlueprintResources/StandardMacros.DoOnce` false :!label _label
      (:`Completed`
        (if (`self.IsLocked`)
          ;[1 1 1] If locked // Check if player has key
          (if (`KismetArrayLibrary.Array_Contains` (`/Game/AdvancedLocomotionV3/Blueprints/MannequinCharacter.KeyInventory` (`self.Character_Ref`)) (`self.KeyRequired`))
            (set `self.IsLocked` false)
            (goto _label :!via `Reset`)
            (else
              (`KismetSystemLibrary.PrintString` "You Need The Right Key")
              ;[1 1 1] Locked Anims
              (`self.DisableInput` (`self.Character_Ref`) (`GameplayStatics.GetPlayerController` 0))
              (`self.DisableCollision`)
              (if (> (`KismetMathLibrary.Vector_Distance` (`self.K2_GetActorLocation` (`self.Character_Ref`)) (`SceneComponent.K2_GetComponentLocation` (`self.LockedTowardsLoc`))) (`KismetMathLibrary.Vector_Distance` (`self.K2_GetActorLocation` (`self.Character_Ref`)) (`SceneComponent.K2_GetComponentLocation` (`self.LockedAwayLoc`))))
                (`AIBlueprintHelperLibrary.SimpleMoveToLocation` (`GameplayStatics.GetPlayerController` 0) (`SceneComponent.K2_GetComponentLocation` (`self.LockedAwayLoc`)))
                (`KismetSystemLibrary.Delay` 0.7)
                (bind (_direction _alpha) (`Timeline|Timeline_1` :!via `PlayFromStart`)
                  (:`Update`
                    (`self.K2_SetActorRotation` _character_ref_5 (`KismetMathLibrary.RLerp` (`self.K2_GetActorRotation` _character_ref_5) (`SceneComponent.K2_GetComponentRotation` (`self.LockedAwayLoc`)) _alpha true) false))
                  (:`Finished`
                    (`|PlayMontage` (`Character.Mesh` (`self.Character_Ref`)) (`self.AwayLockedMontage`)
                      (:`OnCompleted`
                        _)
                      (:`OnInterrupted`
                        (`KismetSystemLibrary.Delay` 1.5 :!label _label_2)))
                    (`self.EnableInput` (`self.Character_Ref`) (`GameplayStatics.GetPlayerController` 0) :!label _label_3)
                    (`PrimitiveComponent.SetCollisionEnabled` (`self.Door`) "QueryAndPhysics")
                    (goto _label :!via `Reset`)))
                (else
                  (`AIBlueprintHelperLibrary.SimpleMoveToLocation` (`GameplayStatics.GetPlayerController` 0) (`SceneComponent.K2_GetComponentLocation` (`self.LockedTowardsLoc`)))
                  (`KismetSystemLibrary.Delay` 0.7)
                  (bind (_direction_2 _alpha_2) (`Timeline|Timeline_2` :!via `PlayFromStart`)
                    (:`Update`
                      (`self.K2_SetActorRotation` _character_ref_4 (`KismetMathLibrary.RLerp` (`self.K2_GetActorRotation` _character_ref_4) (`SceneComponent.K2_GetComponentRotation` (`self.LockedTowardsLoc`)) _alpha_2 true) false))
                    (:`Finished`
                      (`|PlayMontage` (`Character.Mesh` (`self.Character_Ref`)) (`self.TowardsLockedMontage`)
                        (:`OnCompleted`
                          (goto _label_3))
                        (:`OnInterrupted`
                          (goto _label_2)))))))))
          (else
            (`self.DisableInput` (`self.Character_Ref`) (`GameplayStatics.GetPlayerController` 0))
            (if (`self.IsOpen`)
              (`self.DisableCollision`)
              (if (> (`KismetMathLibrary.Vector_Distance` (`self.K2_GetActorLocation` (`self.Character_Ref`)) (`SceneComponent.K2_GetComponentLocation` (`self.CloseAwayLoc`))) (`KismetMathLibrary.Vector_Distance` (`self.K2_GetActorLocation` (`self.Character_Ref`)) (`SceneComponent.K2_GetComponentLocation` (`self.CloseTowardsLoc`))))
                (`AIBlueprintHelperLibrary.SimpleMoveToLocation` (`GameplayStatics.GetPlayerController` 0) (`SceneComponent.K2_GetComponentLocation` (`self.CloseTowardsLoc`)))
                (`KismetSystemLibrary.Delay` 0.6)
                (bind (_direction_3 _alpha_3) (`Timeline|Timeline_3` :!via `PlayFromStart`)
                  (:`Update`
                    (`self.K2_SetActorRotation` _character_ref_3 (`KismetMathLibrary.RLerp` (`self.K2_GetActorRotation` (`self.Character_Ref`)) (`SceneComponent.K2_GetComponentRotation` (`self.CloseTowardsLoc`)) _alpha_3 true) false))
                  (:`Finished`
                    (`|PlayMontage` (`Character.Mesh` _character_ref_3) (`self.CloseTowardsMontage`)
                      (:`OnCompleted`
                        _)
                      (:`OnBlendOut`
                        ;[1 1 1] Unlocked Open
                        (set `self.IsOpen` false :!label _label_4)
                        (`KismetSystemLibrary.MoveComponentTo` (`self.Door`) (`self.DoorClosedLocation`) (`self.DoorClosedRotation`) true true (`self.OpenCloseTime`) true)
                        (goto _label :!via `Reset`))
                      (:`OnInterrupted`
                        (`KismetSystemLibrary.Delay` 1.5 :!label _label_5)))
                    (`self.EnableInput` (`self.Character_Ref`) (`GameplayStatics.GetPlayerController` 0) :!label _label_6)
                    (`PrimitiveComponent.SetCollisionEnabled` (`self.Door`) "QueryAndPhysics")))
                (else
                  (`AIBlueprintHelperLibrary.SimpleMoveToLocation` (`GameplayStatics.GetPlayerController` 0) (`SceneComponent.K2_GetComponentLocation` (`self.CloseAwayLoc`)))
                  (`KismetSystemLibrary.Delay` 1.0)
                  (bind (_direction_4 _alpha_4) (`Timeline|RotatePlayerClose` :!via `PlayFromStart`)
                    (:`Update`
                      (`self.K2_SetActorRotation` _character_ref_2 (`KismetMathLibrary.RLerp` (`self.K2_GetActorRotation` (`self.Character_Ref`)) (`SceneComponent.K2_GetComponentRotation` (`self.CloseAwayLoc`)) _alpha_4 true) false))
                    (:`Finished`
                      (`|PlayMontage` (`Character.Mesh` _character_ref_2) (`self.CloseAwayMontage`)
                        (:`OnCompleted`
                          (goto _label_6))
                        (:`OnBlendOut`
                          (goto _label_4))
                        (:`OnInterrupted`
                          (goto _label_5)))))))
              (else
                (`self.DisableCollision`)
                (if (> (`KismetMathLibrary.Vector_Distance` (`self.K2_GetActorLocation` (`self.Character_Ref`)) (`SceneComponent.K2_GetComponentLocation` (`self.OpenAwayLoc`))) (`KismetMathLibrary.Vector_Distance` (`self.K2_GetActorLocation` (`self.Character_Ref`)) (`SceneComponent.K2_GetComponentLocation` (`self.OpenTowardsLoc`))))
                  (`AIBlueprintHelperLibrary.SimpleMoveToLocation` _returnvalue (`SceneComponent.K2_GetComponentLocation` (`self.OpenTowardsLoc`)))
                  (`KismetSystemLibrary.Delay` 0.5)
                  (bind (_direction_5 _alpha_5) (`Timeline|RotatePlayerOpen` :!via `PlayFromStart`)
                    (:`Update`
                      (`self.K2_SetActorRotation` _character_ref (`KismetMathLibrary.RLerp` (`self.K2_GetActorRotation` (`self.Character_Ref`)) (`SceneComponent.K2_GetComponentRotation` (`self.OpenTowardsLoc`)) _alpha_5 true) false))
                    (:`Finished`
                      (`|PlayMontage` _mesh (`self.OpenTowardsMontage`)
                        (:`OnCompleted`
                          (goto _label_6))
                        (:`OnBlendOut`
                          (set `self.IsOpen` true :!label _label_7)
                          (`KismetSystemLibrary.MoveComponentTo` (`self.Door`) (`self.DoorOpenLocation`) (`self.DoorOpenRotation`) true true (`self.OpenCloseTime`) true)
                          (goto _label :!via `Reset`))
                        (:`OnInterrupted`
                          (goto _label_5)))))
                  (else
                    (`AIBlueprintHelperLibrary.SimpleMoveToLocation` _returnvalue (`SceneComponent.K2_GetComponentLocation` (`self.OpenAwayLoc`)))
                    (`KismetSystemLibrary.Delay` 0.5)
                    (bind (_direction_6 _alpha_6) (`Timeline|Timeline_0` :!via `PlayFromStart`)
                      (:`Update`
                        (`self.K2_SetActorRotation` _character_ref (`KismetMathLibrary.RLerp` (`self.K2_GetActorRotation` (`self.Character_Ref`)) (`SceneComponent.K2_GetComponentRotation` (`self.OpenAwayLoc`)) _alpha_6 true) false))
                      (:`Finished`
                        (`|PlayMontage` _mesh (`self.OpenAwayMontage`)
                          (:`OnCompleted`
                            (goto _label_6))
                          (:`OnBlendOut`
                            (goto _label_7))
                          (:`OnInterrupted`
                            (goto _label_5)))))))))))))))

(event `DisableCollision`
  (`PrimitiveComponent.SetCollisionEnabled` (`self.Door`) "NoCollision"))

(fn `UserConstructionScript`)