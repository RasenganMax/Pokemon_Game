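; Double basement door for the Prof Oak Lab building that the player opens and closes by interacting inside its trigger box.
; Locked doors require a matching key from the character's inventory, with touchpad materials flashing accepted or denied.
; MoveComponentTo eases both leaves between stored transforms, blocking re-triggers while moving, and a timer auto-closes them after the player leaves.
; Montage-based player positioning and locked-door animations exist but never run.
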(event `self.ReceiveBeginPlay`
  (bind _returnvalue (`GameplayStatics.GetPlayerCharacter` 0))
  ;[1 1 1] Set References
  (bind _asals_base_character (cast `/Game/AdvancedLocomotionV3/Blueprints/ALS_BaseCharacter` _returnvalue))
  (set `self.Player` _asals_base_character)
  (bind _asmannequin_character (cast `/Game/AdvancedLocomotionV3/Blueprints/MannequinCharacter` _returnvalue))
  (set `self.Character_Ref` _asmannequin_character))

(event `/Game/Test/BluePrints/Interact/Interact_Interface.Interaction`
  ;[1 0 0] Interaction // Check if picking up
  (`KismetSystemLibrary.Delay` 0.1)
  (if (not (`/Game/AdvancedLocomotionV3/Blueprints/MannequinCharacter.IsPickingUpItem` (`self.Character_Ref`)))
    (`self.DoorEvent`)))

(event `self.Box.OnComponentBeginOverlap`
  (params (OverlappedComponent :type "PrimitiveComponent Object Reference") (OtherActor :type "Actor Object Reference") (OtherComp :type "PrimitiveComponent Object Reference") (OtherBodyIndex :type Integer) (bFromSweep :type Boolean) (SweepResult :type "HitResult Structure (by ref)"))
  ;[1 1 1] Check if near door // Allow input
  (cast `/Game/AdvancedLocomotionV3/Blueprints/MannequinCharacter` OtherActor)
  (set `self.NearDoor` true)
  (`SceneComponent.SetVisibility` (`self.Interact`) true false)
  (`SceneComponent.SetVisibility` (`self.Interact2`) true false)
  ;[1 1 1] Stop timer when overlapping again
  (`KismetSystemLibrary.K2_ClearAndInvalidateTimerHandle` (stale `self.Box.OnComponentEndOverlap` _returnvalue)))

(event `self.Box.OnComponentEndOverlap`
  (params (OverlappedComponent :type "PrimitiveComponent Object Reference") (OtherActor :type "Actor Object Reference") (OtherComp :type "PrimitiveComponent Object Reference") (OtherBodyIndex :type Integer))
  ;[1 1 1] Check if near door // Allow input
  (cast `/Game/AdvancedLocomotionV3/Blueprints/MannequinCharacter` OtherActor)
  (set `self.NearDoor` false)
  (`SceneComponent.SetVisibility` (`self.LoackedDoor`) false false)
  (`SceneComponent.SetVisibility` (`self.Interact2`) false false)
  (`SceneComponent.SetVisibility` (`self.Interact`) false false)
  (`SceneComponent.SetVisibility` (`self.LockedDoor2`) false false)
  ;[1 1 1] Check if opened // Delay // Close door
  (if (`self.IsOpen`)
    (bind _returnvalue (`KismetSystemLibrary.K2_SetTimerDelegate` (delegate `Close On End Overlap`) 20.0))))

(event `DoorEvent`
  (bind _touchpad (`self.TouchPad`))
  (bind _touchpad_2 (`self.TouchPad`))
  ;[1 1 1] Checks if close enough and if door is locked
  (if (`self.NearDoor`)
    (if (`self.IsLocked`)
      ;[1 1 1] If locked // Check if player has key
      (`/Engine/EditorBlueprintResources/StandardMacros.DoOnce` false :!label _label
        (:`Completed`
          (if (`KismetArrayLibrary.Array_Contains` (`/Game/AdvancedLocomotionV3/Blueprints/MannequinCharacter.KeyInventory` (`self.Character_Ref`)) (`self.KeyRequired`))
            (`SceneComponent.SetVisibility` (`self.LoackedDoor`) false false)
            (`SceneComponent.SetVisibility` (`self.LockedDoor2`) false false)
            (`PrimitiveComponent.SetMaterial` _touchpad 1 "/Game/Geometry/Buildings/ProfOakLab/Storage/Accepted.Accepted")
            (`PrimitiveComponent.SetMaterial` (`self.TouchPad1`) 1 "/Game/Geometry/Buildings/ProfOakLab/Storage/Accepted.Accepted")
            (`KismetSystemLibrary.Delay` 0.2)
            (`PrimitiveComponent.SetMaterial` _touchpad 1 "/Game/Geometry/Buildings/ProfOakLab/Storage/Scan_Mat_Inst.Scan_Mat_Inst")
            (`PrimitiveComponent.SetMaterial` (`self.TouchPad1`) 1 "/Game/Geometry/Buildings/ProfOakLab/Storage/Scan_Mat_Inst.Scan_Mat_Inst")
            (set `self.IsLocked` false)
            (`self.Open/Close`)
            (goto _label :!via `Reset`)
            (else
              (`SceneComponent.SetVisibility` (`self.LoackedDoor`) true false)
              (`SceneComponent.SetVisibility` (`self.LockedDoor2`) true false)
              (`PrimitiveComponent.SetMaterial` _touchpad 1 "/Game/Geometry/Buildings/ProfOakLab/Storage/Denied.Denied")
              (`PrimitiveComponent.SetMaterial` (`self.TouchPad1`) 1 "/Game/Geometry/Buildings/ProfOakLab/Storage/Denied.Denied")
              (`KismetSystemLibrary.Delay` 0.2)
              (`PrimitiveComponent.SetMaterial` _touchpad 1 "/Game/Geometry/Buildings/ProfOakLab/Storage/Scan_Mat_Inst.Scan_Mat_Inst")
              (`PrimitiveComponent.SetMaterial` (`self.TouchPad1`) 1 "/Game/Geometry/Buildings/ProfOakLab/Storage/Scan_Mat_Inst.Scan_Mat_Inst")
              (goto _label :!via `Reset`)))))
      (else
        (`SceneComponent.SetVisibility` (`self.LoackedDoor`) false false)
        (`SceneComponent.SetVisibility` (`self.LockedDoor2`) false false)
        (`PrimitiveComponent.SetMaterial` _touchpad_2 1 "/Game/Geometry/Buildings/ProfOakLab/Storage/Accepted.Accepted")
        (`PrimitiveComponent.SetMaterial` (`self.TouchPad1`) 1 "/Game/Geometry/Buildings/ProfOakLab/Storage/Accepted.Accepted")
        (`KismetSystemLibrary.Delay` 0.2)
        (`PrimitiveComponent.SetMaterial` _touchpad_2 1 "/Game/Geometry/Buildings/ProfOakLab/Storage/Scan_Mat_Inst.Scan_Mat_Inst")
        (`PrimitiveComponent.SetMaterial` (`self.TouchPad1`) 1 "/Game/Geometry/Buildings/ProfOakLab/Storage/Scan_Mat_Inst.Scan_Mat_Inst")
        (`self.Open/Close`)))))

(event `Close On End Overlap`
  (bind _door (`self.Door`))
  ;[1 1 1] Unlocked Open
  (set `self.IsOpen` false)
  (`|ExecutionSequence`
    (:`then_0`
      (`KismetSystemLibrary.MoveComponentTo` (`self.Door`) (`self.DoorClosedLocation`) (`self.DoorClosedRotation`) true true (`self.OpenCloseTime`) true :!label _label_2)
      (set `self.IsMoving` false)
      (`PrimitiveComponent.SetCollisionEnabled` _door "QueryAndPhysics"))
    (:`then_1`
      (`KismetSystemLibrary.MoveComponentTo` (`self.Door2`) (`self.Door2ClosedLocation`) (`self.Door2ClosedRotation`) true true (`self.OpenCloseTime`) true :!label _label_3)
      (set `self.IsMoving` false)
      (`PrimitiveComponent.SetCollisionEnabled` _door "QueryAndPhysics"))))

(event `Open/Close`
  (bind _door (`self.Door`))
  (bind _door_2 (`self.Door`))
  ;[1 1 1] Unlocked Open
  ;;[1 1 1] Check if door is moving (Remove if you want door spamming allowed)
  (if (not (`self.IsMoving`))
    ;;[1 1 1] Check if door is open
    (if (`self.IsOpen`)
      (set `self.IsMoving` true)
      (`PrimitiveComponent.SetCollisionEnabled` _door "NoCollision")
      (set `self.IsOpen` false)
      (`|ExecutionSequence`
        (:`then_0`
          (goto _label_2))
        (:`then_1`
          (goto _label_3)))
      (else
        (set `self.IsMoving` true)
        (`PrimitiveComponent.SetCollisionEnabled` _door "NoCollision")
        (set `self.IsOpen` true)
        (`|ExecutionSequence`
          (:`then_0`
            (`KismetSystemLibrary.MoveComponentTo` (`self.Door`) (`self.DoorOpenLocation`) (`self.DoorOpenRotation`) true true (`self.OpenCloseTime`) true)
            (set `self.IsMoving` false)
            (`PrimitiveComponent.SetCollisionEnabled` _door_2 "QueryAndPhysics"))
          (:`then_1`
            (`KismetSystemLibrary.MoveComponentTo` (`self.Door2`) (`self.Door2OpenLocation`) (`self.Door2OpenRotation`) true true (`self.OpenCloseTime`) true)
            (set `self.IsMoving` false)
            (`PrimitiveComponent.SetCollisionEnabled` _door_2 "QueryAndPhysics")))))))

(event `DisableCollision`
  (bind _door (`self.Door`))
  ;[1 1 1] Unlocked Open
  (`PrimitiveComponent.SetCollisionEnabled` _door "NoCollision")
  (`PrimitiveComponent.SetCollisionEnabled` (`self.Door2`) "NoCollision")
  (`PrimitiveComponent.SetCollisionResponseToAllChannels` _door "ECR_Ignore")
  (`PrimitiveComponent.SetCollisionResponseToAllChannels` (`self.Door2`) "ECR_Ignore"))

(fn `UserConstructionScript`)