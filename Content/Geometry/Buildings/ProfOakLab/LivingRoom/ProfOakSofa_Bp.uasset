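; Blueprint for the sofa in Prof Oak's lab living room that lets the player's mannequin character sit down.
; BeginPlay caches the player character as a MannequinCharacter, and overlaps on the Enter component toggle a NearSeat flag.
; The Interaction event routes to SittingDown, which calls SittingOn on the cached player while NearSeat is set, with debug prints along the way.
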(event `self.ReceiveBeginPlay`
  (bind _asmannequin_character (cast `/Game/AdvancedLocomotionV3/Blueprints/MannequinCharacter` (`GameplayStatics.GetPlayerCharacter` 0)))
  (set `self.Player` _asmannequin_character))

(event `self.Enter.OnComponentBeginOverlap`
  (params (OverlappedComponent :type "PrimitiveComponent Object Reference") (OtherActor :type "Actor Object Reference") (OtherComp :type "PrimitiveComponent Object Reference") (OtherBodyIndex :type Integer) (bFromSweep :type Boolean) (SweepResult :type "HitResult Structure (by ref)"))
  (cast `/Game/AdvancedLocomotionV3/Blueprints/MannequinCharacter` OtherActor)
  (set `self.NearSeat` true)
  (`KismetSystemLibrary.PrintString` "Near chair"))

(event `self.Enter.OnComponentEndOverlap`
  (params (OverlappedComponent :type "PrimitiveComponent Object Reference") (OtherActor :type "Actor Object Reference") (OtherComp :type "PrimitiveComponent Object Reference") (OtherBodyIndex :type Integer))
  (cast `/Game/AdvancedLocomotionV3/Blueprints/MannequinCharacter` OtherActor)
  (set `self.NearSeat` false)
  (`KismetSystemLibrary.PrintString` "away from chair"))

(event `SittingDown`
  (if (`self.NearSeat`)
    (`KismetSystemLibrary.PrintString` "pressed E")
    (`/Game/AdvancedLocomotionV3/Blueprints/MannequinCharacter.SittingOn` (`self.Player`))))

(event `/Game/Test/BluePrints/Interact/Interact_Interface.Interaction`
  (`self.SittingDown`))

(fn `UserConstructionScript`)