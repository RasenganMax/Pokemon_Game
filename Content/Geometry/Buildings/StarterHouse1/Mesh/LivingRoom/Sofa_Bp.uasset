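; Sofa_Bp is an interactable living-room sofa that lets the player character sit down.
; BeginPlay caches the player as MannequinCharacter, and the Enter trigger sets or clears that character's InteractActor and a NearSeat flag as the player enters or leaves.
; Interact fires the SittingDown event, which calls the player's SittingOn when NearSeat is set, and always returns false.
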(event `self.ReceiveBeginPlay`
  (bind _asmannequin_character (cast `/Game/AdvancedLocomotionV3/Blueprints/MannequinCharacter` (`GameplayStatics.GetPlayerCharacter` 0)))
  (set `self.Player` _asmannequin_character))

(event `self.Enter.OnComponentBeginOverlap`
  (params (OverlappedComponent :type "PrimitiveComponent Object Reference") (OtherActor :type "Actor Object Reference") (OtherComp :type "PrimitiveComponent Object Reference") (OtherBodyIndex :type Integer) (bFromSweep :type Boolean) (SweepResult :type "HitResult Structure (by ref)"))
  (bind _player (`self.Player`))
  (if (== _player OtherActor)
    (set `/Game/AdvancedLocomotionV3/Blueprints/ALS_BaseCharacter.Interact Actor` self _player)
    (set `self.NearSeat` true)))

(event `self.Enter.OnComponentEndOverlap`
  (params (OverlappedComponent :type "PrimitiveComponent Object Reference") (OtherActor :type "Actor Object Reference") (OtherComp :type "PrimitiveComponent Object Reference") (OtherBodyIndex :type Integer))
  (bind _player (`self.Player`))
  (if (== _player OtherActor)
    (set `/Game/AdvancedLocomotionV3/Blueprints/ALS_BaseCharacter.Interact Actor` null _player)
    (set `self.NearSeat` false)))

(event `SittingDown`
  (if (`self.NearSeat`)
    (`/Game/AdvancedLocomotionV3/Blueprints/MannequinCharacter.SittingOn` (`self.Player`))))

(fn `Interact`
  (returns (Result :type Boolean))
  (`self.SittingDown`)
  (return false))

(fn `UserConstructionScript`)