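; Interactive sofa Blueprint for the StarterHouse1 living room that lets the player character sit down.
; It caches the player as a MannequinCharacter on BeginPlay.
; A box collision sets a NearSeat flag and toggles the Interact prompt's visibility as that player enters or leaves.
; The Interaction event calls SittingON on the player only while NearSeat is true, leaving the sitting logic to the character.
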(event `self.ReceiveBeginPlay`
  (bind _asmannequin_character (cast `/Game/AdvancedLocomotionV3/Blueprints/MannequinCharacter` (`GameplayStatics.GetPlayerCharacter` 0)))
  (set `self.Player` _asmannequin_character))

(event `self.Box Collision.OnComponentBeginOverlap`
  (params (OverlappedComponent :type "PrimitiveComponent Object Reference") (OtherActor :type "Actor Object Reference") (OtherComp :type "PrimitiveComponent Object Reference") (OtherBodyIndex :type Integer) (bFromSweep :type Boolean) (SweepResult :type "HitResult Structure (by ref)"))
  (if (== (`self.Player`) OtherActor)
    (set `self.NearSeat` true)
    (`SceneComponent.SetVisibility` (`self.Interact`) true false)))

(event `self.Box Collision.OnComponentEndOverlap`
  (params (OverlappedComponent :type "PrimitiveComponent Object Reference") (OtherActor :type "Actor Object Reference") (OtherComp :type "PrimitiveComponent Object Reference") (OtherBodyIndex :type Integer))
  (if (== (`self.Player`) OtherActor)
    (set `self.NearSeat` false)
    (`SceneComponent.SetVisibility` (`self.Interact`) false false)))

(event `/Game/Test/BluePrints/Interact/Interact_Interface.Interaction`
  (if (`self.NearSeat`)
    (`/Game/AdvancedLocomotionV3/Blueprints/MannequinCharacter.SittingON` (`self.Player`))))

(fn `UserConstructionScript`)