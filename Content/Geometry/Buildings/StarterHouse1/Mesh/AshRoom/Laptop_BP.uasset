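; Laptop_BP is an interactable laptop prop in the starter house that toggles what its screen shows.
; A box overlap with the ALS character sets a NearLaptop flag and shows or hides a widget.
; The Interaction event, when the player is near, flip-flops material slot 2 of the laptop mesh between a Charmander stats material and a Chair material.
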(event `self.ReceiveBeginPlay`
  (bind _asals_base_character (cast `/Game/AdvancedLocomotionV3/Blueprints/ALS_BaseCharacter` (`GameplayStatics.GetPlayerCharacter` 0)))
  (set `self.Player` _asals_base_character))

(event `self.Box.OnComponentBeginOverlap`
  (params (OverlappedComponent :type "PrimitiveComponent Object Reference") (OtherActor :type "Actor Object Reference") (OtherComp :type "PrimitiveComponent Object Reference") (OtherBodyIndex :type Integer) (bFromSweep :type Boolean) (SweepResult :type "HitResult Structure (by ref)"))
  (cast `/Game/AdvancedLocomotionV3/Blueprints/ALS_BaseCharacter` OtherActor)
  (set `self.NearLaptop` true)
  (`SceneComponent.SetVisibility` (`self.Widget`) true false))

(event `self.Box.OnComponentEndOverlap`
  (params (OverlappedComponent :type "PrimitiveComponent Object Reference") (OtherActor :type "Actor Object Reference") (OtherComp :type "PrimitiveComponent Object Reference") (OtherBodyIndex :type Integer))
  (cast `/Game/AdvancedLocomotionV3/Blueprints/ALS_BaseCharacter` OtherActor)
  (set `self.NearLaptop` false)
  (`SceneComponent.SetVisibility` (`self.Widget`) false false))

(event `/Game/Test/BluePrints/Interact/Interact_Interface.Interaction`
  (`self.TurnOnLaptop`))

(event `TurnOnLaptop`
  (bind _laptop (`self.Laptop`))
  (if (`self.NearLaptop`)
    (`/Engine/EditorBlueprintResources/StandardMacros.FlipFlop`
      (:`A`
        (`PrimitiveComponent.SetMaterial` _laptop 2 "/Game/Geometry/Buildings/StarterHouse1/Materials/House/AshRoom/CharmanderStats_Mat.CharmanderStats_Mat"))
      (:`B`
        (`PrimitiveComponent.SetMaterial` _laptop 2 "/Game/Geometry/Buildings/StarterHouse1/Materials/House/AshRoom/Chair.Chair")))))

(fn `UserConstructionScript`)